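; BP_Crate_Projectile is the projectile version of a crate, given a random mesh from an array on BeginPlay.
; SetOutline applies an outline overlay, then a looping timer checks the player's CanGrab and actor name to swap the overlay to the base material.
; Hits only print debug text, and the actor destroys itself when projectile movement stops.
; Crate respawn and physics impulse logic exist but are disconnected.
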(event `self.ReceiveBeginPlay`
  ;[1 1 1] here we randomly select one of the three assets at spawn but for this actore we want to select it following the non projectile object that the player has in hand
  (`StaticMeshComponent.SetStaticMesh` (`self.StaticMesh`) (`KismetArrayLibrary.Array_Random` (`self.MeshesArray`)))
  (set `self.Base_Material` (`PrimitiveComponent.GetMaterial` (`self.StaticMesh`) 0)))

(event `self.Set_Outline`
  (params (ActorToOutline :type "Actor Object Reference"))
  ;[0.0456 1 0] Gestion de L'outline
  (`MeshComponent.SetOverlayMaterial` (`self.StaticMesh`) "/Game/GA/VFX/Outline_Shader_Inst.Outline_Shader_Inst")
  (bind _returnvalue (`KismetSystemLibrary.K2_SetTimerDelegate` (delegate `CustomEvent`) 0.01 true)))

(event `CustomEvent`
  ;[0.0456 1 0] Gestion de L'outline
  (bind _asbp_player (cast `/Game/DEV/Players/FirstPerson/Blueprints/BP_Player` (`GameplayStatics.GetPlayerCharacter` 0)))
  (if (`/Game/DEV/Players/FirstPerson/Blueprints/BP_Player.CanGrab?` _asbp_player)
    (if (`KismetTextLibrary.EqualEqual_TextText` (`KismetTextLibrary.Conv_StringToText` (`KismetSystemLibrary.GetObjectName` self)) (`KismetTextLibrary.Conv_StringToText` (`KismetSystemLibrary.GetObjectName` (stale `self.Set_Outline` ActorToOutline))))
      (`MeshComponent.SetOverlayMaterial` (`self.StaticMesh`) (`self.Base_Material`) :!label _label)
      (`KismetSystemLibrary.K2_ClearAndInvalidateTimerHandle` (stale `self.Set_Outline` _returnvalue)))
    (else
      (goto _label))))

(event `self.ReceiveHit`
  (params (MyComp :type "PrimitiveComponent Object Reference") (Other :type "Actor Object Reference") (OtherComp :type "PrimitiveComponent Object Reference") (bSelfMoved :type Boolean) (HitLocation :type "Vector Structure") (HitNormal :type "Vector Structure") (NormalImpulse :type "Vector Structure") (Hit :type "HitResult Structure (by ref)"))
  ;[1 1 1] projectile hit
  (`KismetSystemLibrary.PrintString` "PROJECTILE HIT"))

(event `self.ProjectileMovement.OnProjectileStop`
  (params (ImpactResult :type "HitResult Structure (by ref)"))
  ;[1 1 1] projectile has stop
  (`KismetSystemLibrary.PrintString` "PROJECTILE STOPPED")
  (`self.K2_DestroyActor`))

(fn `UserConstructionScript`)