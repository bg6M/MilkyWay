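; Team-sensitive sound trap that fires a Niagara burst and a positional sound when a player enters its trigger sphere.
; Overlaps are handled on authority only, where the player's team selects the spawn count, sound and cooldown.
; GREEZ players cause a larger burst and a much longer cooldown than MANZ, with effects played through MC_Activate.
; The construction script sets the sphere radius from a variable.
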(event `self.ReceiveBeginPlay`
  (bind _asgs_lobby (cast `/Game/_Jam_MilkyWay/Players/MenuPlayer/GS_Lobby` (`GameplayStatics.GetGameState`)))
  (set `self.As GS Lobby` _asgs_lobby))

(event `self.Sphere.OnComponentBeginOverlap`
  (params (OverlappedComponent :type "PrimitiveComponent Object Reference") (OtherActor :type "Actor Object Reference") (OtherComp :type "PrimitiveComponent Object Reference") (OtherBodyIndex :type Integer) (bFromSweep :type Boolean) (SweepResult :type "HitResult Structure (by ref)"))
  (`/Engine/EditorBlueprintResources/ActorMacros.Switch Has Authority`
    (:`Authority`
      (`self.ServerOverlapp` OtherActor))))

(event `ServerOverlapp`
  (params (Actor :type "Actor Object Reference"))
  (bind _asbp_player (cast `/Game/_Jam_MilkyWay/Players/FirstPerson/Blueprints/BP_Player` Actor))
  (if (not (`self.HasTrigger`))
    (switch `/Game/_Jam_MilkyWay/Players/MenuPlayer/E_PlayersTeam` (`/Game/_Jam_MilkyWay/Players/FirstPerson/Blueprints/BP_Player.Team` _asbp_player)
      (:`NewEnumerator0`
        (`self.MC_Activate` 5)
        (set `self.HasTrigger` true)
        (`KismetSystemLibrary.Delay` 10.0)
        (set `self.HasTrigger` false))
      (:`NewEnumerator1`
        (`self.MC_Activate` 15 1)
        (set `self.HasTrigger` true)
        (`KismetSystemLibrary.Delay` 60.0)
        (set `self.HasTrigger` false)))))

(event `MC_Activate`
  (params (CrowValueValue :type Integer) (SoundIndex :type Integer))
  (bind _vfx_greez (`self.VFX_Greez`))
  (`NiagaraComponent.SetVariableInt` _vfx_greez "SpawnCount" CrowValueValue)
  (`ActorComponent.Activate` _vfx_greez true)
  (`GameplayStatics.PlaySoundAtLocation` (`|GetArrayItem` (`self.Sound`) SoundIndex) (`self.K2_GetActorLocation`) (struct) 1.0 1.0 0.0 "/Game/_Jam_MilkyWay/SFX/Attenuation_Types/SA_AnimalsLot.SA_AnimalsLot" null null null))

(fn `UserConstructionScript`
  (`SphereComponent.SetSphereRadius` (`self.Sphere`) (`self.In Sphere Radius`) true))