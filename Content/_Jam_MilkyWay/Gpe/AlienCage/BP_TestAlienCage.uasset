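; BP_TestAlienCage is a test actor for an alien cage that animates a fade effect on the cage's material.
; The construction script creates a dynamic material instance from the Cage component's first material slot.
; From BeginPlay, a timeline drives that instance's Fade scalar parameter and calls the fade event again when finished, so the animation replays continuously.
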(event `self.ReceiveBeginPlay`
  (`self.Change_Fade`))

(event `Change_Fade`
  (bind (_direction _newtrack_0) (`Timeline|Change_Fade_TL` :!via `PlayFromStart`)
    (:`Update`
      (`MaterialInstanceDynamic.SetScalarParameterValue` (`self.DynamicMaterialInstance`) "Fade" (`KismetMathLibrary.Lerp` 0.0 1.0 _newtrack_0)))
    (:`Finished`
      (`self.Change_Fade`))))

(fn `UserConstructionScript`
  (bind _cage (`self.Cage`))
  (bind _returnvalue (`PrimitiveComponent.CreateDynamicMaterialInstance` _cage 0 (`PrimitiveComponent.GetMaterial` _cage 0) "Fade"))
  (set `self.DynamicMaterialInstance` _returnvalue))