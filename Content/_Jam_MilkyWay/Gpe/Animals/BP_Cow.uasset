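; Replicated grabbable animal that becomes a chicken, sheep or cow by AnimalType, which selects its meshes, animation and sounds.
; Interface grabs route through RPCs, activating a lobby-assigned delivery point for GREEZ players; cows debuff the carrier and sheep release themselves after a random delay.
; OnRep_IsGrabed toggles physics and looping audio, while Tick disables movement replication during grabs and OnRep_GrabTransform interpolates the transform.
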(event OnAudioFinished(Audio_Animal)
  (Audio|Components|Audio|Play (Variables|Default|GetAudio_Animal) 0.0))

(event Custom|RPC%20GRAB
  (params (Target :type BP%20Player%20Object%20Reference))
  (Utilities|IsValid (Variables|Default|GetPlayer%20Calling%20Grab)
    (:Is%20Valid
      _)
    (:Is%20Not%20Valid
      (Variables|Default|SetPlayer%20Calling%20Grab Target)))
  (switch Utilities|FlowControl|Switch|SwitchonE_PlayersTeam (Variables|/Game/_Jam_MilkyWay/Players/FirstPerson/Blueprints/BP_Player.BP_Player_C|GetTeam (Variables|Default|GetPlayer%20Calling%20Grab))
    (:NewEnumerator0
      (Variables|Default|SetIsGrabed true))
    (:NewEnumerator1
      (Variables|Default|SetIsGrabed true)
      (Utilities|IsValid (Variables|Default|GetMyDeliveryPoint)
        (:Is%20Valid
          (if (Utilities|Array|ContainsItem (Variables|/Game/_Jam_MilkyWay/Players/MenuPlayer/GameRules/BP_DeliveryPoint.BP_DeliveryPoint_C|GetMyDeliveryList (Variables|Default|GetMyDeliveryPoint)) (Variables|Default|GetAnimalType))
            (Default|ServerActivatePoint (Variables|Default|GetMyDeliveryPoint) (Variables|Default|GetPlayer%20Calling%20Grab) true)
            (else
              (bind (_success _output_get) (Default|GetDelivery (Variables|Default|GetAs%20GS%20Lobby) (Variables|Default|GetAnimalType) (Variables|Default|GetPlayer%20Calling%20Grab) :!label _label))
              (if _success
                (bind _output_get_2 (Variables|Default|SetMyDeliveryPoint _output_get))
                (Default|ServerActivatePoint _output_get_2 (Variables|Default|GetPlayer%20Calling%20Grab) true)))))
        (:Is%20Not%20Valid
          (goto _label))))))

(event Custom|RPC%20UNGRAB
  ;[1 1 1 1 50] MC UNGRAB
  (switch Utilities|FlowControl|Switch|SwitchonE_PlayersTeam (Variables|/Game/_Jam_MilkyWay/Players/FirstPerson/Blueprints/BP_Player.BP_Player_C|GetTeam (Variables|Default|GetPlayer%20Calling%20Grab))
    (:NewEnumerator0
      _)
    (:NewEnumerator1
      (Default|ServerActivatePoint (Variables|Default|GetMyDeliveryPoint) (Variables|Default|GetPlayer%20Calling%20Grab) false)))
  (Variables|Default|SetIsGrabed false)
  (Variables|Default|SetPlayer%20Calling%20Grab 0))

(event Custom|RPC%20OUTLINE)

(event Custom|RPC_SheepUngrabItSelf
  (bind _player_calling_grab (Variables|Default|GetPlayer%20Calling%20Grab))
  (Utilities|FlowControl|Delay (Math|Random|RandomFloatinRange 6.0 15.0))
  (switch Utilities|FlowControl|Switch|SwitchonE_PlayersTeam (Variables|/Game/_Jam_MilkyWay/Players/FirstPerson/Blueprints/BP_Player.BP_Player_C|GetTeam _player_calling_grab)
    (:NewEnumerator0
      (Default|ManzUnActivateGrab _player_calling_grab false))
    (:NewEnumerator1
      (Default|GreezUnActivateGrab _player_calling_grab))))

(event Custom|ServerRPCGRAB
  (params (Player%20Calling%20Grab :type BP%20Player%20Object%20Reference))
  (CallFunction|RPCGRAB Player%20Calling%20Grab))

(event Custom|SERVER%20RPC%20UNGRAB
  (CallFunction|RPCUNGRAB))

(event Custom|Server%20MOO)

(event Custom|RPC%20MOO
  (params (Target :type Audio%20Component%20Object%20Reference))
  (Audio|Components|Audio|Play Target 0.0))

(event Custom|RPC%20SET%20DATA
  (CallFunction|SetData))

(event Custom|Server%20SET%20DATA
  (CallFunction|RPCSETDATA))

(event Custom|ServerAnimalExtracted
  (CallFunction|RPCAnimalExtracted))

(event Custom|RPCAnimalExtracted
  (Physics|SetSimulatePhysics (Variables|Default|GetMAIN_SM) false))

(event EventBeginPlay
  (Variables|Default|SetInitialMaterial (Rendering|Material|GetMaterial (Variables|Default|GetMeat) 0))
  (bind _asgs_lobby (Utilities|Casting|CastToGS_Lobby (Game|GetGameState))
    (:then
      (Variables|Default|SetAs%20GS%20Lobby _asgs_lobby))
    (:CastFailed
      _))
  (Variables|Default|SetIsGrabed false)
  (Audio|Components|Audio|Play (Variables|Default|GetAudio_Animal) 0.0))

(event EventToggleOutlineInteractible
  (params (Player%20Calling :type BP%20Player%20Object%20Reference))
  (Default|ACTIVATEOUTLINE Player%20Calling true (Variables|Default|GetMeat)))

(event EventTick
  (params (DeltaSeconds :type Float%20%28single-precision%29))
  (if (Variables|Default|GetIsGrabed)
    (Class|Actor|SetReplicateMovement false)
    (else
      (Class|Actor|SetReplicateMovement true))))

(event EventGrabInterface
  (params (Player%20calling%20grab :type BP%20Player%20Object%20Reference) (PlayerTeam :type E_PlayersTeam%20Enum :default "NewEnumerator0"))
  (Utilities|FlowControl|Sequence
    (:then_0
      (if (not (Variables|Default|GetIsDelivered))
        (Variables|Default|SetPlayer%20Team PlayerTeam)
        (bind _output_get (Variables|Default|SetPlayer%20Calling%20Grab Player%20calling%20grab))
        (CallFunction|ServerRPCGRAB _output_get)))
    (:then_1
      (Utilities|FlowControl|DoOnce false
        (:Completed
          (switch Utilities|FlowControl|Switch|SwitchonAnimalsList (Variables|Default|GetAnimalType)
            (:NewEnumerator0
              (Utilities|FlowControl|DoOnce false) ; enters at Reset
            )
            (:NewEnumerator1
              (CallFunction|RPCSheepUngrabItSelf)
              (Utilities|FlowControl|DoOnce false) ; enters at Reset
            )
            (:NewEnumerator2
              (Default|RPCApplyGrabDebuff Player%20calling%20grab true)
              (Utilities|FlowControl|DoOnce false) ; enters at Reset
            )))))))

(event EventUnGrabInterface
  (params (Player%20Calling%20Grab :type BP%20Player%20Object%20Reference))
  (Utilities|FlowControl|Sequence
    (:then_0
      (CallFunction|SERVERRPCUNGRAB)
      (if (>= (Transformation|GetDistanceTo (Variables|Default|GetMySpawner)) 1e+03)
        _))
    (:then_1
      (Utilities|FlowControl|DoOnce false
        (:Completed
          (switch Utilities|FlowControl|Switch|SwitchonAnimalsList (Variables|Default|GetAnimalType)
            (:NewEnumerator0
              (Utilities|FlowControl|DoOnce false) ; enters at Reset
            )
            (:NewEnumerator1
              (Utilities|FlowControl|DoOnce false) ; enters at Reset
            )
            (:NewEnumerator2
              (Default|RPCApplyGrabDebuff Player%20Calling%20Grab false)
              (Utilities|FlowControl|DoOnce false) ; enters at Reset
            )))))))

(fn ConstructionScript
  (CallFunction|SetData))

(fn SetData
  (bind _meat (Variables|Default|GetMeat))
  (bind _meat_2 (Variables|Default|GetMeat))
  (bind _meat_3 (Variables|Default|GetMeat))
  (switch Utilities|FlowControl|Switch|SwitchonAnimalsList (Variables|Default|GetAnimalType)
    (:NewEnumerator0
      (Components|StaticMesh|SetStaticMesh (Variables|Default|GetMAIN_SM) (Utilities|Array|Get(acopy) (Variables|Default|GetMain%20Mesh%20Collision)))
      (Components|SkeletalMesh|SetSkeletalMeshAsset _meat_3 (Utilities|Array|Get(acopy) (Variables|Default|GetAnimals%20SKM%20Bank)))
      (Class|SkeletalMeshComponent|SetAnimClass _meat_3 (Utilities|Array|Get(acopy) (Variables|Default|GetAnimals%20AnimBP%20Bank))))
    (:NewEnumerator1
      (Components|StaticMesh|SetStaticMesh (Variables|Default|GetMAIN_SM) (Utilities|Array|Get(acopy) (Variables|Default|GetMain%20Mesh%20Collision) 1))
      (Components|SkeletalMesh|SetSkeletalMeshAsset _meat (Utilities|Array|Get(acopy) (Variables|Default|GetAnimals%20SKM%20Bank) 1))
      (Class|SkeletalMeshComponent|SetAnimClass _meat (Utilities|Array|Get(acopy) (Variables|Default|GetAnimals%20AnimBP%20Bank) 1)))
    (:NewEnumerator2
      (Components|StaticMesh|SetStaticMesh (Variables|Default|GetMAIN_SM) (Utilities|Array|Get(acopy) (Variables|Default|GetMain%20Mesh%20Collision) 2))
      (Components|SkeletalMesh|SetSkeletalMeshAsset _meat_2 (Utilities|Array|Get(acopy) (Variables|Default|GetAnimals%20SKM%20Bank) 2))
      (Class|SkeletalMeshComponent|SetAnimClass _meat_2 (Utilities|Array|Get(acopy) (Variables|Default|GetAnimals%20AnimBP%20Bank) 2))))
  (Components|Animation|SetAnimationMode _meat "AnimationBlueprint" true))

(fn OnRepAnimalType
  (bind _meat (Variables|Default|GetMeat))
  (bind _meat_2 (Variables|Default|GetMeat))
  (bind _meat_3 (Variables|Default|GetMeat))
  (switch Utilities|FlowControl|Switch|SwitchonAnimalsList (Variables|Default|GetAnimalType)
    (:NewEnumerator0
      (Components|SkeletalMesh|SetSkeletalMeshAsset _meat_3 (Utilities|Array|Get(acopy) (Variables|Default|GetAnimals%20SKM%20Bank)))
      (Class|SkeletalMeshComponent|SetAnimClass _meat_3 (Utilities|Array|Get(acopy) (Variables|Default|GetAnimals%20AnimBP%20Bank))))
    (:NewEnumerator1
      (Components|SkeletalMesh|SetSkeletalMeshAsset _meat (Utilities|Array|Get(acopy) (Variables|Default|GetAnimals%20SKM%20Bank) 1))
      (Class|SkeletalMeshComponent|SetAnimClass _meat (Utilities|Array|Get(acopy) (Variables|Default|GetAnimals%20AnimBP%20Bank) 1)))
    (:NewEnumerator2
      (Components|SkeletalMesh|SetSkeletalMeshAsset _meat_2 (Utilities|Array|Get(acopy) (Variables|Default|GetAnimals%20SKM%20Bank) 2))
      (Class|SkeletalMeshComponent|SetAnimClass _meat_2 (Utilities|Array|Get(acopy) (Variables|Default|GetAnimals%20AnimBP%20Bank) 2))))
  (Components|Animation|SetAnimationMode _meat "AnimationBlueprint" true))

(fn OnRepIsDelivered
  (Physics|SetSimulatePhysics (Variables|Default|GetMAIN_SM) (not (Variables|Default|GetIsDelivered))))

(fn OnRepIsGrabed
  (bind _main_sm (Variables|Default|GetMAIN_SM))
  (bind _sound_bank (Variables|Default|GetSOUND%20BANK))
  (bind _audio_animal (Variables|Default|GetAudio_Animal))
  (bind _audio_animal_2 (Variables|Default|GetAudio_Animal))
  (bind _sound_bank_2 (Variables|Default|GetSOUND%20BANK))
  (bind _main_sm_2 (Variables|Default|GetMAIN_SM))
  (if (Variables|Default|GetIsGrabed)
    (Physics|SetSimulatePhysics _main_sm false)
    (Transformation|SetWorldRotation (Variables|Default|GetMAIN_SM) (Pawn|GetControlRotation (Variables|Default|GetPlayer%20Calling%20Grab) :!class /Script/Engine.Pawn) false false)
    (switch Utilities|FlowControl|Switch|SwitchonAnimalsList (Variables|Default|GetAnimalType)
      (:NewEnumerator0
        (Audio|Components|Audio|SetSound _audio_animal_2 (Utilities|Array|Get(acopy) _sound_bank_2 1)))
      (:NewEnumerator1
        (Audio|Components|Audio|SetSound _audio_animal_2 (Utilities|Array|Get(acopy) _sound_bank_2 3)))
      (:NewEnumerator2
        (Audio|Components|Audio|SetSound _audio_animal_2 (Utilities|Array|Get(acopy) _sound_bank_2 5))))
    (else
      (Physics|SetSimulatePhysics _main_sm true)
      (Physics|SetPhysicsLinearVelocity _main_sm_2 (* (Transformation|GetComponentVelocity _main_sm_2) 0.2) false "None")
      (Rendering|Material|SetMaterial (Variables|Default|GetMeat) 0 (Variables|Default|GetInitialMaterial))
      (Collision|SetCollisionEnabled (Variables|Default|GetMAIN_SM) "QueryAndPhysics")
      (switch Utilities|FlowControl|Switch|SwitchonAnimalsList (Variables|Default|GetAnimalType)
        (:NewEnumerator0
          (Audio|Components|Audio|SetSound _audio_animal (Utilities|Array|Get(acopy) _sound_bank)))
        (:NewEnumerator1
          (Audio|Components|Audio|SetSound _audio_animal (Utilities|Array|Get(acopy) _sound_bank 2)))
        (:NewEnumerator2
          (Audio|Components|Audio|SetSound _audio_animal (Utilities|Array|Get(acopy) _sound_bank 4))))))
  (Audio|Components|Audio|Play (Variables|Default|GetAudio_Animal) 0.0))

(fn OnRepGrabTransform
  (Transformation|SetActorTransform (Class|KismetMathLibrary|TInterpto (Transformation|GetActorTransform) (Variables|Default|GetGrabTransform) (Utilities|Time|GetWorldDeltaSeconds) 5.0) false true))