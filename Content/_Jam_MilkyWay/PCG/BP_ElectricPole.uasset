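; PCG electric pole actor that strings sagging cables between consecutive pylon instances of an instanced static mesh.
; PCGConstruction adds a raised cable component per pair, sized by distance plus slack; without SinglePylon it breaks the chain into three equal runs.
; It runs shortly after BeginPlay or on CreateCable, appending to ListCable without clearing.
; Cable ticking stops after a settling delay to freeze the simulation, and StartSimulation and StopSimulation toggle it.
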(event Custom|StopSimulation
  (for _array_element (Variables|Default|GetListCable)
    (Components|Tick|SetComponentTickEnabled _array_element false)))

(event Custom|Start%20Simulation
  (for _array_element (Variables|Default|GetListCable)
    (Components|Tick|SetComponentTickEnabled _array_element true)))

(event Custom|CreateCable
  (CallFunction|PCGConstruction))

(event EventBeginPlay
  (Utilities|FlowControl|Delay 1.0)
  (CallFunction|PCGConstruction)
  (Utilities|FlowControl|Delay 5.0)
  (for _array_element (Variables|Default|GetListCable)
    (Components|Tick|SetComponentTickEnabled _array_element false)))

(event Collision|EventActorBeginOverlap
  (params (OtherActor :type Actor%20Object%20Reference)))

(event EventTick
  (params (DeltaSeconds :type Float%20%28single-precision%29)))

(fn ConstructionScript)

(fn PCGConstruction
  (params (PCGData :type PCG%20Data%20Collection%20Structure))
  (bind _returnvalue (Actor|GetComponentbyClass "/Game/Blueprints/CableInstancedStaticMeshComponent.CableInstancedStaticMeshComponent_C"))
  (for _array_element (Utilities|Array|MakeArray _returnvalue)
    (for _index (range 0 (Components|InstancedStaticMesh|GetInstanceCount _array_element))
      (if (Variables|Default|GetSinglePylon)
        (if (< (+ _index 1) (Components|InstancedStaticMesh|GetInstanceCount _array_element)) :!label _label
          (bind _returnvalue_2 (AddComponent|AddCableComponent false (Math|Conversions|ToTransform(Vector) (+ (.location (.OutInstanceTransform (Components|InstancedStaticMesh|GetInstanceTransform _returnvalue _index false))) "0.000000,0.000000,1013.000000"))))
          (Utilities|Array|Add (Variables|Default|GetListCable) _returnvalue_2)
          (Variables|/Script/CableComponent.CableComponent|SetEndLocation _returnvalue_2 (+ (.location (.OutInstanceTransform (Components|InstancedStaticMesh|GetInstanceTransform _returnvalue (+ _index 1) false))) "0.000000,0.000000,1013.000000"))
          (Variables|/Script/CableComponent.CableComponent|SetCableLength _returnvalue_2 (+ (Math|Vector|Distance(Vector) (.location (.OutInstanceTransform (Components|InstancedStaticMesh|GetInstanceTransform _returnvalue _index false))) (.location (.OutInstanceTransform (Components|InstancedStaticMesh|GetInstanceTransform _returnvalue (+ _index 1) false)))) (Variables|Default|GetExtraLenght)))
          (Variables|/Script/CableComponent.CableComponent|SetCableWidth _returnvalue_2 (Variables|Default|GetCableThickness)))
        (elif (!= _index (- (/ (Components|InstancedStaticMesh|GetInstanceCount _array_element) 3) 1))
          (if (!= _index (+ (* (- (/ (Components|InstancedStaticMesh|GetInstanceCount _array_element) 3) 1) 2) 1))
            (goto _label)))))))