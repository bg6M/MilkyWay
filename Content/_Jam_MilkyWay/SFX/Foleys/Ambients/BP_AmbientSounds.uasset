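; Ambient sound controller that crossfades wind and grass sound cues as trigger boxes are entered and left.
; Low grass zones fade in crickets and grass wind while lowering general wind, and forest boxes swap it for forest wind.
; House, barn and hangar boxes attenuate general wind, the hangar only slightly.
; Timelines drive volume multipliers, with per-box booleans gating play and reverse across neighboring zones; only House's entry checks for BP_Player.
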(event `self.LowGrass_Detection.OnComponentBeginOverlap`
  (params (OverlappedComponent :type "PrimitiveComponent Object Reference") (OtherActor :type "Actor Object Reference") (OtherComp :type "PrimitiveComponent Object Reference") (OtherBodyIndex :type Integer) (bFromSweep :type Boolean) (SweepResult :type "HitResult Structure (by ref)"))
  ;[1 1 1] ACTIVATION DES BRUITS DE CRICKETS ET DU VENT DHERBE HAUTE + DIMINUTION DU VOLUME DU VENT GENERAL
  (set `self.isInLowGrass` true)
  (if (not (or (`self.isInLowGrass_0`) (`self.isInLowGrass_1`) (`self.isInLowGrass_2`) (`self.isInLowGrass_3`) (`self.isInLowGrass_4`) (`self.isInLowGrass_5`) (`self.isInLowGrass_6`) (`self.isInLowGrass_7`) (`self.isInLowGrass_8`) (`self.isInLowGrass_9`) (`self.isInLowGrass_10`) (`self.isInLowGrass_11`) (`self.isInLowGrass_12`)))
    (`|ExecutionSequence` :!label _label
      (:`then_0`
        (bind (_direction _volumemultiplier) (`Timeline|ToLowGrass` :!label _label_2)
          (:`Update`
            (`AudioComponent.SetVolumeMultiplier` (`self.LowGrass_SoundCue`) _volumemultiplier))))
      (:`then_1`
        (bind (_direction_2 _volumemultiplier_2) (`Timeline|WindAttenuationLowGrass` :!label _label_3)
          (:`Update`
            (`AudioComponent.SetVolumeMultiplier` (`self.Wind_SoundCue`) _volumemultiplier_2)))))))

(event `self.WindAttenuation_Box_House.OnComponentBeginOverlap`
  (params (OverlappedComponent :type "PrimitiveComponent Object Reference") (OtherActor :type "Actor Object Reference") (OtherComp :type "PrimitiveComponent Object Reference") (OtherBodyIndex :type Integer) (bFromSweep :type Boolean) (SweepResult :type "HitResult Structure (by ref)"))
  ;[1 1 1] ATTENUATION DU VENT GENERAL QUAND ON RENTRE DANS LA MAISON OU LA GRANGE
  (`self.House` OtherActor))

(event `House`
  (params (ActorOverlap :type "Actor Object Reference"))
  ;[1 1 1] ATTENUATION DU VENT GENERAL QUAND ON RENTRE DANS LA MAISON OU LA GRANGE
  (bind _asbp_player (cast `/Game/_Jam_MilkyWay/Players/FirstPerson/Blueprints/BP_Player` ActorOverlap))
  (if (== _asbp_player ActorOverlap)
    (set `self.isInHouse_0` true)
    (if (not (or (`self.isInHouse_1`) (`self.isInHouse_2`) (`self.isInHouse_3`) (`self.isInGrange`)))
      (bind (_direction _volumemultiplier) (`Timeline|WindAttenuation` :!label _label_4)
        (:`Update`
          (`AudioComponent.SetVolumeMultiplier` (`self.Wind_SoundCue`) _volumemultiplier))))))

(event `self.LowGrass_Detection1.OnComponentBeginOverlap`
  (params (OverlappedComponent :type "PrimitiveComponent Object Reference") (OtherActor :type "Actor Object Reference") (OtherComp :type "PrimitiveComponent Object Reference") (OtherBodyIndex :type Integer) (bFromSweep :type Boolean) (SweepResult :type "HitResult Structure (by ref)"))
  ;[1 1 1] ACTIVATION DES BRUITS DE CRICKETS ET DU VENT DHERBE HAUTE + DIMINUTION DU VOLUME DU VENT GENERAL
  (set `self.isInLowGrass_0` true)
  (if (not (or (`self.isInLowGrass`) (`self.isInLowGrass_1`) (`self.isInLowGrass_2`) (`self.isInLowGrass_3`) (`self.isInLowGrass_4`) (`self.isInLowGrass_5`) (`self.isInLowGrass_6`) (`self.isInLowGrass_7`) (`self.isInLowGrass_8`) (`self.isInLowGrass_9`) (`self.isInLowGrass_10`) (`self.isInLowGrass_11`) (`self.isInLowGrass_12`)))
    (goto _label)))

(event `House1`
  (params (ActorOverlap :type "Actor Object Reference"))
  ;[1 1 1] ATTENUATION DU VENT GENERAL QUAND ON RENTRE DANS LA MAISON OU LA GRANGE
  (set `self.isInHouse_1` true)
  (if (not (or (`self.isInHouse_0`) (`self.isInHouse_2`) (`self.isInHouse_3`) (`self.isInGrange`)))
    (goto _label_4)))

(event `self.WindAttenuation_Box_House2.OnComponentBeginOverlap`
  (params (OverlappedComponent :type "PrimitiveComponent Object Reference") (OtherActor :type "Actor Object Reference") (OtherComp :type "PrimitiveComponent Object Reference") (OtherBodyIndex :type Integer) (bFromSweep :type Boolean) (SweepResult :type "HitResult Structure (by ref)"))
  ;[1 1 1] ATTENUATION DU VENT GENERAL QUAND ON RENTRE DANS LA MAISON OU LA GRANGE
  (`self.House1` OtherActor))

(event `self.LowGrass_Detection2.OnComponentBeginOverlap`
  (params (OverlappedComponent :type "PrimitiveComponent Object Reference") (OtherActor :type "Actor Object Reference") (OtherComp :type "PrimitiveComponent Object Reference") (OtherBodyIndex :type Integer) (bFromSweep :type Boolean) (SweepResult :type "HitResult Structure (by ref)"))
  ;[1 1 1] ACTIVATION DES BRUITS DE CRICKETS ET DU VENT DHERBE HAUTE + DIMINUTION DU VOLUME DU VENT GENERAL
  (set `self.isInLowGrass_1` true)
  (if (not (or (`self.isInLowGrass`) (`self.isInLowGrass_0`) (`self.isInLowGrass_2`) (`self.isInLowGrass_3`) (`self.isInLowGrass_4`) (`self.isInLowGrass_5`) (`self.isInLowGrass_6`) (`self.isInLowGrass_7`) (`self.isInLowGrass_8`) (`self.isInLowGrass_9`) (`self.isInLowGrass_10`) (`self.isInLowGrass_11`) (`self.isInLowGrass_12`)))
    (goto _label)))

(event `House2`
  (params (ActorOverlap :type "Actor Object Reference"))
  ;[1 1 1] ATTENUATION DU VENT GENERAL QUAND ON RENTRE DANS LA MAISON OU LA GRANGE
  (set `self.isInHouse_2` true)
  (if (not (or (`self.isInHouse_0`) (`self.isInHouse_1`) (`self.isInHouse_3`) (`self.isInGrange`)))
    (goto _label_4)))

(event `self.WindAttenuation_Box_House3.OnComponentBeginOverlap`
  (params (OverlappedComponent :type "PrimitiveComponent Object Reference") (OtherActor :type "Actor Object Reference") (OtherComp :type "PrimitiveComponent Object Reference") (OtherBodyIndex :type Integer) (bFromSweep :type Boolean) (SweepResult :type "HitResult Structure (by ref)"))
  ;[1 1 1] ATTENUATION DU VENT GENERAL QUAND ON RENTRE DANS LA MAISON OU LA GRANGE
  (`self.House2` OtherActor))

(event `self.LowGrass_Detection3.OnComponentBeginOverlap`
  (params (OverlappedComponent :type "PrimitiveComponent Object Reference") (OtherActor :type "Actor Object Reference") (OtherComp :type "PrimitiveComponent Object Reference") (OtherBodyIndex :type Integer) (bFromSweep :type Boolean) (SweepResult :type "HitResult Structure (by ref)"))
  ;[1 1 1] ACTIVATION DES BRUITS DE CRICKETS ET DU VENT DHERBE HAUTE + DIMINUTION DU VOLUME DU VENT GENERAL
  (set `self.isInLowGrass_2` true)
  (if (not (or (`self.isInLowGrass`) (`self.isInLowGrass_0`) (`self.isInLowGrass_1`) (`self.isInLowGrass_3`) (`self.isInLowGrass_4`) (`self.isInLowGrass_5`) (`self.isInLowGrass_6`) (`self.isInLowGrass_7`) (`self.isInLowGrass_8`) (`self.isInLowGrass_9`) (`self.isInLowGrass_10`) (`self.isInLowGrass_11`) (`self.isInLowGrass_12`)))
    (goto _label)))

(event `House3`
  (params (ActorOverlap :type "Actor Object Reference"))
  ;[1 1 1] ATTENUATION DU VENT GENERAL QUAND ON RENTRE DANS LA MAISON OU LA GRANGE
  (set `self.isInHouse_3` true)
  (if (not (or (`self.isInHouse_0`) (`self.isInHouse_1`) (`self.isInHouse_2`) (`self.isInGrange`)))
    (goto _label_4)))

(event `self.WindAttenuation_Box_House4.OnComponentBeginOverlap`
  (params (OverlappedComponent :type "PrimitiveComponent Object Reference") (OtherActor :type "Actor Object Reference") (OtherComp :type "PrimitiveComponent Object Reference") (OtherBodyIndex :type Integer) (bFromSweep :type Boolean) (SweepResult :type "HitResult Structure (by ref)"))
  ;[1 1 1] ATTENUATION DU VENT GENERAL QUAND ON RENTRE DANS LA MAISON OU LA GRANGE
  (`self.House3` OtherActor))

(event `self.LowGrass_Detection4.OnComponentBeginOverlap`
  (params (OverlappedComponent :type "PrimitiveComponent Object Reference") (OtherActor :type "Actor Object Reference") (OtherComp :type "PrimitiveComponent Object Reference") (OtherBodyIndex :type Integer) (bFromSweep :type Boolean) (SweepResult :type "HitResult Structure (by ref)"))
  ;[1 1 1] ACTIVATION DES BRUITS DE CRICKETS ET DU VENT DHERBE HAUTE + DIMINUTION DU VOLUME DU VENT GENERAL
  (set `self.isInLowGrass_3` true)
  (if (not (or (`self.isInLowGrass`) (`self.isInLowGrass_0`) (`self.isInLowGrass_1`) (`self.isInLowGrass_2`) (`self.isInLowGrass_4`) (`self.isInLowGrass_5`) (`self.isInLowGrass_6`) (`self.isInLowGrass_7`) (`self.isInLowGrass_8`) (`self.isInLowGrass_9`) (`self.isInLowGrass_10`) (`self.isInLowGrass_11`) (`self.isInLowGrass_12`)))
    (goto _label)))

(event `self.LowGrass_Detection5.OnComponentBeginOverlap`
  (params (OverlappedComponent :type "PrimitiveComponent Object Reference") (OtherActor :type "Actor Object Reference") (OtherComp :type "PrimitiveComponent Object Reference") (OtherBodyIndex :type Integer) (bFromSweep :type Boolean) (SweepResult :type "HitResult Structure (by ref)"))
  ;[1 1 1] ACTIVATION DES BRUITS DE CRICKETS ET DU VENT DHERBE HAUTE + DIMINUTION DU VOLUME DU VENT GENERAL
  (set `self.isInLowGrass_4` true)
  (if (not (or (`self.isInLowGrass`) (`self.isInLowGrass_0`) (`self.isInLowGrass_1`) (`self.isInLowGrass_2`) (`self.isInLowGrass_3`) (`self.isInLowGrass_5`) (`self.isInLowGrass_6`) (`self.isInLowGrass_7`) (`self.isInLowGrass_8`) (`self.isInLowGrass_9`) (`self.isInLowGrass_10`) (`self.isInLowGrass_11`) (`self.isInLowGrass_12`)))
    (goto _label)))

(event `Grange`
  (params (ActorOverlap :type "Actor Object Reference"))
  ;[1 1 1] ATTENUATION DU VENT GENERAL QUAND ON RENTRE DANS LA MAISON OU LA GRANGE
  (set `self.isInGrange` true)
  (if (not (or (`self.isInHouse_0`) (`self.isInHouse_1`) (`self.isInHouse_2`) (`self.isInHouse_3`)))
    (goto _label_4)))

(event `self.WindAttenuation_Box_Grange.OnComponentBeginOverlap`
  (params (OverlappedComponent :type "PrimitiveComponent Object Reference") (OtherActor :type "Actor Object Reference") (OtherComp :type "PrimitiveComponent Object Reference") (OtherBodyIndex :type Integer) (bFromSweep :type Boolean) (SweepResult :type "HitResult Structure (by ref)"))
  ;[1 1 1] ATTENUATION DU VENT GENERAL QUAND ON RENTRE DANS LA MAISON OU LA GRANGE
  (`self.Grange` OtherActor))

(event `self.LowGrass_Detection6.OnComponentBeginOverlap`
  (params (OverlappedComponent :type "PrimitiveComponent Object Reference") (OtherActor :type "Actor Object Reference") (OtherComp :type "PrimitiveComponent Object Reference") (OtherBodyIndex :type Integer) (bFromSweep :type Boolean) (SweepResult :type "HitResult Structure (by ref)"))
  ;[1 1 1] ACTIVATION DES BRUITS DE CRICKETS ET DU VENT DHERBE HAUTE + DIMINUTION DU VOLUME DU VENT GENERAL
  (set `self.isInLowGrass_5` true)
  (if (not (or (`self.isInLowGrass`) (`self.isInLowGrass_0`) (`self.isInLowGrass_1`) (`self.isInLowGrass_2`) (`self.isInLowGrass_3`) (`self.isInLowGrass_4`) (`self.isInLowGrass_6`) (`self.isInLowGrass_7`) (`self.isInLowGrass_8`) (`self.isInLowGrass_9`) (`self.isInLowGrass_10`) (`self.isInLowGrass_11`) (`self.isInLowGrass_12`)))
    (goto _label)))

(event `self.LowGrass_Detection7.OnComponentBeginOverlap`
  (params (OverlappedComponent :type "PrimitiveComponent Object Reference") (OtherActor :type "Actor Object Reference") (OtherComp :type "PrimitiveComponent Object Reference") (OtherBodyIndex :type Integer) (bFromSweep :type Boolean) (SweepResult :type "HitResult Structure (by ref)"))
  ;[1 1 1] ACTIVATION DES BRUITS DE CRICKETS ET DU VENT DHERBE HAUTE + DIMINUTION DU VOLUME DU VENT GENERAL
  (set `self.isInLowGrass_6` true)
  (if (not (or (`self.isInLowGrass`) (`self.isInLowGrass_0`) (`self.isInLowGrass_1`) (`self.isInLowGrass_2`) (`self.isInLowGrass_3`) (`self.isInLowGrass_4`) (`self.isInLowGrass_5`) (`self.isInLowGrass_7`) (`self.isInLowGrass_8`) (`self.isInLowGrass_9`) (`self.isInLowGrass_10`) (`self.isInLowGrass_11`) (`self.isInLowGrass_12`)))
    (goto _label)))

(event `HouseB`
  (params (ActorOverlap :type "Actor Object Reference"))
  ;[1 1 1] ATTENUATION DU VENT GENERAL QUAND ON RENTRE DANS LA MAISON OU LA GRANGE
  (set `self.isInHouse_0` false)
  (if (not (or (`self.isInHouse_0`) (`self.isInHouse_1`) (`self.isInHouse_2`) (`self.isInHouse_3`)))
    (goto _label_4 :!via `Reverse`)))

(event `self.WindAttenuation_Box_House.OnComponentEndOverlap`
  (params (OverlappedComponent :type "PrimitiveComponent Object Reference") (OtherActor :type "Actor Object Reference") (OtherComp :type "PrimitiveComponent Object Reference") (OtherBodyIndex :type Integer))
  ;[1 1 1] ATTENUATION DU VENT GENERAL QUAND ON RENTRE DANS LA MAISON OU LA GRANGE
  (`self.HouseB` OtherActor))

(event `self.LowGrass_Detection8.OnComponentBeginOverlap`
  (params (OverlappedComponent :type "PrimitiveComponent Object Reference") (OtherActor :type "Actor Object Reference") (OtherComp :type "PrimitiveComponent Object Reference") (OtherBodyIndex :type Integer) (bFromSweep :type Boolean) (SweepResult :type "HitResult Structure (by ref)"))
  ;[1 1 1] ACTIVATION DES BRUITS DE CRICKETS ET DU VENT DHERBE HAUTE + DIMINUTION DU VOLUME DU VENT GENERAL
  (set `self.isInLowGrass_7` true)
  (if (not (or (`self.isInLowGrass`) (`self.isInLowGrass_0`) (`self.isInLowGrass_1`) (`self.isInLowGrass_2`) (`self.isInLowGrass_3`) (`self.isInLowGrass_4`) (`self.isInLowGrass_5`) (`self.isInLowGrass_6`) (`self.isInLowGrass_8`) (`self.isInLowGrass_9`) (`self.isInLowGrass_10`) (`self.isInLowGrass_11`) (`self.isInLowGrass_12`)))
    (goto _label)))

(event `self.WindAttenuation_Box_House2.OnComponentEndOverlap`
  (params (OverlappedComponent :type "PrimitiveComponent Object Reference") (OtherActor :type "Actor Object Reference") (OtherComp :type "PrimitiveComponent Object Reference") (OtherBodyIndex :type Integer))
  ;[1 1 1] ATTENUATION DU VENT GENERAL QUAND ON RENTRE DANS LA MAISON OU LA GRANGE
  (`self.House1B` OtherActor))

(event `House1B`
  (params (ActorOverlap :type "Actor Object Reference"))
  ;[1 1 1] ATTENUATION DU VENT GENERAL QUAND ON RENTRE DANS LA MAISON OU LA GRANGE
  (set `self.isInHouse_1` false)
  (if (not (or (`self.isInHouse_0`) (`self.isInHouse_2`) (`self.isInHouse_3`) (`self.isInGrange`)))
    (goto _label_4 :!via `Reverse`)))

(event `self.LowGrass_Detection9.OnComponentBeginOverlap`
  (params (OverlappedComponent :type "PrimitiveComponent Object Reference") (OtherActor :type "Actor Object Reference") (OtherComp :type "PrimitiveComponent Object Reference") (OtherBodyIndex :type Integer) (bFromSweep :type Boolean) (SweepResult :type "HitResult Structure (by ref)"))
  ;[1 1 1] ACTIVATION DES BRUITS DE CRICKETS ET DU VENT DHERBE HAUTE + DIMINUTION DU VOLUME DU VENT GENERAL
  (set `self.isInLowGrass_8` true)
  (if (not (or (`self.isInLowGrass`) (`self.isInLowGrass_0`) (`self.isInLowGrass_1`) (`self.isInLowGrass_2`) (`self.isInLowGrass_3`) (`self.isInLowGrass_4`) (`self.isInLowGrass_5`) (`self.isInLowGrass_6`) (`self.isInLowGrass_7`) (`self.isInLowGrass_9`) (`self.isInLowGrass_10`) (`self.isInLowGrass_11`) (`self.isInLowGrass_12`)))
    (goto _label)))

(event `self.WindAttenuation_Box_House3.OnComponentEndOverlap`
  (params (OverlappedComponent :type "PrimitiveComponent Object Reference") (OtherActor :type "Actor Object Reference") (OtherComp :type "PrimitiveComponent Object Reference") (OtherBodyIndex :type Integer))
  ;[1 1 1] ATTENUATION DU VENT GENERAL QUAND ON RENTRE DANS LA MAISON OU LA GRANGE
  (`self.House2B` OtherActor))

(event `House2B`
  (params (ActorOverlap :type "Actor Object Reference"))
  ;[1 1 1] ATTENUATION DU VENT GENERAL QUAND ON RENTRE DANS LA MAISON OU LA GRANGE
  (set `self.isInHouse_2` false)
  (if (not (or (`self.isInHouse_0`) (`self.isInHouse_1`) (`self.isInHouse_3`) (`self.isInGrange`)))
    (goto _label_4 :!via `Reverse`)))

(event `self.LowGrass_Detection10.OnComponentBeginOverlap`
  (params (OverlappedComponent :type "PrimitiveComponent Object Reference") (OtherActor :type "Actor Object Reference") (OtherComp :type "PrimitiveComponent Object Reference") (OtherBodyIndex :type Integer) (bFromSweep :type Boolean) (SweepResult :type "HitResult Structure (by ref)"))
  ;[1 1 1] ACTIVATION DES BRUITS DE CRICKETS ET DU VENT DHERBE HAUTE + DIMINUTION DU VOLUME DU VENT GENERAL
  (set `self.isInLowGrass_9` true)
  (if (not (or (`self.isInLowGrass`) (`self.isInLowGrass_0`) (`self.isInLowGrass_1`) (`self.isInLowGrass_2`) (`self.isInLowGrass_3`) (`self.isInLowGrass_4`) (`self.isInLowGrass_5`) (`self.isInLowGrass_6`) (`self.isInLowGrass_7`) (`self.isInLowGrass_8`) (`self.isInLowGrass_10`) (`self.isInLowGrass_11`) (`self.isInLowGrass_12`)))
    (goto _label)))

(event `self.WindAttenuation_Box_House4.OnComponentEndOverlap`
  (params (OverlappedComponent :type "PrimitiveComponent Object Reference") (OtherActor :type "Actor Object Reference") (OtherComp :type "PrimitiveComponent Object Reference") (OtherBodyIndex :type Integer))
  ;[1 1 1] ATTENUATION DU VENT GENERAL QUAND ON RENTRE DANS LA MAISON OU LA GRANGE
  (`self.House3B` OtherActor))

(event `House3B`
  (params (ActorOverlap :type "Actor Object Reference"))
  ;[1 1 1] ATTENUATION DU VENT GENERAL QUAND ON RENTRE DANS LA MAISON OU LA GRANGE
  (set `self.isInHouse_3` false)
  (if (not (or (`self.isInHouse_0`) (`self.isInHouse_1`) (`self.isInHouse_2`) (`self.isInGrange`)))
    (goto _label_4 :!via `Reverse`)))

(event `self.LowGrass_Detection11.OnComponentBeginOverlap`
  (params (OverlappedComponent :type "PrimitiveComponent Object Reference") (OtherActor :type "Actor Object Reference") (OtherComp :type "PrimitiveComponent Object Reference") (OtherBodyIndex :type Integer) (bFromSweep :type Boolean) (SweepResult :type "HitResult Structure (by ref)"))
  ;[1 1 1] ACTIVATION DES BRUITS DE CRICKETS ET DU VENT DHERBE HAUTE + DIMINUTION DU VOLUME DU VENT GENERAL
  (set `self.isInLowGrass_10` true)
  (if (not (or (`self.isInLowGrass`) (`self.isInLowGrass_0`) (`self.isInLowGrass_1`) (`self.isInLowGrass_2`) (`self.isInLowGrass_3`) (`self.isInLowGrass_4`) (`self.isInLowGrass_5`) (`self.isInLowGrass_6`) (`self.isInLowGrass_7`) (`self.isInLowGrass_8`) (`self.isInLowGrass_9`) (`self.isInLowGrass_11`) (`self.isInLowGrass_12`)))
    (goto _label)))

(event `self.WindAttenuation_Box_Grange.OnComponentEndOverlap`
  (params (OverlappedComponent :type "PrimitiveComponent Object Reference") (OtherActor :type "Actor Object Reference") (OtherComp :type "PrimitiveComponent Object Reference") (OtherBodyIndex :type Integer))
  ;[1 1 1] ATTENUATION DU VENT GENERAL QUAND ON RENTRE DANS LA MAISON OU LA GRANGE
  (`self.GrangeB` OtherActor))

(event `GrangeB`
  (params (ActorOverlap :type "Actor Object Reference"))
  ;[1 1 1] ATTENUATION DU VENT GENERAL QUAND ON RENTRE DANS LA MAISON OU LA GRANGE
  (set `self.isInGrange` false)
  (if (not (or (`self.isInHouse_0`) (`self.isInHouse_1`) (`self.isInHouse_2`) (`self.isInHouse_3`)))
    (goto _label_4 :!via `Reverse`)))

(event `self.LowGrass_Detection12.OnComponentBeginOverlap`
  (params (OverlappedComponent :type "PrimitiveComponent Object Reference") (OtherActor :type "Actor Object Reference") (OtherComp :type "PrimitiveComponent Object Reference") (OtherBodyIndex :type Integer) (bFromSweep :type Boolean) (SweepResult :type "HitResult Structure (by ref)"))
  ;[1 1 1] ACTIVATION DES BRUITS DE CRICKETS ET DU VENT DHERBE HAUTE + DIMINUTION DU VOLUME DU VENT GENERAL
  (set `self.isInLowGrass_11` true)
  (if (not (or (`self.isInLowGrass`) (`self.isInLowGrass_0`) (`self.isInLowGrass_1`) (`self.isInLowGrass_2`) (`self.isInLowGrass_3`) (`self.isInLowGrass_4`) (`self.isInLowGrass_5`) (`self.isInLowGrass_6`) (`self.isInLowGrass_7`) (`self.isInLowGrass_8`) (`self.isInLowGrass_9`) (`self.isInLowGrass_10`) (`self.isInLowGrass_12`)))
    (goto _label)))

(event `self.LowGrass_Detection13.OnComponentBeginOverlap`
  (params (OverlappedComponent :type "PrimitiveComponent Object Reference") (OtherActor :type "Actor Object Reference") (OtherComp :type "PrimitiveComponent Object Reference") (OtherBodyIndex :type Integer) (bFromSweep :type Boolean) (SweepResult :type "HitResult Structure (by ref)"))
  ;[1 1 1] ACTIVATION DES BRUITS DE CRICKETS ET DU VENT DHERBE HAUTE + DIMINUTION DU VOLUME DU VENT GENERAL
  (set `self.isInLowGrass_12` true)
  (if (not (or (`self.isInLowGrass`) (`self.isInLowGrass_0`) (`self.isInLowGrass_1`) (`self.isInLowGrass_2`) (`self.isInLowGrass_3`) (`self.isInLowGrass_4`) (`self.isInLowGrass_5`) (`self.isInLowGrass_6`) (`self.isInLowGrass_7`) (`self.isInLowGrass_8`) (`self.isInLowGrass_9`) (`self.isInLowGrass_10`) (`self.isInLowGrass_11`)))
    (goto _label)))

(event `self.WindAttenuation_Box_Hangar.OnComponentBeginOverlap`
  (params (OverlappedComponent :type "PrimitiveComponent Object Reference") (OtherActor :type "Actor Object Reference") (OtherComp :type "PrimitiveComponent Object Reference") (OtherBodyIndex :type Integer) (bFromSweep :type Boolean) (SweepResult :type "HitResult Structure (by ref)"))
  ;[1 1 1] ATTENUATION LEGERE DU VENT GENERAL QUAND ON RENTRE DANS LE HANGAR
  (set `self.isInHangar` true)
  (bind (_direction _volumemultiplier) (`Timeline|WindAttenuationFaible` :!label _label_5)
    (:`Update`
      (`AudioComponent.SetVolumeMultiplier` (`self.Wind_SoundCue`) _volumemultiplier))))

(event `self.WindAttenuation_Box_Hangar.OnComponentEndOverlap`
  (params (OverlappedComponent :type "PrimitiveComponent Object Reference") (OtherActor :type "Actor Object Reference") (OtherComp :type "PrimitiveComponent Object Reference") (OtherBodyIndex :type Integer))
  ;[1 1 1] ATTENUATION LEGERE DU VENT GENERAL QUAND ON RENTRE DANS LE HANGAR
  (set `self.isInHangar` false)
  (goto _label_5 :!via `Reverse`))

(event `self.LowGrass_Detection.OnComponentEndOverlap`
  (params (OverlappedComponent :type "PrimitiveComponent Object Reference") (OtherActor :type "Actor Object Reference") (OtherComp :type "PrimitiveComponent Object Reference") (OtherBodyIndex :type Integer))
  ;[1 1 1] ACTIVATION DES BRUITS DE CRICKETS ET DU VENT DHERBE HAUTE + DIMINUTION DU VOLUME DU VENT GENERAL
  (set `self.isInLowGrass` false)
  (if (not (or (`self.isInLowGrass_0`) (`self.isInLowGrass_1`) (`self.isInLowGrass_2`) (`self.isInLowGrass_3`) (`self.isInLowGrass_4`) (`self.isInLowGrass_5`) (`self.isInLowGrass_6`) (`self.isInLowGrass_7`) (`self.isInLowGrass_8`) (`self.isInLowGrass_9`) (`self.isInLowGrass_10`) (`self.isInLowGrass_11`) (`self.isInLowGrass_12`)))
    (`|ExecutionSequence` :!label _label_6
      (:`then_0`
        (goto _label_2 :!via `Reverse`))
      (:`then_1`
        (goto _label_3 :!via `Reverse`)))))

(event `self.LowGrass_Detection1.OnComponentEndOverlap`
  (params (OverlappedComponent :type "PrimitiveComponent Object Reference") (OtherActor :type "Actor Object Reference") (OtherComp :type "PrimitiveComponent Object Reference") (OtherBodyIndex :type Integer))
  ;[1 1 1] ACTIVATION DES BRUITS DE CRICKETS ET DU VENT DHERBE HAUTE + DIMINUTION DU VOLUME DU VENT GENERAL
  (set `self.isInLowGrass_0` false)
  (if (not (or (`self.isInLowGrass`) (`self.isInLowGrass_1`) (`self.isInLowGrass_2`) (`self.isInLowGrass_3`) (`self.isInLowGrass_4`) (`self.isInLowGrass_5`) (`self.isInLowGrass_6`) (`self.isInLowGrass_7`) (`self.isInLowGrass_8`) (`self.isInLowGrass_9`) (`self.isInLowGrass_10`) (`self.isInLowGrass_11`) (`self.isInLowGrass_12`)))
    (goto _label_6)))

(event `self.WindForest_Box.OnComponentBeginOverlap`
  (params (OverlappedComponent :type "PrimitiveComponent Object Reference") (OtherActor :type "Actor Object Reference") (OtherComp :type "PrimitiveComponent Object Reference") (OtherBodyIndex :type Integer) (bFromSweep :type Boolean) (SweepResult :type "HitResult Structure (by ref)"))
  ;[1 1 1] ACTIVATION DU VENT DE FORET ET DESACTIVATION DU VENT GENERAL QUAND ON RENTRE DANS LA FORET
  (set `self.isInForest` true)
  (if (not (or (`self.isInForest_0`) (`self.isInForest_1`)))
    (bind (_direction _windvolume _windforestvolume) (`Timeline|TransitionToForest` :!label _label_7)
      (:`Update`
        (`AudioComponent.SetVolumeMultiplier` (`self.WindForest_SoundCue`) _windforestvolume)
        (`AudioComponent.SetVolumeMultiplier` (`self.Wind_SoundCue`) _windvolume)))))

(event `self.LowGrass_Detection2.OnComponentEndOverlap`
  (params (OverlappedComponent :type "PrimitiveComponent Object Reference") (OtherActor :type "Actor Object Reference") (OtherComp :type "PrimitiveComponent Object Reference") (OtherBodyIndex :type Integer))
  ;[1 1 1] ACTIVATION DES BRUITS DE CRICKETS ET DU VENT DHERBE HAUTE + DIMINUTION DU VOLUME DU VENT GENERAL
  (set `self.isInLowGrass_1` false)
  (if (not (or (`self.isInLowGrass`) (`self.isInLowGrass_0`) (`self.isInLowGrass_2`) (`self.isInLowGrass_3`) (`self.isInLowGrass_4`) (`self.isInLowGrass_5`) (`self.isInLowGrass_6`) (`self.isInLowGrass_7`) (`self.isInLowGrass_8`) (`self.isInLowGrass_9`) (`self.isInLowGrass_10`) (`self.isInLowGrass_11`) (`self.isInLowGrass_12`)))
    (goto _label_6)))

(event `self.WindForest_Box1.OnComponentBeginOverlap`
  (params (OverlappedComponent :type "PrimitiveComponent Object Reference") (OtherActor :type "Actor Object Reference") (OtherComp :type "PrimitiveComponent Object Reference") (OtherBodyIndex :type Integer) (bFromSweep :type Boolean) (SweepResult :type "HitResult Structure (by ref)"))
  ;[1 1 1] ACTIVATION DU VENT DE FORET ET DESACTIVATION DU VENT GENERAL QUAND ON RENTRE DANS LA FORET
  (set `self.isInForest_0` true)
  (if (not (or (`self.isInForest`) (`self.isInForest_1`)))
    (goto _label_7)))

(event `self.LowGrass_Detection3.OnComponentEndOverlap`
  (params (OverlappedComponent :type "PrimitiveComponent Object Reference") (OtherActor :type "Actor Object Reference") (OtherComp :type "PrimitiveComponent Object Reference") (OtherBodyIndex :type Integer))
  ;[1 1 1] ACTIVATION DES BRUITS DE CRICKETS ET DU VENT DHERBE HAUTE + DIMINUTION DU VOLUME DU VENT GENERAL
  (set `self.isInLowGrass_2` false)
  (if (not (or (`self.isInLowGrass`) (`self.isInLowGrass_0`) (`self.isInLowGrass_1`) (`self.isInLowGrass_3`) (`self.isInLowGrass_4`) (`self.isInLowGrass_5`) (`self.isInLowGrass_6`) (`self.isInLowGrass_7`) (`self.isInLowGrass_8`) (`self.isInLowGrass_9`) (`self.isInLowGrass_10`) (`self.isInLowGrass_11`) (`self.isInLowGrass_12`)))
    (goto _label_6)))

(event `self.WindForest_Box2.OnComponentBeginOverlap`
  (params (OverlappedComponent :type "PrimitiveComponent Object Reference") (OtherActor :type "Actor Object Reference") (OtherComp :type "PrimitiveComponent Object Reference") (OtherBodyIndex :type Integer) (bFromSweep :type Boolean) (SweepResult :type "HitResult Structure (by ref)"))
  ;[1 1 1] ACTIVATION DU VENT DE FORET ET DESACTIVATION DU VENT GENERAL QUAND ON RENTRE DANS LA FORET
  (set `self.isInForest_1` true)
  (if (not (or (`self.isInForest`) (`self.isInForest_0`)))
    (goto _label_7)))

(event `self.LowGrass_Detection4.OnComponentEndOverlap`
  (params (OverlappedComponent :type "PrimitiveComponent Object Reference") (OtherActor :type "Actor Object Reference") (OtherComp :type "PrimitiveComponent Object Reference") (OtherBodyIndex :type Integer))
  ;[1 1 1] ACTIVATION DES BRUITS DE CRICKETS ET DU VENT DHERBE HAUTE + DIMINUTION DU VOLUME DU VENT GENERAL
  (set `self.isInLowGrass_3` false)
  (if (not (or (`self.isInLowGrass`) (`self.isInLowGrass_0`) (`self.isInLowGrass_1`) (`self.isInLowGrass_2`) (`self.isInLowGrass_4`) (`self.isInLowGrass_5`) (`self.isInLowGrass_6`) (`self.isInLowGrass_7`) (`self.isInLowGrass_8`) (`self.isInLowGrass_9`) (`self.isInLowGrass_10`) (`self.isInLowGrass_11`) (`self.isInLowGrass_12`)))
    (goto _label_6)))

(event `self.LowGrass_Detection5.OnComponentEndOverlap`
  (params (OverlappedComponent :type "PrimitiveComponent Object Reference") (OtherActor :type "Actor Object Reference") (OtherComp :type "PrimitiveComponent Object Reference") (OtherBodyIndex :type Integer))
  ;[1 1 1] ACTIVATION DES BRUITS DE CRICKETS ET DU VENT DHERBE HAUTE + DIMINUTION DU VOLUME DU VENT GENERAL
  (set `self.isInLowGrass_4` false)
  (if (not (or (`self.isInLowGrass`) (`self.isInLowGrass_0`) (`self.isInLowGrass_1`) (`self.isInLowGrass_2`) (`self.isInLowGrass_3`) (`self.isInLowGrass_5`) (`self.isInLowGrass_6`) (`self.isInLowGrass_7`) (`self.isInLowGrass_8`) (`self.isInLowGrass_9`) (`self.isInLowGrass_10`) (`self.isInLowGrass_11`) (`self.isInLowGrass_12`)))
    (goto _label_6)))

(event `self.WindForest_Box.OnComponentEndOverlap`
  (params (OverlappedComponent :type "PrimitiveComponent Object Reference") (OtherActor :type "Actor Object Reference") (OtherComp :type "PrimitiveComponent Object Reference") (OtherBodyIndex :type Integer))
  ;[1 1 1] ACTIVATION DU VENT DE FORET ET DESACTIVATION DU VENT GENERAL QUAND ON RENTRE DANS LA FORET
  (set `self.isInForest` false)
  (if (not (or (`self.isInForest_0`) (`self.isInForest_1`)))
    (goto _label_7 :!via `Reverse`)))

(event `self.LowGrass_Detection6.OnComponentEndOverlap`
  (params (OverlappedComponent :type "PrimitiveComponent Object Reference") (OtherActor :type "Actor Object Reference") (OtherComp :type "PrimitiveComponent Object Reference") (OtherBodyIndex :type Integer))
  ;[1 1 1] ACTIVATION DES BRUITS DE CRICKETS ET DU VENT DHERBE HAUTE + DIMINUTION DU VOLUME DU VENT GENERAL
  (set `self.isInLowGrass_5` false)
  (if (not (or (`self.isInLowGrass`) (`self.isInLowGrass_0`) (`self.isInLowGrass_1`) (`self.isInLowGrass_2`) (`self.isInLowGrass_3`) (`self.isInLowGrass_4`) (`self.isInLowGrass_6`) (`self.isInLowGrass_7`) (`self.isInLowGrass_8`) (`self.isInLowGrass_9`) (`self.isInLowGrass_10`) (`self.isInLowGrass_11`) (`self.isInLowGrass_12`)))
    (goto _label_6)))

(event `self.WindForest_Box1.OnComponentEndOverlap`
  (params (OverlappedComponent :type "PrimitiveComponent Object Reference") (OtherActor :type "Actor Object Reference") (OtherComp :type "PrimitiveComponent Object Reference") (OtherBodyIndex :type Integer))
  ;[1 1 1] ACTIVATION DU VENT DE FORET ET DESACTIVATION DU VENT GENERAL QUAND ON RENTRE DANS LA FORET
  (set `self.isInForest_0` false)
  (if (not (or (`self.isInForest`) (`self.isInForest_1`)))
    (goto _label_7 :!via `Reverse`)))

(event `self.LowGrass_Detection7.OnComponentEndOverlap`
  (params (OverlappedComponent :type "PrimitiveComponent Object Reference") (OtherActor :type "Actor Object Reference") (OtherComp :type "PrimitiveComponent Object Reference") (OtherBodyIndex :type Integer))
  ;[1 1 1] ACTIVATION DES BRUITS DE CRICKETS ET DU VENT DHERBE HAUTE + DIMINUTION DU VOLUME DU VENT GENERAL
  (set `self.isInLowGrass_6` false)
  (if (not (or (`self.isInLowGrass`) (`self.isInLowGrass_0`) (`self.isInLowGrass_1`) (`self.isInLowGrass_2`) (`self.isInLowGrass_3`) (`self.isInLowGrass_4`) (`self.isInLowGrass_5`) (`self.isInLowGrass_7`) (`self.isInLowGrass_8`) (`self.isInLowGrass_9`) (`self.isInLowGrass_10`) (`self.isInLowGrass_11`) (`self.isInLowGrass_12`)))
    (goto _label_6)))

(event `self.WindForest_Box2.OnComponentEndOverlap`
  (params (OverlappedComponent :type "PrimitiveComponent Object Reference") (OtherActor :type "Actor Object Reference") (OtherComp :type "PrimitiveComponent Object Reference") (OtherBodyIndex :type Integer))
  ;[1 1 1] ACTIVATION DU VENT DE FORET ET DESACTIVATION DU VENT GENERAL QUAND ON RENTRE DANS LA FORET
  (set `self.isInForest_1` false)
  (if (not (or (`self.isInForest`) (`self.isInForest_0`)))
    (goto _label_7 :!via `Reverse`)))

(event `self.LowGrass_Detection8.OnComponentEndOverlap`
  (params (OverlappedComponent :type "PrimitiveComponent Object Reference") (OtherActor :type "Actor Object Reference") (OtherComp :type "PrimitiveComponent Object Reference") (OtherBodyIndex :type Integer))
  ;[1 1 1] ACTIVATION DES BRUITS DE CRICKETS ET DU VENT DHERBE HAUTE + DIMINUTION DU VOLUME DU VENT GENERAL
  (set `self.isInLowGrass_7` false)
  (if (not (or (`self.isInLowGrass`) (`self.isInLowGrass_0`) (`self.isInLowGrass_1`) (`self.isInLowGrass_2`) (`self.isInLowGrass_3`) (`self.isInLowGrass_4`) (`self.isInLowGrass_5`) (`self.isInLowGrass_6`) (`self.isInLowGrass_8`) (`self.isInLowGrass_9`) (`self.isInLowGrass_10`) (`self.isInLowGrass_11`) (`self.isInLowGrass_12`)))
    (goto _label_6)))

(event `self.LowGrass_Detection9.OnComponentEndOverlap`
  (params (OverlappedComponent :type "PrimitiveComponent Object Reference") (OtherActor :type "Actor Object Reference") (OtherComp :type "PrimitiveComponent Object Reference") (OtherBodyIndex :type Integer))
  ;[1 1 1] ACTIVATION DES BRUITS DE CRICKETS ET DU VENT DHERBE HAUTE + DIMINUTION DU VOLUME DU VENT GENERAL
  (set `self.isInLowGrass_8` false)
  (if (not (or (`self.isInLowGrass`) (`self.isInLowGrass_0`) (`self.isInLowGrass_1`) (`self.isInLowGrass_2`) (`self.isInLowGrass_3`) (`self.isInLowGrass_4`) (`self.isInLowGrass_5`) (`self.isInLowGrass_6`) (`self.isInLowGrass_7`) (`self.isInLowGrass_9`) (`self.isInLowGrass_10`) (`self.isInLowGrass_11`) (`self.isInLowGrass_12`)))
    (goto _label_6)))

(event `self.LowGrass_Detection10.OnComponentEndOverlap`
  (params (OverlappedComponent :type "PrimitiveComponent Object Reference") (OtherActor :type "Actor Object Reference") (OtherComp :type "PrimitiveComponent Object Reference") (OtherBodyIndex :type Integer))
  ;[1 1 1] ACTIVATION DES BRUITS DE CRICKETS ET DU VENT DHERBE HAUTE + DIMINUTION DU VOLUME DU VENT GENERAL
  (set `self.isInLowGrass_9` false)
  (if (not (or (`self.isInLowGrass`) (`self.isInLowGrass_0`) (`self.isInLowGrass_1`) (`self.isInLowGrass_2`) (`self.isInLowGrass_3`) (`self.isInLowGrass_4`) (`self.isInLowGrass_5`) (`self.isInLowGrass_6`) (`self.isInLowGrass_7`) (`self.isInLowGrass_8`) (`self.isInLowGrass_10`) (`self.isInLowGrass_11`) (`self.isInLowGrass_12`)))
    (goto _label_6)))

(event `self.LowGrass_Detection11.OnComponentEndOverlap`
  (params (OverlappedComponent :type "PrimitiveComponent Object Reference") (OtherActor :type "Actor Object Reference") (OtherComp :type "PrimitiveComponent Object Reference") (OtherBodyIndex :type Integer))
  ;[1 1 1] ACTIVATION DES BRUITS DE CRICKETS ET DU VENT DHERBE HAUTE + DIMINUTION DU VOLUME DU VENT GENERAL
  (set `self.isInLowGrass_10` false)
  (if (not (or (`self.isInLowGrass`) (`self.isInLowGrass_0`) (`self.isInLowGrass_1`) (`self.isInLowGrass_2`) (`self.isInLowGrass_3`) (`self.isInLowGrass_4`) (`self.isInLowGrass_5`) (`self.isInLowGrass_6`) (`self.isInLowGrass_7`) (`self.isInLowGrass_8`) (`self.isInLowGrass_9`) (`self.isInLowGrass_11`) (`self.isInLowGrass_12`)))
    (goto _label_6)))

(event `self.LowGrass_Detection12.OnComponentEndOverlap`
  (params (OverlappedComponent :type "PrimitiveComponent Object Reference") (OtherActor :type "Actor Object Reference") (OtherComp :type "PrimitiveComponent Object Reference") (OtherBodyIndex :type Integer))
  ;[1 1 1] ACTIVATION DES BRUITS DE CRICKETS ET DU VENT DHERBE HAUTE + DIMINUTION DU VOLUME DU VENT GENERAL
  (set `self.isInLowGrass_11` false)
  (if (not (or (`self.isInLowGrass`) (`self.isInLowGrass_0`) (`self.isInLowGrass_1`) (`self.isInLowGrass_2`) (`self.isInLowGrass_3`) (`self.isInLowGrass_4`) (`self.isInLowGrass_5`) (`self.isInLowGrass_6`) (`self.isInLowGrass_7`) (`self.isInLowGrass_8`) (`self.isInLowGrass_9`) (`self.isInLowGrass_10`) (`self.isInLowGrass_12`)))
    (goto _label_6)))

(event `self.LowGrass_Detection13.OnComponentEndOverlap`
  (params (OverlappedComponent :type "PrimitiveComponent Object Reference") (OtherActor :type "Actor Object Reference") (OtherComp :type "PrimitiveComponent Object Reference") (OtherBodyIndex :type Integer))
  ;[1 1 1] ACTIVATION DES BRUITS DE CRICKETS ET DU VENT DHERBE HAUTE + DIMINUTION DU VOLUME DU VENT GENERAL
  (set `self.isInLowGrass_12` false)
  (if (not (or (`self.isInLowGrass`) (`self.isInLowGrass_0`) (`self.isInLowGrass_1`) (`self.isInLowGrass_2`) (`self.isInLowGrass_3`) (`self.isInLowGrass_4`) (`self.isInLowGrass_5`) (`self.isInLowGrass_6`) (`self.isInLowGrass_7`) (`self.isInLowGrass_8`) (`self.isInLowGrass_9`) (`self.isInLowGrass_10`) (`self.isInLowGrass_11`)))
    (goto _label_6)))

(fn `UserConstructionScript`)