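; Lobby room character actor that displays a player's saved customisation and a player info widget.
; UsePlayerCustomisation, run at BeginPlay and on Custo replication, sets meshes for hair, facial hair and accessories, plus eyelash visibility and suit material.
; Hair and skin colour go through Material Parameter Collections, so they are global rather than per character.
; MC_NETID takes the Net ID from a PlayerState and refreshes the widget; its customisation wiring never runs.
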(event `self.ReceiveBeginPlay`
  (bind _widget (`self.Widget`))
  (bind _netid (`self.NetID`))
  (bind _asgs_lobby (cast `/Game/_Jam_MilkyWay/Players/MenuPlayer/GS_Lobby` (`GameplayStatics.GetGameState`)))
  (set `self.As GS Lobby` _asgs_lobby)
  (`self.UsePlayerCustomisation` (`self.Custo`))
  (`/Engine/EditorBlueprintResources/ActorMacros.Switch Has Authority`
    (:`Authority`
      (bind _asw_player_info_on_server (cast `/Game/_Jam_MilkyWay/Players/MenuPlayer/W_PlayerInfo_onServer` (`WidgetComponent.GetWidget` _widget)))
      (bind _output_get (set `self.As W Player Info on Server` _asw_player_info_on_server))
      (`/Game/_Jam_MilkyWay/Players/MenuPlayer/W_PlayerInfo_onServer.UpdatePlayerData` _output_get _netid))
    (:`Remote`
      (bind _asw_player_info_on_server_2 (cast `/Game/_Jam_MilkyWay/Players/MenuPlayer/W_PlayerInfo_onServer` (`WidgetComponent.GetUserWidgetObject` _widget)))
      (bind _output_get_2 (set `self.As W Player Info on Server` _asw_player_info_on_server_2))
      (`/Game/_Jam_MilkyWay/Players/MenuPlayer/W_PlayerInfo_onServer.UpdatePlayerData` _output_get_2 _netid)))
  (`KismetSystemLibrary.PrintString` (`AdvancedIdentityLibrary.GetPlayerNickname` _netid)))

(event `MC_NETID`
  (params (UniqueNetId :type "BPUniqueNetId Structure") (PlayerState :type "PlayerState Object Reference") (PlayerCustomisation :type "/Game/_Jam_MilkyWay/Players/SaveGame/S_Customization Structure") (MYPC :type "/Game/_Jam_MilkyWay/Players/MenuPlayer/PC_Lobby Object Reference"))
  (bind _uniquenetid (`AdvancedSessionsLibrary.GetUniqueNetIDFromPlayerState` PlayerState))
  (bind _output_get (set `self.NetID` _uniquenetid))
  (`/Game/_Jam_MilkyWay/Players/MenuPlayer/W_PlayerInfo_onServer.UpdatePlayerData` (`self.As W Player Info on Server`) _output_get)
  (`KismetSystemLibrary.PrintString` (`AdvancedIdentityLibrary.GetPlayerNickname` _uniquenetid)))

(fn `AccessoriesSelector`
  (params (Selector :type Integer))
  (bind _output_get (set `self.AccessoriesIndex` Selector))
  (`StaticMeshComponent.SetStaticMesh` (`self.accessories`) (`|GetArrayItem` (`self.AccessoriesArray`) _output_get)))

(fn `BodyAccessoriesSelector`
  (params (Selector :type Integer))
  (bind _output_get (set `self.BodyAccessoriesIndex` Selector))
  (`StaticMeshComponent.SetStaticMesh` (`self.bodyaccessories`) (`|GetArrayItem` (`self.BodyAccessoriesArray`) _output_get)))

(fn `Eyelashes On Off`
  (params (EyelashesVisible :type Boolean))
  (if EyelashesVisible
    (`SceneComponent.SetVisibility` (`self.eyelashes`) true false)
    (else
      (`SceneComponent.SetVisibility` (`self.eyelashes`) false false))))

(fn `FacialHairSelector`
  (params (Selector :type Integer))
  (bind _output_get (set `self.FacialHairIndex` Selector))
  (`StaticMeshComponent.SetStaticMesh` (`self.facialhair`) (`|GetArrayItem` (`self.FacialHairArray`) _output_get)))

(fn `HaircutSelector`
  (params (Selector :type Integer))
  (bind _output_get (set `self.HairIndex` Selector))
  (`StaticMeshComponent.SetStaticMesh` (`self.Hair`) (`|GetArrayItem` (`self.Haircut`) _output_get)))

(fn `OnRep_Custo`
  (`self.UsePlayerCustomisation` (`self.Custo`)))

(fn `Suit`
  (params (Selector :type Integer))
  (bind _output_get (set `self.SuitIndex` Selector))
  (`PrimitiveComponent.SetMaterial` (`self.SkeletalMesh`) 0 (`|GetArrayItem` (`self.SuitArray`) _output_get)))

(fn `UsePlayerCustomisation`
  (params (PlayerCustomisation :type "/Game/_Jam_MilkyWay/Players/SaveGame/S_Customization Structure"))
  (bind _output_get (set `self.AccessoriesIndex` PlayerCustomisation_AccessoriesIndex_Save_8_78068BD8412C091746A5A6BE22CBABBC))
  (bind _output_get_2 (set `self.BodyAccessoriesIndex` PlayerCustomisation_BodyAccessoriesIndex_Save_12_3E88A9F64C83A9B046749F896E206D53))
  (`SceneComponent.SetVisibility` (`self.eyelashes`) PlayerCustomisation_Eyelashes_Save_17_C20BB610490B3413D8B4919F8DD6097B false)
  (bind _output_get_3 (set `self.FacialHairIndex` PlayerCustomisation_FacialHairIndex_Save_10_893C65614233133BE784ACB40DC3643B))
  (bind _output_get_4 (set `self.HairColor` PlayerCustomisation_HairColor_Save_5_944425D34656DB70729D62968283599C))
  (bind _output_get_5 (set `self.HairIndex` PlayerCustomisation_HairIndex_Save_2_99E3DC4B426ABFB81B8B84B619251337))
  (bind _output_get_6 (set `self.SkinColor` PlayerCustomisation_SkinColor_Save_20_2B55B45242FA855FF5B7848464A372A3))
  (bind _output_get_7 (set `self.SuitIndex` PlayerCustomisation_SuitIndex_Save_14_3FFFA55142249704F511228CFDC1E1FA))
  (`self.AccessoriesSelector` _output_get)
  (`self.BodyAccessoriesSelector` _output_get_2)
  (`self.Eyelashes On Off` PlayerCustomisation_Eyelashes_Save_17_C20BB610490B3413D8B4919F8DD6097B)
  (`self.FacialHairSelector` _output_get_3)
  (`KismetMaterialLibrary.SetScalarParameterValue` "/Game/_Jam_MilkyWay/Characters/Manz/Haircuts/MM_HairColor.MM_HairColor" "Scalar" _output_get_4)
  (`self.HaircutSelector` _output_get_5)
  (`KismetMaterialLibrary.SetScalarParameterValue` "/Game/_Jam_MilkyWay/Materials/MPC_SkinIndex.MPC_SkinIndex" "SkinIndex" _output_get_6)
  (`self.Suit` _output_get_7))

(fn `UserConstructionScript`)