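; Lobby room environment actor that stages the menu lobby and spawns the players' customized Manz characters.
; On BeginPlay it caches four placeholder Manz transforms and registers itself with GS_Lobby.
; Clients loop the lobby level sequence and poll on Tick to stop it once the GameState reports the game is ready.
; RPC_Spawn creates a BP_MANZLOBBYROOM on the server with customization and NetID, then adds it to the GameState's bank.
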(event `self.ReceiveBeginPlay`
  (`self.SetManzBank`)
  (bind _asgs_lobby (cast `/Game/_Jam_MilkyWay/Players/MenuPlayer/GS_Lobby` (`GameplayStatics.GetGameState`)))
  (bind _output_get (set `self.As GS Lobby` _asgs_lobby))
  (set `/Game/_Jam_MilkyWay/Players/MenuPlayer/GS_Lobby.LobbyRoomRef` self _output_get)
  (`/Engine/EditorBlueprintResources/ActorMacros.Switch Has Authority`
    (:`Remote`
      (bind (_outactor _returnvalue) (`LevelSequencePlayer.CreateLevelSequencePlayer` "/Game/_Jam_MilkyWay/Sequences/LobbySequence.LobbySequence"))
      (bind _output_get_2 (set `self.LobbySequence` _returnvalue))
      (`MovieSceneSequencePlayer.PlayLooping` _output_get_2 -1))))

(event `STOP SEQUENCE`
  (`MovieSceneSequencePlayer.Stop` (`self.LobbySequence`)))

(event `self.ReceiveTick`
  (params (DeltaSeconds :type "Float (single-precision)"))
  (`/Engine/EditorBlueprintResources/ActorMacros.Switch Has Authority`
    (:`Remote`
      (bind _as_gs_lobby (`self.As GS Lobby`)
        (:`then`
          (if (`/Game/_Jam_MilkyWay/Players/MenuPlayer/GS_Lobby.Game is Ready` _as_gs_lobby)
            (`MovieSceneSequencePlayer.Stop` (`self.LobbySequence`))))
        (:`else`)))))

(event `RPC_Spawn`
  (params (SpawnTransform :type "Transform Structure") (Custo :type "/Game/_Jam_MilkyWay/Players/SaveGame/S_Customization Structure") (NetID :type "BPUniqueNetId Structure"))
  (`/Engine/EditorBlueprintResources/ActorMacros.Switch Has Authority`
    (:`Authority`
      (bind _returnvalue (`|SpawnActorFromClass` :`Class` "/Game/_Jam_MilkyWay/Environment/Menu/BP_MANZLOBBYROOM.BP_MANZLOBBYROOM_C" :`SpawnTransform` SpawnTransform :`CollisionHandlingOverride` "Undefined" :`TransformScaleMethod` "MultiplyWithRoot" :`Custo` Custo :`NetID` NetID :`MyPC` null :`MyPlayerState` null :`Instigator` null))
      (`KismetArrayLibrary.Array_AddUnique` (`/Game/_Jam_MilkyWay/Players/MenuPlayer/GS_Lobby.ManzLobbyBank` (`self.As GS Lobby`)) _returnvalue))))

(fn `SetManzBank`
  (bind _manzskmtransform (`self.ManzSKMTransform`))
  (`KismetArrayLibrary.Array_Add` _manzskmtransform (`SceneComponent.K2_GetComponentToWorld` (`self.Manz04`)))
  (`KismetArrayLibrary.Array_Add` _manzskmtransform (`SceneComponent.K2_GetComponentToWorld` (`self.Manz01`)))
  (`KismetArrayLibrary.Array_Add` _manzskmtransform (`SceneComponent.K2_GetComponentToWorld` (`self.Manz03`)))
  (`KismetArrayLibrary.Array_Add` _manzskmtransform (`SceneComponent.K2_GetComponentToWorld` (`self.Manz02`))))

(fn `UserConstructionScript`)