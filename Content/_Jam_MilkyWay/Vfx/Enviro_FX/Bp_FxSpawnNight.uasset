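; Environment FX Blueprint that randomly toggles Fireflies and a second Niagara effect based on Ultra Dynamic Sky and Weather events.
; Sunset calls DayIsComing, which may start Fireflies, and sunrise calls NightIsComing, which may start the other effect.
; Rain stops both effects.
; When rain ends, daytime reruns DayIsComing and nighttime NightIsComing, the reverse of the sunset/sunrise bindings.
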(event `self.ReceiveTick`
  (params (DeltaSeconds :type "Float (single-precision)")))

(event `self.ReceiveBeginPlay`
  (`ActorComponent.Deactivate` (`self.NiagaraComponent`))
  (bind _uds (`self.Get Ultra Dynamic Sky`))
  (add `self.Sunset` _uds (delegate `DayIsComing`))
  (add `self.Sunrise` _uds (delegate `NightIsComing`))
  (bind _udw (`self.Get Ultra Dynamic Weather`))
  (add `self.Started Raining` _udw (delegate `CustomEvent`))
  (add `self.Finished Raining` _udw (delegate `CustomEvent_0`)))

(event `DayIsComing`
  (if (not (`self.Raining`))
    (set `self.RandomSpawn` (`KismetMathLibrary.RandomInteger` 5))
    (if (<= (`self.RandomSpawn`) 1)
      (`ActorComponent.Activate` (`self.Fireflies`) false)
      (`ActorComponent.Deactivate` (`self.NiagaraComponent`))
      (else
        (`ActorComponent.Deactivate` (`self.NiagaraComponent`) :!label _label)
        (`ActorComponent.Deactivate` (`self.Fireflies`))))))

(event `NightIsComing`
  (if (not (`self.Raining`))
    (set `self.RandomSpawn` (`KismetMathLibrary.RandomInteger` 5))
    (if (<= (`self.RandomSpawn`) 2)
      (`ActorComponent.Activate` (`self.NiagaraComponent`) false)
      (`ActorComponent.Deactivate` (`self.Fireflies`))
      (else
        (goto _label)))))

(event `CustomEvent_0`
  (set `self.Raining` false)
  (if (`self.Is it Daytime?` (stale `self.ReceiveBeginPlay` _uds))
    (`self.DayIsComing`)
    (else
      (`self.NightIsComing`))))

(event `CustomEvent`
  (set `self.Raining` true)
  (`ActorComponent.Deactivate` (`self.NiagaraComponent`))
  (`ActorComponent.Deactivate` (`self.Fireflies`)))

(fn `UserConstructionScript`)