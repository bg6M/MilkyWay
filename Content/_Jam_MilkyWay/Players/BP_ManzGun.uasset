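; BP_ManzGun is a player gun Blueprint that switches a Niagara laser effect on and off.
; RepNotifies on Fire and LaserReplication both lead to LASERRPCEND, which activates or deactivates the effect from the Fire value.
; LaserFire ignores its OnOff input and only forwards to that event, and nothing in this file sets Fire.
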(event `LaserFire`
  (params (`On/Off` :type Boolean))
  (`self.LASER RPC END`))

(event `LASER RPC END`
  (bind _niagara (`self.Niagara`))
  (if (`self.Fire`)
    (`ActorComponent.Activate` _niagara true)
    (else
      (`ActorComponent.Deactivate` _niagara))))

(fn `OnRep_Fire`
  (`self.LaserFire` (`self.Fire`)))

(fn `OnRep_LaserReplication`
  (`self.LASER RPC END`))

(fn `UserConstructionScript`)