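; Placed barricade item that behaves as a jaw trap, with open, close and break sounds, and expires after a fixed lifetime.
; RPCOVERLAP accepts only players on the server, then triggers a timed sequence that plays sounds, clears the active and trigger flags, and destroys the actor.
; The OnRep functions have no effect; code to immobilize and snap the caught player to the trap is disconnected.
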(event `self.ReceiveBeginPlay`
  (bind _asgs_lobby (cast `/Game/_Jam_MilkyWay/Players/MenuPlayer/GS_Lobby` (`GameplayStatics.GetGameState`)))
  (set `self.As GS Lobby` _asgs_lobby)
  (set `self.IsActive` true)
  (`GameplayStatics.PlaySoundAtLocation` "/Game/_Jam_MilkyWay/SFX/Foleys/Items/JawTrap_Open_SFX.JawTrap_Open_SFX" (`self.K2_GetActorLocation`) (struct) 0.75 1.0 0.0 "/Game/_Jam_MilkyWay/SFX/Attenuation_Types/SA_Trap.SA_Trap" null null null)
  (`KismetSystemLibrary.Delay` 120.0)
  (`self.K2_DestroyActor`))

(event `RPC OVERLAP`
  (params (Object :type "Object Object Reference"))
  (`/Engine/EditorBlueprintResources/ActorMacros.Switch Has Authority`
    (:`Authority`
      (bind _asbp_player (cast `/Game/_Jam_MilkyWay/Players/FirstPerson/Blueprints/BP_Player` Object))
      (set `self.As BP Player` _asbp_player)
      (`self.RPC TRIGGER TRAP`))))

(event `RPC TRIGGER TRAP`
  (set `self.IsTrigger` true)
  (`self.MC_SoundTrigger`)
  (`KismetSystemLibrary.Delay` 5.5)
  (`self.MCSoundBreak`)
  (`KismetSystemLibrary.Delay` 0.5)
  (set `self.IsActive` false)
  (set `self.IsTrigger` false)
  (`KismetSystemLibrary.Delay` 2.0)
  (`self.K2_DestroyActor`))

(event `MCSoundBreak`
  (`GameplayStatics.PlaySoundAtLocation` "/Game/_Jam_MilkyWay/SFX/Foleys/Items/JawTrap_Destroyed_SFX.JawTrap_Destroyed_SFX" (`self.K2_GetActorLocation`) (struct) 0.75 1.0 0.0 "/Game/_Jam_MilkyWay/SFX/Attenuation_Types/SA_Trap.SA_Trap" null null null))

(event `MC_SoundTrigger`
  (`GameplayStatics.PlaySoundAtLocation` "/Game/_Jam_MilkyWay/SFX/Foleys/Items/JawTrap_Close_SFX.JawTrap_Close_SFX" (`self.K2_GetActorLocation`) (struct) 0.9 1.0 0.0 "/Game/_Jam_MilkyWay/SFX/Attenuation_Types/SA_Trap.SA_Trap" null null null))

(fn `OnRep_IsActive`)

(fn `OnRep_IsGrabed`
  (if (`self.IsGrabed`)
    _))

(fn `OnRep_IsTrigger`)

(fn `UserConstructionScript`)