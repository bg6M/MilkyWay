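; An active sound alarm trap item that sounds an alarm when a GREEZ-team player enters its sphere.
; Overlap events route through RPC events to set IsTrigger, whose OnRep plays or stops the alarm audio.
; When the tracked player leaves, the alarm stops after a short delay unless they have re-entered.
; The trap destroys itself after five minutes with a pouf effect and sound.
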(event `self.ReceiveBeginPlay`
  (bind _returnvalue (`self.K2_GetActorLocation`))
  (bind _asbp_game_instance (cast `/Game/_Jam_MilkyWay/Players/FirstPerson/Blueprints/BP_GameInstance` (`GameplayStatics.GetGameInstance`)))
  (set `self.As BP Game Instance` _asbp_game_instance)
  (bind _asgs_lobby (cast `/Game/_Jam_MilkyWay/Players/MenuPlayer/GS_Lobby` (`GameplayStatics.GetGameState`))
    (:`then`
      (set `self.As GS Lobby` _asgs_lobby))
    (:`CastFailed`
      _))
  (set `self.IsActive` true)
  (`KismetSystemLibrary.Delay` 300.0)
  (`NiagaraFunctionLibrary.SpawnSystemAtLocation` "/Game/_Jam_MilkyWay/Vfx/FX_Pouf.FX_Pouf" _returnvalue)
  (`GameplayStatics.SpawnSoundAtLocation` "/Game/_Jam_MilkyWay/SFX/Foleys/Pouf_SFX.Pouf_SFX" _returnvalue (struct) 1.0 1.0 0.0 "/Game/_Jam_MilkyWay/SFX/SA_VoiceChat.SA_VoiceChat" null)
  (`self.K2_DestroyActor`))

(event `self.Sphere.OnComponentBeginOverlap`
  (params (OverlappedComponent :type "PrimitiveComponent Object Reference") (OtherActor :type "Actor Object Reference") (OtherComp :type "PrimitiveComponent Object Reference") (OtherBodyIndex :type Integer) (bFromSweep :type Boolean) (SweepResult :type "HitResult Structure (by ref)"))
  (if (`self.IsActive`)
    (`self.RPC OVERLAP` OtherActor)))

(event `RPC OVERLAP`
  (params (Object :type "Object Object Reference"))
  (bind _asbp_player (cast `/Game/_Jam_MilkyWay/Players/FirstPerson/Blueprints/BP_Player` Object))
  (bind _output_get (set `self.As BP Player` _asbp_player))
  (switch `/Game/_Jam_MilkyWay/Players/MenuPlayer/E_PlayersTeam` (`/Game/_Jam_MilkyWay/Players/FirstPerson/Blueprints/BP_Player.Team` _output_get)
    (:`NewEnumerator1`
      (`self.RPC TRIGGER TRAP` true))))

(event `RPC TRIGGER TRAP`
  (params (IsTrigger :type Boolean))
  (set `self.IsTrigger` IsTrigger))

(event `self.Sphere.OnComponentEndOverlap`
  (params (OverlappedComponent :type "PrimitiveComponent Object Reference") (OtherActor :type "Actor Object Reference") (OtherComp :type "PrimitiveComponent Object Reference") (OtherBodyIndex :type Integer))
  (if (`self.IsActive`)
    (`self.RPC_ENDOVERLAP` OtherActor)))

(event `RPC_ENDOVERLAP`
  (params (Actor :type "Actor Object Reference"))
  (bind _as_bp_player (`self.As BP Player`))
  (if (== Actor _as_bp_player)
    (`KismetSystemLibrary.Delay` 3.0)
    (if (not (`self.IsOverlappingActor` _as_bp_player self))
      (`self.RPC TRIGGER TRAP` false))))

(fn `OnRep_IsActive`)

(fn `OnRep_IsGrabed`)

(fn `OnRep_IsTrigger`
  (bind _alamrcue (`self.AlamrCUE`))
  (if (`self.IsTrigger`)
    (if (not (`AudioComponent.IsPlaying` _alamrcue))
      (`AudioComponent.Play` _alamrcue 0.0))
    (else
      (`AudioComponent.Stop` _alamrcue))))

(fn `UserConstructionScript`)