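; BP_Trap is a trap item that players can pick up and drop through a grab interface while it is not active.
; Grab and ungrab pass through server RPC events that attach the skeletal mesh to the player's grab point or detach it, toggling physics and collision.
; Release adds the player's movement velocity as an impulse.
; Trigger behavior is absent here, and the active, trigger and grabbed RepNotifies are empty.
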(event Custom|RPC%20GRAB
  (params (Target :type BP%20Player%20Object%20Reference))
  (bind _skeletalmesh (Variables|Default|GetSkeletalMesh))
  (Transformation|AttachComponentToComponent (Variables|/Game/_Jam_MilkyWay/Players/FirstPerson/Blueprints/BP_Player.BP_Player_C|GetManz_Grab_Fps_Location Target) "None" "SnapToTarget" "SnapToTarget" "KeepWorld" false)
  (Transformation|SetWorldRotation _skeletalmesh (Pawn|GetControlRotation Target :!class /Script/Engine.Pawn) false false)
  (Physics|SetSimulatePhysics _skeletalmesh false)
  (Variables|Default|SetIsGrabed true)
  (Collision|SetCollisionEnabled _skeletalmesh "PhysicsOnly"))

(event Custom|RPC%20UNGRAB
  (bind _skeletalmesh (Variables|Default|GetSkeletalMesh))
  (Variables|Default|SetIsGrabed false)
  (Physics|SetSimulatePhysics _skeletalmesh true)
  (Transformation|DetachFromActor "KeepWorld" "KeepWorld" "KeepRelative")
  (Physics|AddImpulse (Variables|Default|GetSkeletalMesh) (* (Pawn|Components|CharacterMovement|GetLastUpdateVelocity (Variables|/Script/Engine.Character|GetCharacterMovement (Variables|Default|GetPlayer%20Calling%20Grab))) 1.0) "None" true)
  (Collision|SetCollisionEnabled _skeletalmesh "QueryAndPhysics")
  (Variables|Default|SetPlayer%20Calling%20Grab 0))

(event Custom|ServerRPCGRAB
  (params (Player%20Calling%20Grab :type BP%20Player%20Object%20Reference))
  (CallFunction|RPCGRAB Player%20Calling%20Grab))

(event Custom|SERVER%20RPC%20UNGRAB
  (CallFunction|RPCUNGRAB))

(event EventBeginPlay
  (bind _asbp_game_instance (Utilities|Casting|CastToBP_GameInstance (Game|GetGameInstance)))
  (Variables|Default|SetAs%20BP%20Game%20Instance _asbp_game_instance)
  (bind _asgs_lobby (Utilities|Casting|CastToGS_Lobby (Game|GetGameState)))
  (Variables|Default|SetAs%20GS%20Lobby _asgs_lobby))

(event EventGrabInterface
  (params (Player%20calling%20grab :type BP%20Player%20Object%20Reference))
  (if (not (Variables|Default|GetIsActive))
    (bind _output_get (Variables|Default|SetPlayer%20Calling%20Grab Player%20calling%20grab))
    (CallFunction|ServerRPCGRAB _output_get)))

(event EventUnGrabInterface
  (CallFunction|SERVERRPCUNGRAB))

(fn ConstructionScript)

(fn OnRepIsGrabed)

(fn OnRepIsActive)

(fn OnRepIsTrigger)