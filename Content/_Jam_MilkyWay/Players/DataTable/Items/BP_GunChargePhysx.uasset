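; Grabbable physics pickup named as a gun charge, whose interaction is a placeholder that only prints "BUFF SOON" through the SpawnTrap RepNotify.
; Grab and ungrab route through server RPC events that toggle collision and set IsGrabed, whose RepNotify switches physics simulation; grabbing also aligns the mesh to the grabber's control rotation.
; Disconnected trap logic, which would trace to ground, spawn an active trap with Niagara burst and destroy the item, never runs.
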(event Custom|RPC%20GRAB
  (params (Target :type BP%20Player%20Object%20Reference))
  (bind _trapsm (Variables|Default|GetTrapSM))
  (Transformation|SetWorldRotation _trapsm (Pawn|GetControlRotation Target :!class /Script/Engine.Pawn) false false)
  (Variables|Default|SetIsGrabed true)
  (Collision|SetCollisionEnabled _trapsm "PhysicsOnly"))

(event Custom|RPC%20UNGRAB
  (Variables|Default|SetIsGrabed false)
  (Collision|SetCollisionEnabled (Variables|Default|GetTrapSM) "QueryAndPhysics")
  (Variables|Default|SetPlayer%20Calling%20Grab 0))

(event Custom|ServerRPCGRAB
  (params (Player%20Calling%20Grab :type BP%20Player%20Object%20Reference))
  (CallFunction|RPCGRAB Player%20Calling%20Grab))

(event Custom|SERVER%20RPC%20UNGRAB
  (CallFunction|RPCUNGRAB))

(event Custom|RPC%20SPAWN%20TRAP
  (Development|PrintString "BUFF SOON"))

(event EventBeginPlay
  (bind _asbp_game_instance (Utilities|Casting|CastToBP_GameInstance (Game|GetGameInstance)))
  (Variables|Default|SetAs%20BP%20Game%20Instance _asbp_game_instance)
  (bind _asgs_lobby (Utilities|Casting|CastToGS_Lobby (Game|GetGameState)))
  (Variables|Default|SetAs%20GS%20Lobby _asgs_lobby))

(event EventGrabInterface
  (params (Player%20calling%20grab :type BP%20Player%20Object%20Reference) (PlayerTeam :type E_PlayersTeam%20Enum :default "NewEnumerator0"))
  (bind _output_get (Variables|Default|SetPlayer%20Calling%20Grab Player%20calling%20grab))
  (CallFunction|ServerRPCGRAB _output_get))

(event EventInteractInt
  (Variables|Default|SetSpawnTrap true))

(event EventUnGrabInterface
  (CallFunction|SERVERRPCUNGRAB))

(fn ConstructionScript)

(fn OnRepIsGrabed
  (bind _trapsm (Variables|Default|GetTrapSM))
  (if (Variables|Default|GetIsGrabed)
    (Physics|SetSimulatePhysics _trapsm false)
    (else
      (Physics|SetSimulatePhysics _trapsm true))))

(fn OnRepSpawnTrap
  (CallFunction|RPCSPAWNTRAP))