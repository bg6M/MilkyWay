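; Physics-driven jaw trap item that players can grab, release, bump with an impulse, or activate.
; Interacting sets SpawnTrap, whose RepNotify traces down to the ground, spawns an active BP_TrapActive with random yaw and destroys the item.
; Grab and release go through RPC events that set IsGrabed, whose RepNotify toggles physics and collision, while grabbing also adjusts team-specific spring arms.
; The "Activate" interaction widget is toggled only for MANZ players.
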(event Custom|RPC%20GRAB
  (params (Target :type BP%20Player%20Object%20Reference))
  (bind _trapsm (Variables|Default|GetTrapSM))
  (Transformation|SetWorldRotation _trapsm (Pawn|GetControlRotation Target :!class /Script/Engine.Pawn) false false)
  (Variables|Default|SetIsGrabed true)
  (Collision|SetCollisionEnabled _trapsm "PhysicsOnly")
  (switch Utilities|FlowControl|Switch|SwitchonE_PlayersTeam (Variables|/Game/_Jam_MilkyWay/Players/FirstPerson/Blueprints/BP_Player.BP_Player_C|GetTeam Target)
    (:NewEnumerator0
      (Variables|/Script/Engine.SpringArmComponent|SetTargetArmLength (Variables|/Game/_Jam_MilkyWay/Players/FirstPerson/Blueprints/BP_Player.BP_Player_C|GetManzGrabSpringArm Target) -4e+02))
    (:NewEnumerator1
      (Variables|/Script/Engine.SpringArmComponent|SetTargetArmLength (Variables|/Game/_Jam_MilkyWay/Players/FirstPerson/Blueprints/BP_Player.BP_Player_C|GetGrabSpringArm Target) -2e+02))))

(event Custom|RPC%20UNGRAB
  (Variables|Default|SetIsGrabed false)
  (Collision|SetCollisionEnabled (Variables|Default|GetTrapSM) "QueryAndPhysics")
  (Variables|Default|SetPlayer%20Calling%20Grab 0))

(event Custom|ServerRPCGRAB
  (params (Player%20Calling%20Grab :type BP%20Player%20Object%20Reference))
  (CallFunction|RPCGRAB Player%20Calling%20Grab))

(event Custom|SERVER%20RPC%20UNGRAB
  (CallFunction|RPCUNGRAB))

(event Custom|RPC%20SPAWN%20TRAP
  (bind _trapsm (Variables|Default|GetTrapSM))
  (bind _returnvalue (Transformation|GetWorldLocation _trapsm))
  (bind _outhit (Collision|LineTraceByChannel _returnvalue (- _returnvalue "0.000000,0.000000,1000.000000") "TraceTypeQuery1" false 0 "None"))
  (Variables|Default|SetSpawnLocation (.Location (Collision|BreakHitResult _outhit)))
  (bind _returnvalue_2 (Game|SpawnActorfromClass "/Game/_Jam_MilkyWay/Players/DataTable/Items/BP_TrapActive.BP_TrapActive_C" (Math|Transform|MakeTransform (Variables|Default|GetSpawnLocation) (Math|Rotator|MakeRotator 0.0 0.0 (Math|Random|RandomFloat))) "Undefined" "MultiplyWithRoot" 0 0))
  (Variables|/Game/_Jam_MilkyWay/Players/DataTable/Items/BP_TrapActive.BP_TrapActive_C|SetIsActive _returnvalue_2 true)
  (Actor|DestroyActor))

(event EventBeginPlay
  (bind _widget (Variables|Default|GetWidget))
  (bind _asbp_game_instance (Utilities|Casting|CastToBP_GameInstance (Game|GetGameInstance)))
  (Variables|Default|SetAs%20BP%20Game%20Instance _asbp_game_instance)
  (bind _asgs_lobby (Utilities|Casting|CastToGS_Lobby (Game|GetGameState)))
  (Variables|Default|SetAs%20GS%20Lobby _asgs_lobby)
  (Networking|SwitchHasAuthority
    (:Authority
      (bind _asw_interaction (Utilities|Casting|CastToW_Interaction (UserInterface|GetWidget _widget)))
      (Variables|Default|SetAs%20W%20Interaction _asw_interaction))
    (:Remote
      (bind _asw_interaction_2 (Utilities|Casting|CastToW_Interaction (UserInterface|GetUserWidgetObject _widget)))
      (Variables|Default|SetAs%20W%20Interaction _asw_interaction_2)))
  (Default|SetDATA (Variables|Default|GetAs%20W%20Interaction) "JAW TRAP      " "Activate" false)
  (Networking|SwitchHasAuthority
    (:Authority
      (Physics|SetSimulatePhysics (Variables|Default|GetTrapSM) true))))

(event EventToggleOutlineInteractible
  (params (Player%20Calling :type BP%20Player%20Object%20Reference))
  (Default|ACTIVATEOUTLINE Player%20Calling true (Variables|Default|GetSKM_Trap)))

(event EventBumpINT
  (params (PCCallingBump :type PC%20Lobby%20Object%20Reference))
  (Physics|SetSimulatePhysics (Variables|Default|GetTrapSM) true)
  (Physics|AddImpulse (Variables|Default|GetTrapSM) (* (Math|Vector|Normalize (Math|Vector|GetForwardVector (Pawn|GetControlRotation PCCallingBump :!class /Script/Engine.Controller))) 6e+02) "None" true))

(event EventInteractInt
  (params (Bp_Player :type BP%20Player%20Object%20Reference))
  (Variables|Default|SetSpawnTrap true))

(event EventGrabInterface
  (params (Player%20calling%20grab :type BP%20Player%20Object%20Reference) (PlayerTeam :type E_PlayersTeam%20Enum :default "NewEnumerator0"))
  (Networking|SwitchHasAuthority
    (:Authority
      (bind _output_get (Variables|Default|SetPlayer%20Calling%20Grab Player%20calling%20grab))
      (CallFunction|ServerRPCGRAB _output_get))))

(event EventUnGrabInterface
  (params (Player%20Calling%20Grab :type BP%20Player%20Object%20Reference) (Bump? :type Boolean) (ControllerCallingBump :type PC%20Lobby%20Object%20Reference))
  (CallFunction|SERVERRPCUNGRAB))

(event EventToggleWidget
  (params (On/Off :type Boolean) (PlayerCallingWidget :type BP%20Player%20Object%20Reference))
  (Utilities|IsValid PlayerCallingWidget
    (:Is%20Valid
      (switch Utilities|FlowControl|Switch|SwitchonE_PlayersTeam (Variables|/Game/_Jam_MilkyWay/Players/FirstPerson/Blueprints/BP_Player.BP_Player_C|GetTeam PlayerCallingWidget)
        (:NewEnumerator0
          (Default|ActivateEWdiget PlayerCallingWidget On/Off (Variables|Default|GetWidget)))))))

(fn ConstructionScript)

(fn OnRepIsGrabed
  (bind _trapsm (Variables|Default|GetTrapSM))
  (bind _trapsm_2 (Variables|Default|GetTrapSM))
  (bind _trapsm_3 (Variables|Default|GetTrapSM))
  (if (Variables|Default|GetIsGrabed)
    (Physics|SetSimulatePhysics _trapsm false)
    (Variables|Default|SetDisplayInteractionWidget false)
    (Collision|SetCollisionEnabled _trapsm_3 "NoCollision")
    (else
      (Physics|SetPhysicsLinearVelocity _trapsm_2 (* (Transformation|GetComponentVelocity _trapsm_2) 0.2) false "None")
      (Collision|SetCollisionEnabled _trapsm_3 "QueryAndPhysics")
      (Networking|SwitchHasAuthority
        (:Authority
          (Physics|SetSimulatePhysics _trapsm true))))))

(fn OnRepSpawnTrap
  (CallFunction|RPCSPAWNTRAP))

(fn OnRepDisplayInteractionWidget
  (Development|SetHiddeninGame (Variables|Default|GetWidget) (not (Variables|Default|GetDisplayInteractionWidget)) false))