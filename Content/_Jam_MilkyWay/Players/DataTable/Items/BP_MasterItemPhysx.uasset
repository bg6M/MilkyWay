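; Master networked physics pickup that players can grab or use to receive a buff.
; Replicated item data drives the buff type, mesh, materials and rarity VFX through OnRep functions.
; Interacting while not grabbed applies the buff, plays an explosion and destroys the actor.
; Grab and release route through RPCs, with OnRep toggling physics and VFX and damping release velocity; trap spawning is unwired, leaving a placeholder print.
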(event Custom|RPC%20GRAB
  (params (Target :type BP%20Player%20Object%20Reference))
  (bind _sm (Variables|Default|GetSM))
  (Transformation|SetWorldRotation _sm (Pawn|GetControlRotation Target :!class /Script/Engine.Pawn) false false)
  (Variables|Default|SetIsGrabed true)
  (Collision|SetCollisionEnabled _sm "PhysicsOnly"))

(event Custom|RPC%20UNGRAB
  (Variables|Default|SetIsGrabed false)
  (Collision|SetCollisionEnabled (Variables|Default|GetSM) "QueryAndPhysics")
  (Variables|Default|SetPlayer%20Calling%20Grab 0))

(event Custom|ServerRPCGRAB
  (params (Player%20Calling%20Grab :type BP%20Player%20Object%20Reference))
  (CallFunction|RPCGRAB Player%20Calling%20Grab))

(event Custom|SERVER%20RPC%20UNGRAB
  (CallFunction|RPCUNGRAB))

(event Custom|RPC%20SPAWN%20TRAP
  (Development|PrintString "BUFF SOON"))

(event Custom|Server%20Interact
  (params (Player :type BP%20Player%20Object%20Reference))
  (Variables|Default|SetUseItem true)
  (Default|ActiveBuff Player (Variables|Default|GetPerma?) (Variables|Default|GetTime) (Variables|Default|GetE%20Buff))
  (Niagara|SpawnSystematLocation "/Niagara/DefaultAssets/Templates/Systems/SimpleExplosion.SimpleExplosion" (Transformation|GetActorLocation) "0, 0, 0" "0.500000,0.500000,0.500000")
  (Actor|DestroyActor))

(event Custom|RPC%20SETDATA
  (params (BonusItemStructure :type S%20Drop%20Box%20Upgrade%20Structure))
  (CallFunction|SETDATA BonusItemStructure))

(event EventBeginPlay
  (bind _asbp_game_instance (Utilities|Casting|CastToBP_GameInstance (Game|GetGameInstance)))
  (Variables|Default|SetAs%20BP%20Game%20Instance _asbp_game_instance)
  (bind _asgs_lobby (Utilities|Casting|CastToGS_Lobby (Game|GetGameState)))
  (Variables|Default|SetAs%20GS%20Lobby _asgs_lobby))

(event EventGrabInterface
  (params (Player%20calling%20grab :type BP%20Player%20Object%20Reference) (PlayerTeam :type E_PlayersTeam%20Enum :default "NewEnumerator0"))
  (bind _output_get (Variables|Default|SetPlayer%20Calling%20Grab Player%20calling%20grab))
  (CallFunction|ServerRPCGRAB _output_get))

(event EventInteractInt
  (params (Bp_Player :type BP%20Player%20Object%20Reference))
  (if (not (Variables|Default|GetIsGrabed))
    (bind _output_get (Variables|Default|SetBp%20Player Bp_Player))
    (CallFunction|ServerInteract _output_get)))

(event EventSetDropBoxData
  (params (DATA :type S%20Drop%20Box%20Upgrade%20Structure))
  (CallFunction|RPCSETDATA))

(event EventUnGrabInterface
  (CallFunction|SERVERRPCUNGRAB))

(fn ConstructionScript)

(fn OnRepIsGrabed
  (bind _sm (Variables|Default|GetSM))
  (bind _rarityvfx (Variables|Default|GetRarityVFX))
  (bind _sm_2 (Variables|Default|GetSM))
  (if (Variables|Default|GetIsGrabed)
    (Physics|SetSimulatePhysics _sm false)
    (Development|SetHiddeninGame _rarityvfx true false)
    (else
      (Physics|SetSimulatePhysics _sm true)
      (Development|SetHiddeninGame _rarityvfx false false)
      (Physics|SetPhysicsLinearVelocity _sm_2 (* (Transformation|GetComponentVelocity _sm_2) 0.2) false "None"))))

(fn SETDATA
  (params (BonusItemStructure :type S%20Drop%20Box%20Upgrade%20Structure))
  (Variables|Default|SetBonus%20Item%20Structure BonusItemStructure))

(fn OnRepQuality
  (bind _rarityvfx (Variables|Default|GetRarityVFX))
  (bind _material (Variables|Default|GetMaterial))
  (bind _rarityvfx_2 (Variables|Default|GetRarityVFX))
  (bind _material_2 (Variables|Default|GetMaterial))
  (bind _rarityvfx_3 (Variables|Default|GetRarityVFX))
  (bind _material_3 (Variables|Default|GetMaterial))
  (switch Utilities|FlowControl|Switch|SwitchonE_DropBoxType (Variables|Default|GetQuality)
    (:NewEnumerator0
      (Rendering|Material|SetMaterial _rarityvfx_2 0 (Utilities|Array|Get(acopy) _material_2))
      (Rendering|Material|SetMaterial _rarityvfx_2 1 (Utilities|Array|Get(acopy) _material_2 3)))
    (:NewEnumerator1
      (Rendering|Material|SetMaterial _rarityvfx_3 1 (Utilities|Array|Get(acopy) _material_3))
      (Rendering|Material|SetMaterial _rarityvfx_3 4 (Utilities|Array|Get(acopy) _material_3 3)))
    (:NewEnumerator2
      (Rendering|Material|SetMaterial _rarityvfx 2 (Utilities|Array|Get(acopy) _material))
      (Rendering|Material|SetMaterial _rarityvfx 5 (Utilities|Array|Get(acopy) _material 3)))))

(fn OnRepUseItem
  (CallFunction|RPCSPAWNTRAP))

(fn OnRepBonusItemStructure
  (bind _sm (Variables|Default|GetSM))
  (bind _bonus_item_structure (Variables|Default|GetBonus%20Item%20Structure))
  (bind (_quality _upgradetype _actor_structure _item_structure) (Utilities|Struct|BreakS_DropBox_Upgrade _bonus_item_structure))
  (bind (_actortospawn _numbers _setdata_ _sm_2 _mi_bank _buff_to_call) (Utilities|Struct|BreakS_Items _item_structure))
  (Variables|Default|SetQuality _quality)
  (Variables|Default|SetE%20Buff _buff_to_call)
  (Components|StaticMesh|SetStaticMesh _sm _sm_2)
  (for (_ _array_index) (Rendering|Material|GetMaterials _sm)
    (Rendering|Material|SetMaterial _sm _array_index (Utilities|Array|Get(acopy) _mi_bank _array_index))))