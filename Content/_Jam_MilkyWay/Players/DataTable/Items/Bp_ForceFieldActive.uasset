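; Deployed force field item that briefly immobilizes any player who hits it.
; On BeginPlay a timeline scales the field up, then sets IsActive, whose RepNotify starts a two-minute timer before it shrinks and is destroyed.
; Hits while active spawn a burst at the impact and toggle IsTrigger, whose RepNotify disables the player's movement, then restores walking two seconds later.
; RPC- and MC-prefixed events carry activation, scaling and trigger logic.
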(event `self.ReceiveBeginPlay`
  (bind _asbp_game_instance (cast `/Game/_Jam_MilkyWay/Players/FirstPerson/Blueprints/BP_GameInstance` (`GameplayStatics.GetGameInstance`)))
  (set `self.As BP Game Instance` _asbp_game_instance)
  (bind _asgs_lobby (cast `/Game/_Jam_MilkyWay/Players/MenuPlayer/GS_Lobby` (`GameplayStatics.GetGameState`))
    (:`then`
      (set `self.As GS Lobby` _asgs_lobby))
    (:`CastFailed`
      _))
  (`self.RPC ACTIVATED`))

(event `RPC ACTIVATED`
  (bind (_direction _scale) (`Timeline|OPEN` :!via `PlayFromStart`)
    (:`Update`
      (`self.MC ACTIVATED` _scale))
    (:`Finished`
      (set `self.IsActive` true))))

(event `RPC OVERLAP`
  (params (Object :type "Object Object Reference") (Location :type "Vector Structure"))
  (bind _asbp_player (cast `/Game/_Jam_MilkyWay/Players/FirstPerson/Blueprints/BP_Player` Object))
  (set `self.As BP Player` _asbp_player)
  (`self.RPC TRIGGER TRAP` Location))

(event `RPC TRIGGER TRAP`
  (params (Location :type "Vector Structure"))
  (set `self.IsTrigger` true)
  (`NiagaraFunctionLibrary.SpawnSystemAtLocation` "/Niagara/DefaultAssets/Templates/Systems/DirectionalBurst.DirectionalBurst" Location)
  (`KismetSystemLibrary.Delay` 2.0)
  (set `self.IsTrigger` false))

(event `MC ACTIVATED`
  (params (NewScale3D :type "Vector Structure"))
  (`SceneComponent.SetRelativeScale3D` (`self.MFX_ForceField`) NewScale3D))

(event `Timer`
  (`KismetSystemLibrary.Delay` 120.0)
  (bind (_direction _scale) (`Timeline|Timeline` :!via `ReverseFromEnd`)
    (:`Update`
      (`self.MC TIMER` _scale))
    (:`Finished`
      (`self.K2_DestroyActor`))))

(event `self.MFX_ForceField.OnComponentHit`
  (params (HitComponent :type "PrimitiveComponent Object Reference") (OtherActor :type "Actor Object Reference") (OtherComp :type "PrimitiveComponent Object Reference") (NormalImpulse :type "Vector Structure") (Hit :type "HitResult Structure (by ref)"))
  (if (`self.IsActive`)
    (`self.RPC OVERLAP` OtherActor (`.ImpactPoint` (`GameplayStatics.BreakHitResult` Hit)))))

(event `MC TIMER`
  (params (NewScale3D :type "Vector Structure"))
  (`SceneComponent.SetRelativeScale3D` (`self.MFX_ForceField`) NewScale3D))

(fn `OnRep_IsActive`
  (`self.Timer`))

(fn `OnRep_IsGrabed`
  (bind _skeletalmesh (`self.SkeletalMesh`))
  (if (`self.IsGrabed`)
    (`PrimitiveComponent.SetSimulatePhysics` _skeletalmesh false)
    (else
      (`PrimitiveComponent.SetSimulatePhysics` _skeletalmesh true))))

(fn `OnRep_IsTrigger`
  (bind _charactermovement (`Character.CharacterMovement` (`self.As BP Player`)))
  (if (`self.IsTrigger`)
    (`NavMovementComponent.StopActiveMovement` _charactermovement)
    (`CharacterMovementComponent.DisableMovement` _charactermovement)
    (else
      (`CharacterMovementComponent.SetMovementMode` (`Character.CharacterMovement` (`self.As BP Player`)) "MOVE_Walking" 0))))

(fn `UserConstructionScript`)