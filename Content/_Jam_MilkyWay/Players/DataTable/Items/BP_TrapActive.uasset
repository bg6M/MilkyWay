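; BP_TrapActive is an armed trap item that immobilizes any player who steps into its sphere.
; BeginPlay caches the game instance and lobby game state, then arms the trap.
; An overlap passes through RPC-named events that stop and disable the player's movement, teleport them onto the trap and set IsTrigger.
; The IsGrabed RepNotify turns skeletal mesh physics off while held; the other RepNotifies are empty.
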(event `self.ReceiveBeginPlay`
  (bind _asbp_game_instance (cast `/Game/_Jam_MilkyWay/Players/FirstPerson/Blueprints/BP_GameInstance` (`GameplayStatics.GetGameInstance`)))
  (set `self.As BP Game Instance` _asbp_game_instance)
  (bind _asgs_lobby (cast `/Game/_Jam_MilkyWay/Players/MenuPlayer/GS_Lobby` (`GameplayStatics.GetGameState`)))
  (set `self.As GS Lobby` _asgs_lobby)
  (set `self.IsActive` true))

(event `self.Sphere.OnComponentBeginOverlap`
  (params (OverlappedComponent :type "PrimitiveComponent Object Reference") (OtherActor :type "Actor Object Reference") (OtherComp :type "PrimitiveComponent Object Reference") (OtherBodyIndex :type Integer) (bFromSweep :type Boolean) (SweepResult :type "HitResult Structure (by ref)"))
  (if (`self.IsActive`)
    (`self.RPC OVERLAP` OtherActor)))

(event `RPC OVERLAP`
  (params (Object :type "Object Object Reference"))
  (bind _asbp_player (cast `/Game/_Jam_MilkyWay/Players/FirstPerson/Blueprints/BP_Player` Object))
  (set `self.As BP Player` _asbp_player)
  (`self.RPC TRIGGER TRAP`))

(event `RPC TRIGGER TRAP`
  (bind _as_bp_player (`self.As BP Player`))
  (bind _charactermovement (`Character.CharacterMovement` _as_bp_player))
  (`NavMovementComponent.StopActiveMovement` _charactermovement)
  (`CharacterMovementComponent.DisableMovement` _charactermovement)
  (`self.K2_TeleportTo` :`self` _as_bp_player :`DestLocation` (`self.K2_GetActorLocation`))
  (set `self.IsTrigger` true))

(fn `OnRep_IsActive`)

(fn `OnRep_IsGrabed`
  (bind _skeletalmesh (`self.SkeletalMesh`))
  (if (`self.IsGrabed`)
    (`PrimitiveComponent.SetSimulatePhysics` _skeletalmesh false)
    (else
      (`PrimitiveComponent.SetSimulatePhysics` _skeletalmesh true))))

(fn `OnRep_IsTrigger`)

(fn `UserConstructionScript`)