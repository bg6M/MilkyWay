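; BP_ItemSpawner_LD is a placed item spawn point that registers itself on the server in the GS_Lobby game state's ItemSpawnerBank.
; RPC_SpawnItem removes it from the bank, spawns an item at its Arrow, then destroys the spawner.
; The item is either a manually set class or a random pick, with a roughly one-in-four rare roll that GS_Lobby's shared RareItemSpawn flag limits to one success.
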(event `self.ReceiveBeginPlay`
  (`/Engine/EditorBlueprintResources/ActorMacros.Switch Has Authority`
    (:`Authority`
      (bind _asgs_lobby (cast `/Game/_Jam_MilkyWay/Players/MenuPlayer/GS_Lobby` (`GameplayStatics.GetGameState`)))
      (bind _output_get (set `self.As GS Lobby` _asgs_lobby))
      (`KismetArrayLibrary.Array_AddUnique` (`/Game/_Jam_MilkyWay/Players/MenuPlayer/GS_Lobby.ItemSpawnerBank` _output_get) self))))

(event `RPC_SpawnItem`
  (`/Engine/EditorBlueprintResources/ActorMacros.Switch Has Authority`
    (:`Authority`
      (`KismetArrayLibrary.Array_RemoveItem` (`/Game/_Jam_MilkyWay/Players/MenuPlayer/GS_Lobby.ItemSpawnerBank` (`self.As GS Lobby`)) self)
      (if (`self.ManualSpawn`)
        (`|SpawnActorFromClass` (`self.ManualActorToSpawn`) (`SceneComponent.K2_GetComponentToWorld` (`self.Arrow`)) "Undefined" "MultiplyWithRoot" null null)
        (elif (>= (`KismetMathLibrary.RandomIntegerInRange` 0 100) 75)
          (if (`/Game/_Jam_MilkyWay/Players/MenuPlayer/GS_Lobby.RareItemSpawn` (`self.As GS Lobby`))
            (`|SpawnActorFromClass` (`|GetArrayItem` (`self.Class`) (`KismetMathLibrary.RandomIntegerInRange` 0 1)) (`SceneComponent.K2_GetComponentToWorld` (`self.Arrow`)) "Undefined" "MultiplyWithRoot" null null :!label _label)
            (else
              (`|SpawnActorFromClass` (`|GetArrayItem` (`self.Class`) (`KismetMathLibrary.RandomIntegerInRange` 2 3)) (`SceneComponent.K2_GetComponentToWorld` (`self.Arrow`)) "Undefined" "MultiplyWithRoot" null null)
              (set `/Game/_Jam_MilkyWay/Players/MenuPlayer/GS_Lobby.RareItemSpawn` true (`self.As GS Lobby`))))
          (else
            (goto _label))))
      (`self.K2_DestroyActor`))))

(fn `UserConstructionScript`)