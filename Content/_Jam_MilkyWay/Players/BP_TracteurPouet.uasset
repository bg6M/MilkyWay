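; BP_TracteurPouet is an interactable tractor that plays an alarm sound when a player interacts with it.
; Interaction calls an RPC event that relays to a multicast event, which plays the sound at the actor's location with far attenuation and prints a debug string.
; BeginPlay also caches the game instance, though the graph never uses it afterwards.
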(event `self.ReceiveBeginPlay`
  (bind _asbp_game_instance (cast `/Game/_Jam_MilkyWay/Players/FirstPerson/Blueprints/BP_GameInstance` (`GameplayStatics.GetGameInstance`)))
  (set `self.As BP Game Instance` _asbp_game_instance))

(event `/Game/_Jam_MilkyWay/Players/FirstPerson/Blueprints/Interface/BPI_Interaction.Interact_Int`
  (params (Bp_Player :type "/Game/_Jam_MilkyWay/Players/FirstPerson/Blueprints/BP_Player Object Reference"))
  (`self.RPC_TractorSound`))

(event `MC_TractorSound`
  (`GameplayStatics.PlaySoundAtLocation` "/Game/_Jam_MilkyWay/SFX/Foleys/Alarm/Alarm_Average_SFX.Alarm_Average_SFX" (`self.K2_GetActorLocation`) (struct) 1.0 1.0 0.0 "/Game/_Jam_MilkyWay/SFX/Attenuation/Far_SoundAttenuation.Far_SoundAttenuation" null null null)
  (`KismetSystemLibrary.PrintString` "TRACTEUR"))

(event `RPC_TractorSound`
  (`self.MC_TractorSound`))

(fn `UserConstructionScript`)