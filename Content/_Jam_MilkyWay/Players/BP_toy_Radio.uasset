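; Interactable toy radio actor that players can switch on and off and that can be outlined as interactive.
; Interaction toggles the OnOff RepNotify variable, whose OnRep plays or stops the RadioMusic01 audio and the looping skeletal mesh animation.
; After a short delay, SetMusic stops a separate 2D sound created at BeginPlay when off.
; Its PlayMusic counterpart is an empty stub.
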(event `self.ReceiveBeginPlay`
  (bind _asbp_game_instance (cast `/Game/_Jam_MilkyWay/Players/FirstPerson/Blueprints/BP_GameInstance` (`GameplayStatics.GetGameInstance`)))
  (set `self.As BP Game Instance` _asbp_game_instance)
  (bind _returnvalue (`GameplayStatics.CreateSound2D` (`self.Sound`) 1.0 1.0 0.0 null false false))
  (set `self.MusicPlayed` _returnvalue))

(event `self.INTERACTION_TEST_INTERFACE`
  (`self.TOUCHE` :!label _label)
  (`KismetSystemLibrary.Delay` 0.2)
  (`self.SetMusic`))

(event `/Game/_Jam_MilkyWay/Players/FirstPerson/Blueprints/Interface/BPI_Interaction.Interact_Int`
  (params (Bp_Player :type "/Game/_Jam_MilkyWay/Players/FirstPerson/Blueprints/BP_Player Object Reference"))
  (goto _label))

(event `TOUCHE`
  (if (`self.On/Off`)
    (set `self.On/Off` false)
    (else
      (set `self.On/Off` true))))

(event `RunServerTOUCH`
  (bind _radiomusic01 (`self.RadioMusic01`))
  (bind _skeletalmesh (`self.SkeletalMesh`))
  (if (`self.On/Off`)
    (`AudioComponent.Play` _radiomusic01 0.0)
    (`SkeletalMeshComponent.PlayAnimation` _skeletalmesh "/Game/_Jam_MilkyWay/Gpe/Radio/ANIM_RadioMusic.ANIM_RadioMusic" true)
    (else
      (`AudioComponent.Stop` _radiomusic01)
      (`SkeletalMeshComponent.Stop` _skeletalmesh))))

(event `SetMusic`
  (if (`self.On/Off`)
    (`/Engine/EditorBlueprintResources/StandardMacros.IsValid` (`self.MusicPlayed`)
      (:`Is Not Valid`
        (`self.PlayMusic`)))
    (else
      (`self.StopMusic`))))

(event `PlayMusic`)

(event `StopMusic`
  (`AudioComponent.Stop` (`self.MusicPlayed`)))

(event `/Game/_Jam_MilkyWay/Players/FirstPerson/Blueprints/Interface/BPI_Interaction.ToggleOutlineInteractible`
  (params (`Player Calling` :type "/Game/_Jam_MilkyWay/Players/FirstPerson/Blueprints/BP_Player Object Reference"))
  (`/Game/_Jam_MilkyWay/Players/FirstPerson/Blueprints/BP_Player.ACTIVATE OUTLINE` `Player Calling` true (`self.SkeletalMesh`)))

(fn `OnRep_CurrentSound`)

(fn `OnRep_MusicPlayed`
  (`self.PlayMusic`))

(fn `OnRep_On/Off`
  (`self.RunServerTOUCH`))

(fn `UserConstructionScript`)