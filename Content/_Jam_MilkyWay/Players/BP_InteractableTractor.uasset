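; BP_InteractableTractor is an interactable tractor that honks and flashes its headlights when used.
; Interaction calls a sound RPC, which relays to a multicast event that plays the klaxon and starts the HeadLights timeline.
; The timeline drives spotlight intensity, light-cone opacity and gradient, and the tractor material's intensity.
; BeginPlay caches the game instance and has a sound call, with no sound assigned, noted for looping engine noise.
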(event `self.ReceiveBeginPlay`
  (bind _asbp_game_instance (cast `/Game/_Jam_MilkyWay/Players/FirstPerson/Blueprints/BP_GameInstance` (`GameplayStatics.GetGameInstance`)))
  (set `self.As BP Game Instance` _asbp_game_instance)
  ;[1 1 1] jouer en continu le bruit de moteur du tracteur, s'assurer que c'est repliqué
  (`GameplayStatics.PlaySoundAtLocation` null (`self.K2_GetActorLocation`) (struct) 1.0 1.0 0.0 "/Game/_Jam_MilkyWay/SFX/Attenuation_Types/Far_SoundAttenuation.Far_SoundAttenuation" null null null))

(event `/Game/_Jam_MilkyWay/Players/FirstPerson/Blueprints/Interface/BPI_Interaction.Interact_Int`
  (params (Bp_Player :type "/Game/_Jam_MilkyWay/Players/FirstPerson/Blueprints/BP_Player Object Reference"))
  (`self.RPC_TractorSound`))

(event `MC_TractorSound`
  (bind _coner (`self.ConeR`))
  (`GameplayStatics.PlaySoundAtLocation` "/Game/_Jam_MilkyWay/SFX/Foleys/Horns/TractorKlaxon_SC.TractorKlaxon_SC" (`self.K2_GetActorLocation`) (struct) 1.0 1.0 0.0 "/Game/_Jam_MilkyWay/SFX/Attenuation_Types/Far_SoundAttenuation.Far_SoundAttenuation" null null null)
  (bind (_direction _intensitymultiplier _tractormaterial) (`Timeline|HeadLights` :!via `PlayFromStart`)
    (:`Update`
      (`MeshComponent.SetScalarParameterValueOnMaterials` _coner "IntensityGradient" (`KismetMathLibrary.Lerp` 0.0 10.0 _intensitymultiplier))
      (`MeshComponent.SetScalarParameterValueOnMaterials` (`self.ConeL`) "IntensityGradient" (`KismetMathLibrary.Lerp` 0.0 10.0 _intensitymultiplier))
      (`MeshComponent.SetScalarParameterValueOnMaterials` _coner "GlobalOpacity" (`KismetMathLibrary.Lerp` 0.0 3.693107 _intensitymultiplier))
      (`MeshComponent.SetScalarParameterValueOnMaterials` (`self.ConeL`) "GlobalOpacity" (`KismetMathLibrary.Lerp` 0.0 3.693107 _intensitymultiplier))
      (`LightComponent.SetIntensity` (`self.SpotLightL`) (`KismetMathLibrary.Lerp` 0.0 16.0 _intensitymultiplier))
      (`LightComponent.SetIntensity` (`self.SpotLightR`) (`KismetMathLibrary.Lerp` 0.0 16.0 _intensitymultiplier))
      (`MeshComponent.SetScalarParameterValueOnMaterials` (`self.Tractor`) "Intensity" (`KismetMathLibrary.Lerp` 0.0 0.75 _tractormaterial)))))

(event `RPC_TractorSound`
  (`self.MC_TractorSound`))

(fn `UserConstructionScript`)