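; BP_InteractableHarvester is an interactable harvester that honks its horn and animates its headlights when a player interacts with it.
; Interaction calls an RPC that forwards to a multicast event, which plays the klaxon and runs a timeline driving the harvester material's Intensity.
; BeginPlay caches the game instance and has a sound call for engine noise with no sound assigned.
; Light cone and spotlight intensity logic is present but unconnected.
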(event `self.ReceiveBeginPlay`
  (bind _asbp_game_instance (cast `/Game/_Jam_MilkyWay/Players/FirstPerson/Blueprints/BP_GameInstance` (`GameplayStatics.GetGameInstance`)))
  (set `self.As BP Game Instance` _asbp_game_instance)
  ;[1 1 1] jouer en continu le bruit de moteur de la moiss, s'assurer que c'est repliqué
  (`GameplayStatics.PlaySoundAtLocation` null (`self.K2_GetActorLocation`) (struct) 1.0 1.0 0.0 "/Game/_Jam_MilkyWay/SFX/Attenuation_Types/Far_SoundAttenuation.Far_SoundAttenuation" null null null))

(event `self.Interact_Int`
  (params (Bp_Player :type "/Game/_Jam_MilkyWay/Players/FirstPerson/Blueprints/BP_Player Object Reference"))
  (`self.RPC_TractorSound`))

(event `MC_TractorSound`
  (`GameplayStatics.PlaySoundAtLocation` "/Game/_Jam_MilkyWay/SFX/Foleys/Horns/HarvesterKlaxon_SoundCue.HarvesterKlaxon_SoundCue" (`self.K2_GetActorLocation`) (struct) 1.0 1.0 0.0 "/Game/_Jam_MilkyWay/SFX/Attenuation_Types/Far_SoundAttenuation.Far_SoundAttenuation" null null null)
  (bind (_direction _intensitymultiplier _tractormaterial) (`Timeline|HeadLights`)
    (:`Update`
      ;[1 1 1] eteindre les phares
      (`MeshComponent.SetScalarParameterValueOnMaterials` (`self.Harvester`) "Intensity" (`KismetMathLibrary.Lerp` 0.0 0.75 _tractormaterial)))))

(event `RPC_TractorSound`
  (`self.MC_TractorSound`))

(fn `UserConstructionScript`)