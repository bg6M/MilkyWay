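; Lobby Game Mode that gathers session players and launches a GREEZ versus MANZ team match.
; PostLogin tracks controllers, waits briefly, kicks players beyond session capacity, and launches once the server is full.
; Launch delegates team building and spawning to GS_Lobby; local BuildTeam (one random GREEZ, rest MANZ) and SpawnTeam (hardcoded spawn points) are uncalled here.
; Logout removes and kicks the player, and EndGame tears down sessions.
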(event `self.ReceiveBeginPlay`
  (bind _asbp_game_instance (cast `/Game/_Jam_MilkyWay/Players/FirstPerson/Blueprints/BP_GameInstance` (`GameplayStatics.GetGameInstance`)))
  (set `self.As BP Game Instance` _asbp_game_instance)
  (bind _asgs_lobby (cast `/Game/_Jam_MilkyWay/Players/MenuPlayer/GS_Lobby` (`GameplayStatics.GetGameState`)))
  (set `self.As GS Lobby` _asgs_lobby))

(event `self.K2_OnLogout`
  (params (ExitingController :type "Controller Object Reference"))
  (bind _asplayer_controller (cast `PlayerController` ExitingController))
  (`KismetArrayLibrary.Array_RemoveItem` (`self.PlayersController`) _asplayer_controller)
  (`AdvancedSessionsLibrary.KickPlayer` _asplayer_controller "Quit"))

(event `self.K2_PostLogin`
  (params (NewPlayer :type "PlayerController Object Reference"))
  (`KismetArrayLibrary.Array_AddUnique` (`self.PlayersController`) NewPlayer)
  (`KismetArrayLibrary.Array_AddUnique` (`self.Unique Net Id`) (`AdvancedSessionsLibrary.GetUniqueNetID` NewPlayer))
  (`KismetSystemLibrary.RetriggerableDelay` 2.0)
  (bind (_numconnections _numprivateconnections _bislan _bisdedicated _ballowinvites _ballowjoininprogress _bisanticheatenabled _builduniqueid _extrasettings) (`AdvancedSessionsLibrary.GetSessionSettings`)
    (:`OnSuccess`
      (if (> (`KismetArrayLibrary.Array_Length` (`GameStateBase.PlayerArray` (`GameplayStatics.GetGameState`))) _numconnections)
        (bind (_arrayindex _arrayelement) (`/Engine/EditorBlueprintResources/StandardMacros.ReverseForEachLoop` (`self.PlayersController`))
          (:`LoopBody`
            (if (>= _arrayindex _numconnections)
              (`AdvancedSessionsLibrary.KickPlayer` _arrayelement "Server Full")))
          (:`Completed`
            (`UpdateSessionCallbackProxyAdvanced.UpdateSession` _extrasettings _numconnections 0 _bislan :!label _label
              (:`OnSuccess`
                (`/Engine/EditorBlueprintResources/ActorMacros.Switch Has Authority`
                  (:`Authority`
                    (if (`self.HasAuthority` (`GameplayStatics.GetPlayerController` 0))
                      (`self.LAUNCH GAME`))))))))
        (elif (== _numconnections (`KismetArrayLibrary.Array_Length` (`GameStateBase.PlayerArray` (`GameplayStatics.GetGameState`))))
          (goto _label))))))

(event `LAUNCH GAME`
  (`KismetSystemLibrary.Delay` 3.0)
  (bind (_success _player_in_equip) (`/Game/_Jam_MilkyWay/Players/MenuPlayer/GS_Lobby.Build Team` (`self.As GS Lobby`)))
  (set `self.Player in Equip` _player_in_equip)
  (if _success
    (`KismetSystemLibrary.Delay` 3.0)
    (`/Game/_Jam_MilkyWay/Players/MenuPlayer/GS_Lobby.SpawnTeam` (`self.As GS Lobby`))))

(event `SpawnTeamRPC`)

(event `End Game`
  (for _array_element (`self.PlayersController`)
    (`EndSessionCallbackProxy.EndSession` _array_element
      (:`OnFailure`
        (`DestroySessionCallbackProxy.DestroySession` _array_element
          (:`OnFailure`
            (`AdvancedSessionsLibrary.KickPlayer` _array_element "GameEnd"))))))
  (`KismetSystemLibrary.PrintString` "ALLO LE FOOT?")
  (`DestroySessionCallbackProxy.DestroySession` (`GameplayStatics.GetPlayerController` 0)))

(fn `Build Team`
  (locals (IsGrezz :type Boolean))
  (bind _playerscontroller (`self.PlayersController`))
  (bind _player_in_equip (`self.Player in Equip`))
  (if (`BlueprintMapLibrary.Map_IsNotEmpty` _player_in_equip)
    (`BlueprintMapLibrary.Map_Clear` _player_in_equip))
  (`BlueprintMapLibrary.Map_Add` (`self.Player in Equip`) (`|GetArrayItem` _playerscontroller (`KismetMathLibrary.RandomIntegerInRange` 0 (- (`KismetArrayLibrary.Array_Length` _playerscontroller) 1))) "NewEnumerator1")
  (for _array_element _playerscontroller
    (if (not (`.ReturnValue` (`BlueprintMapLibrary.Map_Find` (`self.Player in Equip`) _array_element)))
      (`BlueprintMapLibrary.Map_Add` (`self.Player in Equip`) _array_element "NewEnumerator0"))))

(fn `Spawn Team`
  (bind _as_gs_lobby (`self.As GS Lobby`))
  (bind _as_gs_lobby_2 (`self.As GS Lobby`))
  (if (`/Game/_Jam_MilkyWay/Players/MenuPlayer/GS_Lobby.Team Ready` _as_gs_lobby)
    (for _array_element (`GameStateBase.PlayerArray` _as_gs_lobby)
      (bind _returnvalue (`PlayerState.GetPlayerController` _array_element))
      (bind (_value _returnvalue_2) (`BlueprintMapLibrary.Map_Find` (`/Game/_Jam_MilkyWay/Players/MenuPlayer/GS_Lobby.Player in Equip` _as_gs_lobby) _returnvalue))
      (if _returnvalue_2
        (switch `/Game/_Jam_MilkyWay/Players/MenuPlayer/E_PlayersTeam` _value
          (:`NewEnumerator0`
            (bind _returnvalue_3 (`GameplayStatics.GetActorOfClass` "/Game/_Jam_MilkyWay/Players/MenuPlayer/BP_MANZ_SpawnZone.BP_MANZ_SpawnZone_C"))
            (set `self.Spawn Transform` (`KismetMathLibrary.MakeTransform` (-1549.0 -789.0 400.0)))
            (bind _returnvalue_4 (`|SpawnActorFromClass` "/Game/_Jam_MilkyWay/Players/FirstPerson/Blueprints/BP_Player.BP_Player_C" (`self.Spawn Transform`) "AdjustIfPossibleButAlwaysSpawn" "MultiplyWithRoot" null "NewEnumerator0" 0 null))
            (set `/Game/_Jam_MilkyWay/Players/FirstPerson/Blueprints/BP_Player.Team` "NewEnumerator0" _returnvalue_4)
            (`KismetArrayLibrary.Array_Add` (`/Game/_Jam_MilkyWay/Players/MenuPlayer/GS_Lobby.Manz` _as_gs_lobby_2) _returnvalue_4)
            (`Controller.Possess` _returnvalue _returnvalue_4)
            (`WidgetBlueprintLibrary.SetInputMode_GameOnly` _returnvalue)
            (`/Game/_Jam_MilkyWay/Players/FirstPerson/Blueprints/BP_Player.RemoveLobby` _returnvalue_4)
            (message `/Game/_Jam_MilkyWay/Players/FirstPerson/Blueprints/Interface/Damage_Interface.INTERACTION_TEST_INTERFACE` _returnvalue)
            (`/Game/_Jam_MilkyWay/Players/FirstPerson/Blueprints/BP_Player.RPC UpdateTeam` _returnvalue_4))
          (:`NewEnumerator1`
            (bind _returnvalue_5 (`GameplayStatics.GetActorOfClass` "/Game/_Jam_MilkyWay/Players/MenuPlayer/BP_GREEZ_SpawnZone.BP_GREEZ_SpawnZone_C"))
            (set `self.Spawn Transform` (`KismetMathLibrary.MakeTransform` (-2910.0 -2670.0 350.0)))
            (bind _returnvalue_6 (`|SpawnActorFromClass` "/Game/_Jam_MilkyWay/Players/FirstPerson/Blueprints/BP_Player.BP_Player_C" (`self.Spawn Transform`) "AdjustIfPossibleButAlwaysSpawn" "MultiplyWithRoot" null "NewEnumerator1" 0 null))
            (`KismetArrayLibrary.Array_Add` (`/Game/_Jam_MilkyWay/Players/MenuPlayer/GS_Lobby.Greez` _as_gs_lobby_2))
            (`Controller.Possess` _returnvalue _returnvalue_6)
            (`WidgetBlueprintLibrary.SetInputMode_GameOnly` _returnvalue)
            (`/Game/_Jam_MilkyWay/Players/FirstPerson/Blueprints/BP_Player.RemoveLobby` _returnvalue_6)
            (message `/Game/_Jam_MilkyWay/Players/FirstPerson/Blueprints/Interface/Damage_Interface.INTERACTION_TEST_INTERFACE` _returnvalue_6)
            (`/Game/_Jam_MilkyWay/Players/FirstPerson/Blueprints/BP_Player.RPC UpdateTeam` _returnvalue_6)))))
    (set `/Game/_Jam_MilkyWay/Players/MenuPlayer/GS_Lobby.Game is Ready` true _as_gs_lobby)
    (`KismetSystemLibrary.PrintString` "TEAM SPAWNED")))

(fn `StartGame`)

(fn `UserConstructionScript`)