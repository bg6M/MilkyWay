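; Menu player controller that puts the menu widget on screen, prepares input mappings and provides proximity voice chat toggles.
; BeginPlay creates the widget, passes it the controller, then adds and registers the default Enhanced Input context and caches its mappable keys.
; InitializeVOIP joins or leaves an Onset VOIP channel and switches voice capture through ToggleProxiChat.
; Delay-based retry loops wait for the controller, VOIP subsystem and PlayerState to become valid.
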(event `self.ReceiveBeginPlay`
  (bind _returnvalue (`GameplayStatics.GetPlayerController` 0))
  (bind _asbp_game_instance (cast `/Game/_Jam_MilkyWay/Players/FirstPerson/Blueprints/BP_GameInstance` (`GameplayStatics.GetGameInstance`)))
  (set `self.As BP Game Instance` _asbp_game_instance)
  (`/Engine/EditorBlueprintResources/StandardMacros.IsValid` _returnvalue :!label _label
    (:`Is Valid`
      (bind _returnvalue_2 (`|CreateWidget` (`self.Class`) _returnvalue))
      (bind _output_get (set `self.MenuWidget` _returnvalue_2))
      (`UserWidget.AddToViewport` _output_get 0)
      (message `/Game/_Jam_MilkyWay/Players/MenuPlayer/Menu_Interface.Int_Call_Menu` _output_get _returnvalue)
      (`self.GetPlayerMappingInput`))
    (:`Is Not Valid`
      (`KismetSystemLibrary.Delay` 3.0)
      (goto _label))))

(event `GetPlayerMappingInput`
  (bind _returnvalue (subsystem `EnhancedInputLocalPlayerSubsystem`))
  (bind _returnvalue_2 (`EnhancedInputSubsystemInterface.GetUserSettings` _returnvalue))
  (`/Engine/EditorBlueprintResources/StandardMacros.IsValid` _returnvalue
    (:`Is Valid`
      (`EnhancedInputSubsystemInterface.AddMappingContext` _returnvalue "/Game/_Jam_MilkyWay/Players/FirstPerson/Inputs/IMC_Default.IMC_Default" 0 (struct))
      (if (not (`EnhancedInputUserSettings.IsMappingContextRegistered` _returnvalue_2 "/Game/_Jam_MilkyWay/Players/FirstPerson/Inputs/IMC_Default.IMC_Default"))
        (`EnhancedInputUserSettings.RegisterInputMappingContext` _returnvalue_2 "/Game/_Jam_MilkyWay/Players/FirstPerson/Inputs/IMC_Default.IMC_Default"))
      (bind _returnvalue_3 (message `EnhancedInputSubsystemInterface.GetAllPlayerMappableActionKeyMappings` _returnvalue_2))
      (set `self.CurrentMappableActionKey` _returnvalue_3))))

(event `Toggle Proxi Chat`
  (params (`On/Off` :type Boolean))
  (bind _returnvalue (subsystem `OnsetVoipLocalPlayerSubsystem`))
  (`/Engine/EditorBlueprintResources/StandardMacros.IsValid` _returnvalue :!label _label_2
    (:`Is Valid`
      (if `On/Off`
        (`OnsetVoipLocalPlayerSubsystem.ToggleVoiceCaptureWithChannel` _returnvalue true 0)
        (else
          (`OnsetVoipLocalPlayerSubsystem.ToggleVoiceCaptureWithChannel` _returnvalue false 0))))
    (:`Is Not Valid`
      (`KismetSystemLibrary.Delay` 1.0)
      (goto _label_2))))

(event `Initialize VOIP`
  (params (`On/Off` :type Boolean))
  (bind _returnvalue (`OnsetVoipWorldSubsystem.GetVoipTalker` (subsystem `OnsetVoipWorldSubsystem`) (`self.PlayerState`)))
  (`self.PlayerState` :!label _label_3
    (:`then`
      (if `On/Off`
        (`OnsetVoipTalker.SetVoiceChannel` _returnvalue 0 true)
        (`self.Toggle Proxi Chat` true)
        (else
          (`OnsetVoipTalker.SetVoiceChannel` _returnvalue 0 false)
          (`self.Toggle Proxi Chat` false))))
    (:`else`
      (`KismetSystemLibrary.Delay` 0.5)
      (goto _label_3))))

(fn `UserConstructionScript`)