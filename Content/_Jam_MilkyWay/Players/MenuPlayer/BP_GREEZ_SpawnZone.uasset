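; BP_GREEZ_SpawnZone is a box zone actor for the lobby, apparently marking where GREEZ spawn.
; On BeginPlay it caches the game instance and registers itself on GS_Lobby as the GreezSpawnZone, so other code can find it through the game state.
; The construction script sizes the box from an exposed extent variable; the spawning logic itself lives outside this Blueprint.
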(event `self.ReceiveBeginPlay`
  (bind _asbp_game_instance (cast `/Game/_Jam_MilkyWay/Players/FirstPerson/Blueprints/BP_GameInstance` (`GameplayStatics.GetGameInstance`)))
  (set `self.As BP Game Instance` _asbp_game_instance)
  (bind _asgs_lobby (cast `/Game/_Jam_MilkyWay/Players/MenuPlayer/GS_Lobby` (`GameplayStatics.GetGameState`)))
  (bind _output_get (set `self.As GS Lobby` _asgs_lobby))
  (set `/Game/_Jam_MilkyWay/Players/MenuPlayer/GS_Lobby.GreezSpawnZone` self _output_get))

(fn `UserConstructionScript`
  (`BoxComponent.SetBoxExtent` (`self.Box`) (`self.In Box Extent`) true))