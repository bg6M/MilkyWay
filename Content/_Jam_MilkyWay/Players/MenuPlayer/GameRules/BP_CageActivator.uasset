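; Interactable cage terminal that lets a player open a code-entry console to trigger its linked cage trap, with outline and prompt shown only to the MANZ team.
; Server-side interaction, blocked once Greez can extract, records the user via RPC and multicast and opens the code widget.
; Activation fires the cage trap and animates the screen widget; exiting clears the user after a short delay.
; Calls to the camera view-target switch are left disconnected.
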(event `self.ReceiveBeginPlay`
  (bind _widget (`self.Widget`))
  (bind _screenwidget (`self.ScreenWidget`))
  (bind _asgs_lobby (cast `/Game/_Jam_MilkyWay/Players/MenuPlayer/GS_Lobby` (`GameplayStatics.GetGameState`)))
  (set `self.As GS Lobby` _asgs_lobby)
  (`/Engine/EditorBlueprintResources/ActorMacros.Switch Has Authority`
    (:`Authority`
      (bind _asw_cage_code_manz (cast `/Game/_Jam_MilkyWay/Players/MenuPlayer/GameWidgets/W_CageCodeManz` (`WidgetComponent.GetWidget` _screenwidget)))
      (bind _output_get (set `self.As W Cage Code Manz` _asw_cage_code_manz))
      (set `/Game/_Jam_MilkyWay/Players/MenuPlayer/GameWidgets/W_CageCodeManz.MyActor` self _output_get))
    (:`Remote`
      (bind _asw_cage_code_manz_2 (cast `/Game/_Jam_MilkyWay/Players/MenuPlayer/GameWidgets/W_CageCodeManz` (`WidgetComponent.GetUserWidgetObject` _screenwidget)))
      (bind _output_get_2 (set `self.As W Cage Code Manz` _asw_cage_code_manz_2))
      (set `/Game/_Jam_MilkyWay/Players/MenuPlayer/GameWidgets/W_CageCodeManz.MyActor` self _output_get_2)))
  (`/Engine/EditorBlueprintResources/ActorMacros.Switch Has Authority`
    (:`Authority`
      (bind _asw_interaction (cast `/Game/_Jam_MilkyWay/Players/MenuPlayer/GameWidgets/W_Interaction` (`WidgetComponent.GetWidget` _widget)))
      (set `self.As W Interaction` _asw_interaction))
    (:`Remote`
      (bind _asw_interaction_2 (cast `/Game/_Jam_MilkyWay/Players/MenuPlayer/GameWidgets/W_Interaction` (`WidgetComponent.GetUserWidgetObject` _widget)))
      (set `self.As W Interaction` _asw_interaction_2)))
  (`/Game/_Jam_MilkyWay/Players/MenuPlayer/GameWidgets/W_Interaction.SetDATA` (`self.As W Interaction`) "CAGE TERMINAL      " "Interact" false))

(event `/Game/_Jam_MilkyWay/Players/FirstPerson/Blueprints/Interface/BPI_Interaction.Interact_Int`
  (params (Bp_Player :type "/Game/_Jam_MilkyWay/Players/FirstPerson/Blueprints/BP_Player Object Reference"))
  (`/Engine/EditorBlueprintResources/ActorMacros.Switch Has Authority`
    (:`Authority`
      (if (not (`/Game/_Jam_MilkyWay/Players/MenuPlayer/GS_Lobby.GreezCanExtract` (`self.As GS Lobby`)))
        (`self.RPC_INTERACT` Bp_Player)
        (`/Game/_Jam_MilkyWay/Players/MenuPlayer/PC_Lobby.CreateCodeCageWidget` (`/Game/_Jam_MilkyWay/Players/FirstPerson/Blueprints/BP_Player.MyController` Bp_Player) self (`self.As W Cage Code Manz`))))))

(event `RPC_INTERACT`
  (params (`Bp Player` :type "/Game/_Jam_MilkyWay/Players/FirstPerson/Blueprints/BP_Player Object Reference"))
  (`self.MC_INTERACT` `Bp Player`))

(event `MC_INTERACT`
  (params (Target :type "/Game/_Jam_MilkyWay/Players/FirstPerson/Blueprints/BP_Player Object Reference"))
  (`/Engine/EditorBlueprintResources/StandardMacros.IsValid` (`self.Bp Player`)
    (:`Is Not Valid`
      (bind _output_get (set `self.Bp Player` Target))
      (set `/Game/_Jam_MilkyWay/Players/MenuPlayer/GameWidgets/W_CageCodeManz.MyPlayerController` (`/Game/_Jam_MilkyWay/Players/FirstPerson/Blueprints/BP_Player.MyController` _output_get) (`self.As W Cage Code Manz`)))))

(event `MC_ViewTarget`
  (params (`ON/OFF` :type Boolean))
  (bind _bp_player (`self.Bp Player`))
  (bind _widgetinteraction_pointer (`/Game/_Jam_MilkyWay/Players/FirstPerson/Blueprints/BP_Player.WidgetInteraction_POINTER` (`self.Bp Player`)))
  (if `ON/OFF`
    (`PlayerController.SetViewTargetWithBlend` (`/Game/_Jam_MilkyWay/Players/FirstPerson/Blueprints/BP_Player.MyController` (stale `MC_INTERACT` _output_get)) self 0.0 "VTBlend_Linear" 0.0 false)
    (`ActorComponent.Activate` _widgetinteraction_pointer true)
    (`/Game/_Jam_MilkyWay/Players/MenuPlayer/PC_Lobby.CreateCodeCageWidget` (`/Game/_Jam_MilkyWay/Players/FirstPerson/Blueprints/BP_Player.MyController` (`self.Bp Player`)) self null)
    (else
      (`PlayerController.SetViewTargetWithBlend` (`/Game/_Jam_MilkyWay/Players/FirstPerson/Blueprints/BP_Player.MyController` _bp_player) _bp_player 0.0 "VTBlend_Linear" 0.0 false)
      (`ActorComponent.Deactivate` _widgetinteraction_pointer))))

(event `ExitConsole`
  (set `self.IsUsed` false)
  (`KismetSystemLibrary.Delay` 0.2)
  (set `self.Bp Player` null))

(event `ACTIVATE`
  (`/Game/_Jam_MilkyWay/Players/MenuPlayer/GameRules/BP_Cage.RPC ACTIVE TRAP` (`self.MyCage`))
  (`/Game/_Jam_MilkyWay/Players/MenuPlayer/GameWidgets/W_CageCodeManz.ToggleOpenCageAnim` (`self.As W Cage Code Manz`)))

(event `/Game/_Jam_MilkyWay/Players/FirstPerson/Blueprints/Interface/BPI_Interaction.ToggleOutlineInteractible`
  (params (`Player Calling` :type "/Game/_Jam_MilkyWay/Players/FirstPerson/Blueprints/BP_Player Object Reference"))
  (switch `/Game/_Jam_MilkyWay/Players/MenuPlayer/E_PlayersTeam` (`/Game/_Jam_MilkyWay/Players/FirstPerson/Blueprints/BP_Player.Team` `Player Calling`)
    (:`NewEnumerator0`
      (`/Game/_Jam_MilkyWay/Players/FirstPerson/Blueprints/BP_Player.ACTIVATE OUTLINE` `Player Calling` true (`self.SkeletalMesh`)))))

(event `MC_TerminalSound`
  (params (`Good/Bad` :type Boolean))
  (bind _returnvalue (`self.K2_GetActorLocation`))
  (if `Good/Bad`
    (`GameplayStatics.PlaySoundAtLocation` "/Game/_Jam_MilkyWay/SFX/GPE/Terminal/Terminal_Granted__SFX.Terminal_Granted__SFX" _returnvalue (struct) 1.0 1.0 0.0 "/Game/_Jam_MilkyWay/SFX/Attenuation_Types/SA_VOIP.SA_VOIP" null null null)
    (else
      (`GameplayStatics.PlaySoundAtLocation` "/Game/_Jam_MilkyWay/SFX/GPE/Terminal/Terminal_Denied__SFX.Terminal_Denied__SFX" _returnvalue (struct) 1.0 1.0 0.0 "/Game/_Jam_MilkyWay/SFX/Attenuation_Types/SA_VOIP.SA_VOIP" null null null))))

(event `/Game/_Jam_MilkyWay/Players/FirstPerson/Blueprints/Interface/BPI_Interaction.ToggleWidget`
  (params (`On/Off` :type Boolean) (PlayerCallingWidget :type "/Game/_Jam_MilkyWay/Players/FirstPerson/Blueprints/BP_Player Object Reference"))
  (`/Engine/EditorBlueprintResources/StandardMacros.IsValid` PlayerCallingWidget
    (:`Is Valid`
      (switch `/Game/_Jam_MilkyWay/Players/MenuPlayer/E_PlayersTeam` (`/Game/_Jam_MilkyWay/Players/FirstPerson/Blueprints/BP_Player.Team` PlayerCallingWidget)
        (:`NewEnumerator0`
          (`/Game/_Jam_MilkyWay/Players/FirstPerson/Blueprints/BP_Player.Activate E Wdiget` PlayerCallingWidget `On/Off` (`self.Widget`)))))))

(fn `UserConstructionScript`)