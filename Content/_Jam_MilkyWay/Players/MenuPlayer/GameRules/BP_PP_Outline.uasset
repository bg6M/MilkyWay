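; Post-process actor for the lobby that drives an outline selector material and registers itself with GS_Lobby as MyPPActor.
; On BeginPlay it creates a dynamic instance of the outline material at a default dimmed color intensity and assigns it as the PostProcess component's only blendable.
; SetOutlineIntensity toggles that intensity between full and dimmed, then reapplies the post-process settings.
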(event `self.ReceiveBeginPlay`
  (bind _asgs_lobby (cast `/Game/_Jam_MilkyWay/Players/MenuPlayer/GS_Lobby` (`GameplayStatics.GetGameState`)))
  (bind _output_get (set `self.As GS Lobby` _asgs_lobby))
  (set `/Game/_Jam_MilkyWay/Players/MenuPlayer/GS_Lobby.MyPPActor` self _output_get)
  (set `self.ColorIntensityValue` 0.6)
  (bind _returnvalue (`KismetMaterialLibrary.CreateDynamicMaterialInstance` "/Game/ConceptArtShaders/Post_Process_Materials/Materials/PP_OutlinesSelector_Inst1.PP_OutlinesSelector_Inst1"))
  (bind _output_get_2 (set `self.NewDynamicMaterialInstance` _returnvalue))
  (`MaterialInstanceDynamic.SetScalarParameterValue` _output_get_2 "ColorIntensity" (`self.ColorIntensityValue`))
  (set `PostProcessComponent.Settings` (make `PostProcessSettings` :`WeightedBlendables` (make `WeightedBlendables` (`|MakeArray` (make `WeightedBlendable` 1.0 _output_get_2)))) (`self.PostProcess`)))

(event `SetOutlineIntensity`
  (params (`Max/Default` :type Boolean))
  (bind _newdynamicmaterialinstance (`self.NewDynamicMaterialInstance`))
  (if `Max/Default`
    (set `self.ColorIntensityValue` 1.0)
    (else
      (set `self.ColorIntensityValue` 0.6)))
  (`MaterialInstanceDynamic.SetScalarParameterValue` _newdynamicmaterialinstance "ColorIntensity" (`self.ColorIntensityValue`))
  (set `PostProcessComponent.Settings` (make `PostProcessSettings` :`WeightedBlendables` (make `WeightedBlendables` (`|MakeArray` (make `WeightedBlendable` 1.0 _newdynamicmaterialinstance)))) (`self.PostProcess`)))

(fn `UserConstructionScript`)