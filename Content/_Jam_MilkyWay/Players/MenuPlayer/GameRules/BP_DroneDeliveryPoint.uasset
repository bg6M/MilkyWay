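; Lobby delivery point that flies a drone over its location to drop a replicated BP_Dropbox, registering itself with GS_Lobby on BeginPlay.
; ServerAppear builds a three-point spline swooping down over the point, then runs a timeline that moves and tilts the drone through UFOAPPEAR.
; A timeline event spawns the box just below the drone.
; The IsActive RepNotify toggles drone visibility and sound for the duration of the flight.
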(event `self.ReceiveBeginPlay`
  (bind _asbp_game_instance (cast `/Game/_Jam_MilkyWay/Players/FirstPerson/Blueprints/BP_GameInstance` (`GameplayStatics.GetGameInstance`)))
  (set `self.As BP Game Instance` _asbp_game_instance)
  (bind _asgs_lobby (cast `/Game/_Jam_MilkyWay/Players/MenuPlayer/GS_Lobby` (`GameplayStatics.GetGameState`)))
  (bind _output_get (set `self.As GS Lobby` _asgs_lobby))
  (`KismetArrayLibrary.Array_Add` (`/Game/_Jam_MilkyWay/Players/MenuPlayer/GS_Lobby.MyDrones` _output_get) self))

(event `UFO APPEAR`
  (params (NewLocation :type "Vector Structure") (NewRotation :type "Rotator Structure") (`New Rotation X (Roll)` :type "Float (single-precision)") (`New Rotation Y (Pitch)` :type "Float (single-precision)"))
  (bind _drone (`self.Drone`))
  (`SceneComponent.K2_SetWorldLocationAndRotation` _drone NewLocation NewRotation false false)
  (`SceneComponent.K2_SetRelativeRotation` _drone (`KismetMathLibrary.MakeRotator` `New Rotation X (Roll)` `New Rotation Y (Pitch)`) false false))

(event `ServerAppear`
  (bind _myspline (`self.MySpline`))
  (set `self.IsActive` true)
  (bind _success (`self.SetSpline`))
  (if _success
    (bind (_direction _distance_on_spline _relative_roll_n_pitch) (`Timeline|Timeline` :!via `PlayFromStart`)
      (:`Update`
        (bind _returnvalue (* (`SplineComponent.GetSplineLength` _myspline) _distance_on_spline))
        (bind (_returnvalue_roll _returnvalue_pitch _returnvalue_yaw) (`KismetMathLibrary.BreakRotator` (`SplineComponent.GetRotationAtDistanceAlongSpline` _myspline _returnvalue "World")))
        (`self.UFO APPEAR` (`SplineComponent.GetLocationAtDistanceAlongSpline` _myspline _returnvalue "World") (`KismetMathLibrary.MakeRotator` _returnvalue_roll _returnvalue_pitch _returnvalue_yaw) (.x _relative_roll_n_pitch) (.y _relative_roll_n_pitch)))
      (:`Finished`
        (set `self.IsActive` false))
      (:`DropDuhBox`
        (`self.Spawn DropBox`)))))

(event `Spawn DropBox`
  (bind _returnvalue (`|SpawnActorFromClass` "/Game/_Jam_MilkyWay/Gpe/Dropbox/BP_Dropbox.BP_Dropbox_C" (`KismetMathLibrary.MakeTransform` (- (`SceneComponent.K2_GetComponentLocation` (`self.Drone`)) (0.0 0.0 20.0)) (`SceneComponent.K2_GetComponentRotation` (`self.Sphere`))) "Undefined" "MultiplyWithRoot" null "NewEnumerator0" null))
  (`self.SetReplicates` _returnvalue true))

(fn `OnRep_IsActive`
  (bind _drone (`self.Drone`))
  (bind _drone_sfx_cue (`self.Drone_SFX_Cue`))
  (if (`self.IsActive`)
    (`SceneComponent.SetHiddenInGame` _drone false false)
    (`AudioComponent.Play` _drone_sfx_cue 0.0)
    (else
      (`SceneComponent.SetHiddenInGame` _drone true false)
      (`AudioComponent.Stop` _drone_sfx_cue))))

(fn `SetSpline`
  (returns (Success :type Boolean))
  (bind _returnvalue (`SceneComponent.K2_GetComponentLocation` (`self.Sphere`)))
  (bind _array (`|MakeArray` (+ _returnvalue (2500.0 -10000.0 6000.0)) (+ _returnvalue (0.0 0.0 600.0)) (+ _returnvalue (-2500.0 16000.0 6000.0))))
  (set `self.Spline Array` _array)
  (bind _returnvalue_2 (`AddComponent|NODE_AddSplineComponent-0`))
  (bind _output_get (set `self.MySpline` _returnvalue_2))
  (`SplineComponent.SetSplinePoints` _output_get _array "World" true)
  (return true))

(fn `UserConstructionScript`)