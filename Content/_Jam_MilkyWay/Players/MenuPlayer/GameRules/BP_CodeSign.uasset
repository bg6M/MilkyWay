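; BP_CodeSign is a grabbable, physics-driven notepad sign in the lobby, registered on the server in GS_Lobby's code sign bank.
; Grab and ungrab interface calls pass through RPC events that set IsGrabed, switch collision and, on grab, set the holder's team-specific spring arm length.
; IsGrabed's RepNotify toggles physics, damping velocity on release.
; Server_Destroy removes the actor; following the holder is not handled here.
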(event Custom|RPC%20GRAB
  (params (Target :type BP%20Player%20Object%20Reference))
  (Variables|Default|SetIsGrabed true)
  (Collision|SetCollisionEnabled (Variables|Default|GetSM_Notepad) "PhysicsOnly")
  (switch Utilities|FlowControl|Switch|SwitchonE_PlayersTeam (Variables|/Game/_Jam_MilkyWay/Players/FirstPerson/Blueprints/BP_Player.BP_Player_C|GetTeam Target)
    (:NewEnumerator0
      (Variables|/Script/Engine.SpringArmComponent|SetTargetArmLength (Variables|/Game/_Jam_MilkyWay/Players/FirstPerson/Blueprints/BP_Player.BP_Player_C|GetManzGrabSpringArm Target) -1e+02))
    (:NewEnumerator1
      (Variables|/Script/Engine.SpringArmComponent|SetTargetArmLength (Variables|/Game/_Jam_MilkyWay/Players/FirstPerson/Blueprints/BP_Player.BP_Player_C|GetGrabSpringArm Target) -2e+02))))

(event Custom|RPC%20UNGRAB
  (Variables|Default|SetIsGrabed false)
  (Collision|SetCollisionEnabled (Variables|Default|GetSM_Notepad) "QueryAndPhysics")
  (Variables|Default|SetPlayer%20Calling%20Grab 0))

(event Custom|ServerRPCGRAB
  (params (Player%20Calling%20Grab :type BP%20Player%20Object%20Reference))
  (CallFunction|RPCGRAB Player%20Calling%20Grab))

(event Custom|SERVER%20RPC%20UNGRAB
  (CallFunction|RPCUNGRAB))

(event Custom|Server_Destroy
  (Actor|DestroyActor))

(event EventBeginPlay
  (Networking|SwitchHasAuthority
    (:Authority
      (bind _asgs_lobby (Utilities|Casting|CastToGS_Lobby (Game|GetGameState)))
      (bind _output_get (Variables|Default|SetAs%20GS%20Lobby _asgs_lobby))
      (Utilities|Array|Add (Variables|/Game/_Jam_MilkyWay/Players/MenuPlayer/GS_Lobby.GS_Lobby_C|GetMyCodeSignBank _output_get) self)
      (Physics|SetSimulatePhysics (Variables|Default|GetSM_Notepad) true))))

(event EventGrabInterface
  (params (Player%20calling%20grab :type BP%20Player%20Object%20Reference) (PlayerTeam :type E_PlayersTeam%20Enum :default "NewEnumerator0"))
  (Networking|SwitchHasAuthority
    (:Authority
      (bind _output_get (Variables|Default|SetPlayer%20Calling%20Grab Player%20calling%20grab))
      (CallFunction|ServerRPCGRAB _output_get))))

(event EventUnGrabInterface
  (params (Player%20Calling%20Grab :type BP%20Player%20Object%20Reference) (Bump? :type Boolean) (ControllerCallingBump :type PC%20Lobby%20Object%20Reference))
  (CallFunction|SERVERRPCUNGRAB))

(fn ConstructionScript)

(fn OnRepIsGrabed
  (bind _sm_notepad (Variables|Default|GetSM_Notepad))
  (bind _sm_notepad_2 (Variables|Default|GetSM_Notepad))
  (if (Variables|Default|GetIsGrabed)
    (Physics|SetSimulatePhysics _sm_notepad false)
    (else
      (Physics|SetSimulatePhysics _sm_notepad true)
      (Physics|SetPhysicsLinearVelocity _sm_notepad_2 (* (Transformation|GetComponentVelocity _sm_notepad_2) 0.2) false "None"))))