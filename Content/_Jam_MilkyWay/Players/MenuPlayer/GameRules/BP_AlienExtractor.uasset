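; Extraction objective actor where the GREEZ team tries to escape through a pod, King-of-the-Hill style, before time runs out.
; IsActive's RepNotify starts timeline-driven mothership warp and shuttle descent, then opens the overlap zone and unpauses a one-second timer.
; GREEZ presence raises the score and absence drains it, shown on the shuttle material, until GameState's ManzWin settles the match.
; RepNotifies and multicasts sync visuals and audio, and two world clock widgets reference the actor.
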(event `self.ReceiveBeginPlay`
  (bind _as_gs_lobby (`self.As GS Lobby`))
  (bind _timerclock1 (`self.TIMERCLOCK1`))
  (bind _timerclock2 (`self.TIMERCLOCK2`))
  (`/Engine/EditorBlueprintResources/ActorMacros.Switch Has Authority`
    (:`Authority`
      (bind _asw_koth_timer (cast `/Game/_Jam_MilkyWay/Players/MenuPlayer/GameWidgets/W_KOTH_Timer` (`WidgetComponent.GetWidget` _timerclock1)))
      (set `self.As W KOTH Timer` _asw_koth_timer)
      (bind _asw_koth_timer_2 (cast `/Game/_Jam_MilkyWay/Players/MenuPlayer/GameWidgets/W_KOTH_Timer` (`WidgetComponent.GetWidget` _timerclock2)))
      (set `self.As W KOTH Timer_2` _asw_koth_timer_2))
    (:`Remote`
      (bind _asw_koth_timer_3 (cast `/Game/_Jam_MilkyWay/Players/MenuPlayer/GameWidgets/W_KOTH_Timer` (`WidgetComponent.GetUserWidgetObject` _timerclock1)))
      (set `self.As W KOTH Timer` _asw_koth_timer_3)
      (bind _asw_koth_timer_4 (cast `/Game/_Jam_MilkyWay/Players/MenuPlayer/GameWidgets/W_KOTH_Timer` (`WidgetComponent.GetUserWidgetObject` _timerclock2)))
      (set `self.As W KOTH Timer_2` _asw_koth_timer_4)))
  (set `/Game/_Jam_MilkyWay/Players/MenuPlayer/GameWidgets/W_KOTH_Timer.MyParent` self (`self.As W KOTH Timer`))
  (set `/Game/_Jam_MilkyWay/Players/MenuPlayer/GameWidgets/W_KOTH_Timer.MyParent` self (`self.As W KOTH Timer_2`))
  (bind _asgs_lobby (cast `/Game/_Jam_MilkyWay/Players/MenuPlayer/GS_Lobby` (`GameplayStatics.GetGameState`)))
  (bind _output_get (set `self.As GS Lobby` _asgs_lobby))
  (set `/Game/_Jam_MilkyWay/Players/MenuPlayer/GS_Lobby.MyExtractor` self _output_get)
  (`KismetSystemLibrary.Delay` 2.0)
  (`self.ServerArrival`)
  (bind _returnvalue (`KismetSystemLibrary.K2_SetTimerDelegate` (delegate `Add Score`) 1.0 true true))
  (bind _output_get_2 (set `self.TimerGreezScore` _returnvalue))
  (`KismetSystemLibrary.K2_PauseTimerHandle` _output_get_2)
  (`/Game/_Jam_MilkyWay/Players/MenuPlayer/GS_Lobby.Server Call Game State Message` _as_gs_lobby "NewEnumerator0" "The End is near..." 4.0 0.0)
  (`/Game/_Jam_MilkyWay/Players/MenuPlayer/GS_Lobby.Server Call Game State Message` _as_gs_lobby "NewEnumerator1" "MOTHERSHIP SUCCESSFULLY BREACHED." 4.0 0.0))

(event `ServerArrival`
  (set `self.IsActive` true)
  (`self.MC_SETShuffleINTENSITY` false)
  (`self.MC_ExtractionJauge`))

(event `RPCArrival`
  (params (Alpha :type "Float (single-precision)"))
  (`SceneComponent.K2_SetWorldLocation` (`self.SKM_Shuttle`) (`KismetMathLibrary.VLerp` (`SceneComponent.K2_GetComponentLocation` (`self.MotherShip`)) (`SceneComponent.K2_GetComponentLocation` (`self.Sphere`)) Alpha) false false))

(event `self.Sphere.OnComponentBeginOverlap`
  (params (OverlappedComponent :type "PrimitiveComponent Object Reference") (OtherActor :type "Actor Object Reference") (OtherComp :type "PrimitiveComponent Object Reference") (OtherBodyIndex :type Integer) (bFromSweep :type Boolean) (SweepResult :type "HitResult Structure (by ref)"))
  (if (`self.CanEscape`)
    (`self.ServerOverlapp` OtherActor)))

(event `MC SPACEJUMP`
  (bind _as_gs_lobby (`self.As GS Lobby`))
  (`GameplayStatics.PlaySound2D` "/Game/_Jam_MilkyWay/SFX/UFO/UFO_MotherShip_Warp_SFX.UFO_MotherShip_Warp_SFX" 1.0 1.0 0.0 null null)
  (bind (_direction _alpha _alpha2) (`Timeline|MotherShipEntrance` :!via `PlayFromStart`)
    (:`Update`
      (`self.MC MOTHERSHIP APPEAR` _alpha _alpha2))
    (:`Finished`
      (bind (_direction_2 _alpha_2) (`Timeline|Arrival` :!via `PlayFromStart`)
        (:`Update`
          (`self.RPCArrival` _alpha_2))
        (:`Finished`
          (set `self.CanEscape` true)
          (`/Game/_Jam_MilkyWay/Players/MenuPlayer/GS_Lobby.Server Call Game State Message` _as_gs_lobby "NewEnumerator0" "Secure the escape pod, prevent the Intruder to LEAVE !" 6.0 0.0)
          (`/Game/_Jam_MilkyWay/Players/MenuPlayer/GS_Lobby.Server Call Game State Message` _as_gs_lobby "NewEnumerator1" "REACH THE POD TO COME BACK HOME." 6.0 0.0)
          (`KismetSystemLibrary.K2_UnPauseTimerHandle` (`self.TimerGreezScore`))
          (`GameplayStatics.PlaySound2D` "/Game/_Jam_MilkyWay/Musics/MainTheme.MainTheme" 1.0 1.0 0.0 null null))))))

(event `MC MOTHERSHIP APPEAR`
  (params (Alpha :type "Float (single-precision)") (Alpha2 :type "Float (single-precision)"))
  (`SceneComponent.K2_SetRelativeTransform` (`self.MotherShip`) (`KismetMathLibrary.MakeTransform` (`KismetMathLibrary.VLerp` (-400000.0 0.0 40000.0) (0.0 0.0 40000.0) Alpha2) (struct) (`KismetMathLibrary.VLerp` (100.0 0.1 10.0) (10.0 10.0 10.0) Alpha)) false false))

(event `ServerOverlapp`
  (params (ActorOverlap :type "Actor Object Reference"))
  (bind _asbp_player (cast `/Game/_Jam_MilkyWay/Players/FirstPerson/Blueprints/BP_Player` ActorOverlap))
  (switch `/Game/_Jam_MilkyWay/Players/MenuPlayer/E_PlayersTeam` (`/Game/_Jam_MilkyWay/Players/FirstPerson/Blueprints/BP_Player.Team` _asbp_player)
    (:`NewEnumerator1`
      (`KismetArrayLibrary.Array_Add` (`self.PlayerInZone`) (`Pawn.PlayerState` _asbp_player))
      (set `self.GreezInZone` true)
      (`self.MC_SETShuffleINTENSITY` true))))

(event `MC_SETShuffleINTENSITY`
  (params (`ON/OFF` :type Boolean))
  (if `ON/OFF`
    (`MeshComponent.SetScalarParameterValueOnMaterials` (`self.SKM_Shuttle`) "Intensity" 0.3)
    (else
      (`MeshComponent.SetScalarParameterValueOnMaterials` (`self.SKM_Shuttle`) "Intensity" 0.0))))

(event `self.Sphere.OnComponentEndOverlap`
  (params (OverlappedComponent :type "PrimitiveComponent Object Reference") (OtherActor :type "Actor Object Reference") (OtherComp :type "PrimitiveComponent Object Reference") (OtherBodyIndex :type Integer))
  (if (`self.CanEscape`)
    (`self.Server_End Overlapp` OtherActor)))

(event `Server_End Overlapp`
  (params (ActorOverlap :type "Actor Object Reference"))
  (bind _asbp_player (cast `/Game/_Jam_MilkyWay/Players/FirstPerson/Blueprints/BP_Player` ActorOverlap))
  (switch `/Game/_Jam_MilkyWay/Players/MenuPlayer/E_PlayersTeam` (`/Game/_Jam_MilkyWay/Players/FirstPerson/Blueprints/BP_Player.Team` _asbp_player)
    (:`NewEnumerator1`
      (`KismetArrayLibrary.Array_RemoveItem` (`self.PlayerInZone`) (`Pawn.PlayerState` _asbp_player))
      (set `self.GreezInZone` false)
      (`self.MC_SETShuffleINTENSITY` false))))

(event `Add Score`
  (bind _as_gs_lobby (`self.As GS Lobby`))
  (bind _kothcurrentscore (`self.KOTHCurrentScore`))
  (bind _result (`/Engine/EditorBlueprintResources/StandardMacros.DecrementInt` (`self.Timer`))
    (:`  `
      (bind _output_get (set `self.Timer` _result))
      (if (<= _output_get 0)
        (bind _returnvalue (>= (stale _output_get_2) (`self.KOTHMAXSCORE`)))
        (if _returnvalue
          (if _returnvalue :!label _label
            (`/Engine/EditorBlueprintResources/StandardMacros.DoOnce` false
              (:`Completed`
                (`/Game/_Jam_MilkyWay/Players/MenuPlayer/GS_Lobby.ManzWin` _as_gs_lobby false)))
            (else
              (`self.MC_ExtractionJauge` :!label _label_2)))
          (else
            (`/Engine/EditorBlueprintResources/StandardMacros.DoOnce` false
              (:`Completed`
                (`/Game/_Jam_MilkyWay/Players/MenuPlayer/GS_Lobby.ManzWin` _as_gs_lobby true)))))
        (elif (`self.GreezInZone`)
          (bind _output_get_2 (set `self.KOTHCurrentScore` (`KismetMathLibrary.FClamp` (+ (`self.KOTHCurrentScore`) 1.0) 0.0 20.0)))
          (goto _label)
          (elif (> _kothcurrentscore 0.0)
            (set `self.KOTHCurrentScore` (`KismetMathLibrary.FClamp` (- _kothcurrentscore 0.5) 0.0 20.0))
            (goto _label_2)))))))

(event `MC_ExtractionJauge`
  (`MeshComponent.SetScalarParameterValueOnMaterials` (`self.SKM_Shuttle`) "JuiceQuantity" (`KismetMathLibrary.NormalizeToRange` (* (`self.KOTHCurrentScore`) -1.0) 0.0 (* (`self.KOTHMAXSCORE`) -1.0))))

(fn `OnRep_CanEscape`
  (bind _sphere (`self.Sphere`))
  (if (`self.CanEscape`)
    (`PrimitiveComponent.SetCollisionResponseToChannel` _sphere "ECC_Pawn" "ECR_Overlap")
    (`SceneComponent.SetHiddenInGame` (`self.FX_OvniBeam_CastingTime`) false false)
    (else
      (`PrimitiveComponent.SetCollisionResponseToChannel` _sphere "ECC_Pawn" "ECR_Ignore"))))

(fn `OnRep_GreezInZone`
  (bind _koth_aliendetect_sfx (`self.KOTH_AlienDetect_SFX`))
  (if (`self.GreezInZone`)
    (`AudioComponent.Play` _koth_aliendetect_sfx 0.0)
    (else
      (`AudioComponent.Stop` _koth_aliendetect_sfx))))

(fn `OnRep_IsActive`
  (bind _mothership (`self.MotherShip`))
  (if (`self.IsActive`)
    (`SceneComponent.SetHiddenInGame` _mothership false false)
    (`self.MC SPACEJUMP`)
    (else
      (`SceneComponent.SetHiddenInGame` _mothership true false))))

(fn `OnRep_KOTHCurrentScore`)

(fn `UserConstructionScript`)