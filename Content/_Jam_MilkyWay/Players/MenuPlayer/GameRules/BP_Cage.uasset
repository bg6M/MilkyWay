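; BP_Cage is an interactable trap that captures Greez-team players and triggers the Manz team's win.
; Interaction arms it for 30 seconds; a Greez player from the lobby list who overlaps the box meanwhile is ungrabbed, teleported inside, immobilized and attached.
; RepNotifies on IsActive and MANZWIN report the win to GS_Lobby and call RPC events that forward to MC events.
; These play foghorn audio and drive material parameters, partly through timelines.
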(event `self.ReceiveBeginPlay`
  (bind _asbp_game_instance (cast `/Game/_Jam_MilkyWay/Players/FirstPerson/Blueprints/BP_GameInstance` (`GameplayStatics.GetGameInstance`)))
  (set `self.As BP Game Instance` _asbp_game_instance)
  (bind _asgs_lobby (cast `/Game/_Jam_MilkyWay/Players/MenuPlayer/GS_Lobby` (`GameplayStatics.GetGameState`)))
  (set `self.As GS Lobby` _asgs_lobby)
  (`self.RPC OPEN CAGE` true))

(event `/Game/_Jam_MilkyWay/Players/FirstPerson/Blueprints/Interface/BPI_Interaction.Interact_Int`
  (params (Bp_Player :type "/Game/_Jam_MilkyWay/Players/FirstPerson/Blueprints/BP_Player Object Reference"))
  (`self.RPC ACTIVE TRAP`))

(event `RPC ACTIVE TRAP`
  (if (not (`self.IsActive`))
    (set `self.IsActive` true)
    (`KismetSystemLibrary.Delay` 30.0)
    (set `self.IsActive` false)))

(event `self.Box.OnComponentBeginOverlap`
  (params (OverlappedComponent :type "PrimitiveComponent Object Reference") (OtherActor :type "Actor Object Reference") (OtherComp :type "PrimitiveComponent Object Reference") (OtherBodyIndex :type Integer) (bFromSweep :type Boolean) (SweepResult :type "HitResult Structure (by ref)"))
  (if (`self.IsActive`)
    (`self.AlienServerOverlapp` OtherActor)))

(event `AlienServerOverlapp`
  (params (ActorOverlap :type "Actor Object Reference"))
  (bind _asbp_player (cast `/Game/_Jam_MilkyWay/Players/FirstPerson/Blueprints/BP_Player` ActorOverlap))
  (switch `/Game/_Jam_MilkyWay/Players/MenuPlayer/E_PlayersTeam` (`/Game/_Jam_MilkyWay/Players/FirstPerson/Blueprints/BP_Player.Team` _asbp_player)
    (:`NewEnumerator1`
      (for _array_element (`/Game/_Jam_MilkyWay/Players/MenuPlayer/GS_Lobby.Greez` (`self.As GS Lobby`))
        (if (== _array_element _asbp_player)
          (set `self.MANZWIN` true)
          (message `/Game/_Jam_MilkyWay/Players/FirstPerson/Blueprints/Interface/BPI_Grab.UnGrab Interface` _array_element)
          (`self.RPC CLOSE CAGE` _array_element))))))

(event `RPC CLOSE CAGE`
  (params (`BP PLAYER` :type "/Game/_Jam_MilkyWay/Players/FirstPerson/Blueprints/BP_Player Object Reference"))
  (bind _charactermovement (`Character.CharacterMovement` `BP PLAYER`))
  (`self.MC CLOSE CAGE` `BP PLAYER`)
  (`self.K2_TeleportTo` :`self` (stale `MC CLOSE CAGE` `BP PLAYER`) :`DestLocation` (`SceneComponent.K2_GetComponentLocation` (`self.GreezCaptureLocation`)))
  (`MovementComponent.StopMovementImmediately` _charactermovement)
  (`CharacterMovementComponent.DisableMovement` _charactermovement)
  (`self.K2_AttachToActor` `BP PLAYER` self "None" "KeepWorld" "KeepWorld" "KeepWorld" true)
  (`GameplayStatics.PlaySound2D` "/Game/_Jam_MilkyWay/Musics/ChestOpening.ChestOpening" 1.0 1.0 0.0 null null))

(event `RPC ACTIVE CAGE`
  (params (`Open/Close` :type Boolean))
  (`self.MC ACTIVE CAGE` `Open/Close`))

(event `MC CLOSE CAGE`
  (params (`BP PLAYER` :type "/Game/_Jam_MilkyWay/Players/FirstPerson/Blueprints/BP_Player Object Reference"))
  (bind (_direction _alpha) (`Timeline|CLOSECAGE` :!via `PlayFromStart`)
    (:`Update`
      (`MeshComponent.SetScalarParameterValueOnMaterials` (`self.StaticMesh`) "GlobalOpacity" _alpha))))

(event `RPC OPEN CAGE`
  (params (`Open/Close` :type Boolean))
  (`self.MC OPEN CAGE` `Open/Close`))

(event `MC OPEN CAGE`
  (params (`Open/Close` :type Boolean))
  (bind _staticmesh (`self.StaticMesh`))
  (if `Open/Close`
    (bind (_direction _wavefadein _wavefadeout) (`Timeline|OpenCage` :!via `PlayFromStart` :!label _label)
      (:`Update`
        (`MeshComponent.SetScalarParameterValueOnMaterials` _staticmesh "WaveFadeIn" _wavefadein)
        (`MeshComponent.SetScalarParameterValueOnMaterials` _staticmesh "WaveFadeOut" _wavefadeout)))
    (else
      (goto _label :!via `ReverseFromEnd`))))

(event `MC ACTIVE CAGE`
  (params (Condition :type Boolean))
  (bind _staticmesh (`self.StaticMesh`))
  (if Condition
    (`MeshComponent.SetScalarParameterValueOnMaterials` _staticmesh "Intensity" 10.0)
    (`GameplayStatics.PlaySoundAtLocation` "/Game/_Jam_MilkyWay/SFX/Foleys/Horns/loud-fog-horn-47514.loud-fog-horn-47514" (`self.K2_GetActorLocation`) (struct) 1.0 1.0 0.0 "/Game/_Jam_MilkyWay/SFX/Attenuation_Types/Far_SoundAttenuation.Far_SoundAttenuation" null null null)
    (else
      (`MeshComponent.SetScalarParameterValueOnMaterials` _staticmesh "Intensity" 0.0))))

(fn `OnRep_IsActive`
  (`self.RPC ACTIVE CAGE` (`self.IsActive`))
  (`self.RPC OPEN CAGE` true))

(fn `OnRep_MANZWIN`
  (`/Game/_Jam_MilkyWay/Players/MenuPlayer/GS_Lobby.ManzWin` (`self.As GS Lobby`) true)
  (`self.RPC OPEN CAGE` false))

(fn `UserConstructionScript`)