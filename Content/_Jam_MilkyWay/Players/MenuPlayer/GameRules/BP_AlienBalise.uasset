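; Delivery beacon objective that only Greez-team players can see outlined and interact with, registered in the lobby GameState on BeginPlay.
; Interacting with an active beacon starts a server-gated alien QTE on the player's controller.
; Success increments BeaconScore and resets objectives; failure waits a random delay, then reactivates the beacon unless an objective exists.
; Activation is relayed through each Greez player to show or hide the mesh and sound.
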(event `/Game/_Jam_MilkyWay/Players/FirstPerson/Blueprints/Interface/BPI_Interaction.ToggleOutlineInteractible`
  (params (`Player Calling` :type "/Game/_Jam_MilkyWay/Players/FirstPerson/Blueprints/BP_Player Object Reference"))
  (if (`self.IsActive`)
    (switch `/Game/_Jam_MilkyWay/Players/MenuPlayer/E_PlayersTeam` (`/Game/_Jam_MilkyWay/Players/FirstPerson/Blueprints/BP_Player.Team` `Player Calling`)
      (:`NewEnumerator1`
        (`/Game/_Jam_MilkyWay/Players/FirstPerson/Blueprints/BP_Player.ACTIVATE OUTLINE` `Player Calling` true (`self.Mailbox`))))))

(event `/Game/_Jam_MilkyWay/Players/FirstPerson/Blueprints/Interface/BPI_Interaction.ToggleWidget`
  (params (`On/Off` :type Boolean) (PlayerCallingWidget :type "/Game/_Jam_MilkyWay/Players/FirstPerson/Blueprints/BP_Player Object Reference"))
  (if (`self.IsActive`)
    (`/Engine/EditorBlueprintResources/StandardMacros.IsValid` PlayerCallingWidget
      (:`Is Valid`
        (switch `/Game/_Jam_MilkyWay/Players/MenuPlayer/E_PlayersTeam` (`/Game/_Jam_MilkyWay/Players/FirstPerson/Blueprints/BP_Player.Team` PlayerCallingWidget)
          (:`NewEnumerator1`
            (`/Game/_Jam_MilkyWay/Players/FirstPerson/Blueprints/BP_Player.Activate E Wdiget` PlayerCallingWidget `On/Off` (`self.Widget`))))))))

(event `self.ReceiveBeginPlay`
  (bind _widget (`self.Widget`))
  (bind _asgs_lobby (cast `/Game/_Jam_MilkyWay/Players/MenuPlayer/GS_Lobby` (`GameplayStatics.GetGameState`)))
  (bind _output_get (set `self.As GS Lobby` _asgs_lobby))
  (`KismetArrayLibrary.Array_Add` (`/Game/_Jam_MilkyWay/Players/MenuPlayer/GS_Lobby.MyAlienBalise` _output_get) self)
  (`/Engine/EditorBlueprintResources/ActorMacros.Switch Has Authority`
    (:`Authority`
      (bind _asw_interaction (cast `/Game/_Jam_MilkyWay/Players/MenuPlayer/GameWidgets/W_Interaction` (`WidgetComponent.GetWidget` _widget)))
      (set `self.As W Interaction` _asw_interaction))
    (:`Remote`
      (bind _asw_interaction_2 (cast `/Game/_Jam_MilkyWay/Players/MenuPlayer/GameWidgets/W_Interaction` (`WidgetComponent.GetUserWidgetObject` _widget)))
      (set `self.As W Interaction` _asw_interaction_2)))
  (`/Game/_Jam_MilkyWay/Players/MenuPlayer/GameWidgets/W_Interaction.SetDATA` (`self.As W Interaction`) "DELIVERY BEACON " "INTERACT" true))

(event `Server_QTESUccessCheck`
  (params (Condition :type Boolean))
  (`KismetSystemLibrary.PrintString` (`KismetStringLibrary.Concat_StrStr` "Server_QTESuccessCheck" "//" "" "Condition =" (`KismetStringLibrary.Conv_BoolToString` Condition))))

(event `/Game/_Jam_MilkyWay/Players/FirstPerson/Blueprints/Interface/BPI_Interaction.Interact_Int`
  (params (Bp_Player :type "/Game/_Jam_MilkyWay/Players/FirstPerson/Blueprints/BP_Player Object Reference"))
  (switch `/Game/_Jam_MilkyWay/Players/MenuPlayer/E_PlayersTeam` (`/Game/_Jam_MilkyWay/Players/FirstPerson/Blueprints/BP_Player.Team` Bp_Player)
    (:`NewEnumerator1`
      (`self.RPC_Interaction` Bp_Player))))

(event `/Game/_Jam_MilkyWay/Players/FirstPerson/Blueprints/Interface/BPI_Interaction.QTE SUCCESS CHECK`
  (params (`Actor to Trigger` :type "Actor Object Reference") (`Success?` :type Boolean) (AlienBalise :type "/Game/_Jam_MilkyWay/Players/MenuPlayer/GameRules/BP_AlienBalise Object Reference"))
  (if `Success?`
    (`self.SERVER QTE WIN` (`self.Player Ref`))
    (else
      (set `self.HasBeenUsed` true)
      (`KismetSystemLibrary.Delay` (`KismetMathLibrary.RandomFloatInRange` 30.0 60.0))
      (if (`/Game/_Jam_MilkyWay/Players/MenuPlayer/GS_Lobby.HaveObjective?` (`self.As GS Lobby`))
        (`self.ServerActivateAlienBalise` false (`self.Greez`))
        (else
          (set `self.HasBeenUsed` false)
          (`self.ServerActivateAlienBalise` true (`self.Greez`)))))))

(event `SERVER QTE WIN`
  (params (Player :type "/Game/_Jam_MilkyWay/Players/FirstPerson/Blueprints/BP_Player Object Reference"))
  (bind _as_gs_lobby (`self.As GS Lobby`))
  (`/Engine/EditorBlueprintResources/StandardMacros.DoOnce` false :!label _label
    (:`Completed`
      (if (`self.IsActive`)
        (bind _result (`/Engine/EditorBlueprintResources/StandardMacros.IncrementInt` (`/Game/_Jam_MilkyWay/Players/MenuPlayer/GS_Lobby.BeaconScore` _as_gs_lobby))
          (:`  `
            (set `/Game/_Jam_MilkyWay/Players/MenuPlayer/GS_Lobby.BeaconScore` _result _as_gs_lobby)
            (`/Game/_Jam_MilkyWay/Players/MenuPlayer/GS_Lobby.Server Reset Objectives` _as_gs_lobby)
            (set `self.IsInteracted` true)
            (`KismetSystemLibrary.Delay` 1.0)
            (`self.ServerActivateAlienBalise` false (`self.Greez`))
            (set `self.IsInteracted` false)
            (goto _label :!via `Reset`)))
        (else
          (goto _label :!via `Reset`))))))

(event `RPC_Interaction`
  (params (`Player Ref` :type "/Game/_Jam_MilkyWay/Players/FirstPerson/Blueprints/BP_Player Object Reference"))
  (`/Engine/EditorBlueprintResources/ActorMacros.Switch Has Authority`
    (:`Authority`
      (if (and (`self.IsActive`) (not (`self.IsInteracted`)) (not (`self.HasBeenUsed`)))
        (bind _output_get (set `self.Player Ref` `Player Ref`))
        (`/Game/_Jam_MilkyWay/Players/MenuPlayer/PC_Lobby.RPC_CreateAlienQTE` (`/Game/_Jam_MilkyWay/Players/FirstPerson/Blueprints/BP_Player.MyController` _output_get) 3.0 self self)))))

(event `Server UnActivate`
  (set `self.IsActive` false)
  (set `self.HasBeenUsed` false))

(event `Server_Reset`)

(event `ClientToggleWidget`
  (params (`On/off` :type Boolean))
  (bind _beaconsfx (`self.BeaconSFX`))
  (bind _mailbox (`self.Mailbox`))
  ;[1 1 1 1 50] ENABLE BEACON
  (if `On/off`
    (`SceneComponent.SetHiddenInGame` _mailbox false false)
    (`SceneComponent.SetHiddenInGame` (`self.Cylinder`) false false)
    (`AudioComponent.Play` _beaconsfx 0.0)
    (else
      (`SceneComponent.SetHiddenInGame` _mailbox true false)
      (`SceneComponent.SetHiddenInGame` (`self.Cylinder`) true false)
      (`AudioComponent.Stop` _beaconsfx))))

(event `ServerActivateAlienBalise`
  (params (`Activate Point` :type Boolean) (Greez :type "Array of /Game/_Jam_MilkyWay/Players/FirstPerson/Blueprints/BP_Player Object Reference"))
  ;[1 1 1 1 50] ENABLE BEACON
  (set `self.HasBeenUsed` false)
  (bind _output_get (set `self.Greez` Greez))
  (bind _output_get_2 (set `self.IsActive` `Activate Point`))
  (for _array_element _output_get
    (`/Game/_Jam_MilkyWay/Players/FirstPerson/Blueprints/BP_Player.Client MailBox Toggle Widget` _array_element _output_get_2 self)))

(event `self.ReceiveTick`
  (params (DeltaSeconds :type "Float (single-precision)")))

(fn `OnRep_ActivateUFO`
  (bind _mailbox (`self.Mailbox`))
  (if (`self.ActivateUFO`)
    (`SceneComponent.SetHiddenInGame` _mailbox false false)
    (else
      (`SceneComponent.SetHiddenInGame` _mailbox true false))))

(fn `OnRep_IsActive`
  (bind _bip (`self.Bip`))
  (if (`self.IsActive`)
    (`AudioComponent.Play` _bip 0.0)
    (else
      (`AudioComponent.Stop` _bip))))

(fn `OnRep_MySpline`
  (`SplineComponent.SetSplinePoints` (`self.MySpline`) (`self.Spline Array`) "World" true))

(fn `Set Spline `)

(fn `UserConstructionScript`)