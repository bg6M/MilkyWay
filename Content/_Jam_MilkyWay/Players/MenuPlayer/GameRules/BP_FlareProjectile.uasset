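; Flare gun projectile that lives for a fixed time, then has its player reload the flare gun through ServerReloadFlareGun and destroys itself.
; On any Sphere hit it deactivates its Niagara effect.
; If the hit actor's class is in the StickyActors list, it attaches to that actor, snapping to its location and rotation.
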(event `self.ReceiveBeginPlay`
  (`KismetSystemLibrary.Delay` 20.0)
  (`/Game/_Jam_MilkyWay/Players/FirstPerson/Blueprints/BP_Player.Server_ReloadFlareGun` (`self.MyPlayer`))
  (`self.K2_DestroyActor`))

(event `self.Sphere.OnComponentHit`
  (params (HitComponent :type "PrimitiveComponent Object Reference") (OtherActor :type "Actor Object Reference") (OtherComp :type "PrimitiveComponent Object Reference") (NormalImpulse :type "Vector Structure") (Hit :type "HitResult Structure (by ref)"))
  (`ActorComponent.Deactivate` (`self.Niagara`))
  (if (`KismetArrayLibrary.Array_Contains` (`self.StickyActors`) (`GameplayStatics.GetObjectClass` OtherActor))
    (`self.K2_AttachToActor` self OtherActor "None" "SnapToTarget" "SnapToTarget" "KeepRelative" true)))

(event `self.Sphere1.OnComponentBeginOverlap`
  (params (OverlappedComponent :type "PrimitiveComponent Object Reference") (OtherActor :type "Actor Object Reference") (OtherComp :type "PrimitiveComponent Object Reference") (OtherBodyIndex :type Integer) (bFromSweep :type Boolean) (SweepResult :type "HitResult Structure (by ref)")))

(fn `UserConstructionScript`)