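; Multiplayer delivery point where GREEZ-team players drop grabbed animals for a UFO to abduct, registered with GS_Lobby.
; While active, its sphere overlap validates the animal type, releases the grab, completes the objective, triggers spawner respawn and notifies the game state.
; Deactivation clears the player's pin and runs a timeline that flies the saucer along a runtime-built spline, hiding then destroying the animal.
; RPCs and RepNotifies sync the visuals.
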(event `self.ReceiveBeginPlay`
  (bind _asbp_game_instance (cast `/Game/_Jam_MilkyWay/Players/FirstPerson/Blueprints/BP_GameInstance` (`GameplayStatics.GetGameInstance`)))
  (set `self.As BP Game Instance` _asbp_game_instance)
  (bind _asgs_lobby (cast `/Game/_Jam_MilkyWay/Players/MenuPlayer/GS_Lobby` (`GameplayStatics.GetGameState`)))
  (bind _output_get (set `self.As GS Lobby` _asgs_lobby))
  (`KismetArrayLibrary.Array_Add` (`/Game/_Jam_MilkyWay/Players/MenuPlayer/GS_Lobby.MyDeliveryPoint` _output_get) self))

(event `ServerTakingAnimal`
  (`/Game/_Jam_MilkyWay/Gpe/Animals/BP_Cow.ServerAnimalExtracted` (`self.Cow in Range`))
  (`self.RPCTakingAnimal`))

(event `RPCTakingAnimal`
  (`SceneComponent.K2_SetWorldLocationAndRotation` (`/Game/_Jam_MilkyWay/Gpe/Animals/BP_Cow.Meat` (`self.Cow in Range`)) (`self.K2_GetActorLocation`) (`SceneComponent.K2_GetComponentRotation` (`self.SplineMIDTarget`)) false false))

(event `Server Overlap`
  (params (`Actor Overlap` :type "Actor Object Reference"))
  (bind _cow_in_range (`self.Cow in Range`))
  (bind _as_gs_lobby (`self.As GS Lobby`))
  (bind _myspawner (`/Game/_Jam_MilkyWay/Gpe/Animals/BP_Cow.MySpawner` _cow_in_range))
  (bind _mycowlist (`/Game/_Jam_MilkyWay/Players/MenuPlayer/GameRules/AnimalSpawner.MyCowList` _myspawner))
  (bind _asbp_player (cast `/Game/_Jam_MilkyWay/Players/FirstPerson/Blueprints/BP_Player` `Actor Overlap`))
  (switch `/Game/_Jam_MilkyWay/Players/MenuPlayer/E_PlayersTeam` (`/Game/_Jam_MilkyWay/Players/FirstPerson/Blueprints/BP_Player.Team` _asbp_player)
    (:`NewEnumerator1`
      (bind _asbp_cow (cast `/Game/_Jam_MilkyWay/Gpe/Animals/BP_Cow` (`/Game/_Jam_MilkyWay/Players/FirstPerson/Blueprints/BP_Player.MyGrabedActor` _asbp_player)))
      (bind _output_get (set `self.Cow in Range` _asbp_cow))
      (if (`/Game/_Jam_MilkyWay/Gpe/Animals/BP_Cow.IsGrabed` _output_get)
        (bind _animaltype (`/Game/_Jam_MilkyWay/Gpe/Animals/BP_Cow.AnimalType` _output_get))
        (if (`KismetArrayLibrary.Array_Contains` (`self.MyDeliveryList`) _animaltype)
          (`/Game/_Jam_MilkyWay/Players/FirstPerson/Blueprints/BP_Player.Greez_UnActivateGrab` _asbp_player)
          (set `/Game/_Jam_MilkyWay/Players/FirstPerson/Blueprints/BP_Player.MyGrabedActor` null _asbp_player)
          (`/Game/_Jam_MilkyWay/Players/MenuPlayer/GS_Lobby.Complete Objective` _as_gs_lobby _animaltype)
          (`KismetArrayLibrary.Array_Remove` _mycowlist (`KismetArrayLibrary.Array_Find` _mycowlist _cow_in_range))
          (bind _success (`/Game/_Jam_MilkyWay/Players/MenuPlayer/GameRules/AnimalSpawner.ReSpawn Animals` _myspawner))
          (set `/Game/_Jam_MilkyWay/Gpe/Animals/BP_Cow.IsDelivered` true _cow_in_range)
          (`/Game/_Jam_MilkyWay/Players/MenuPlayer/GS_Lobby.SERVER DELIVERY ANIMAL` _as_gs_lobby self))))))

(event `self.Sphere.OnComponentBeginOverlap`
  (params (OverlappedComponent :type "PrimitiveComponent Object Reference") (OtherActor :type "Actor Object Reference") (OtherComp :type "PrimitiveComponent Object Reference") (OtherBodyIndex :type Integer) (bFromSweep :type Boolean) (SweepResult :type "HitResult Structure (by ref)"))
  (if (`self.IsActive`)
    (`self.Server Overlap` OtherActor)))

(event `Server DeActivate Point`
  (bind _output_get (set `self.IsActive` false))
  (`/Game/_Jam_MilkyWay/Players/FirstPerson/Blueprints/BP_Player.CLIENT PINPOINT` (`self.Player Ref`) _output_get self)
  (`self.ServerTakingAnimal`)
  (`self.RPCDeActivatePoint`)
  (`self.SERVER UFO APPEAR`))

(event `RPCDeActivatePoint`
  (`SceneComponent.SetHiddenInGame` (`self.SM_Soucoupe`) false false))

(event `/Game/_Jam_MilkyWay/Players/FirstPerson/Blueprints/Interface/BPI_Gamerules.Set Delivery Point`
  (params (`Current Delivery Point` :type "/Game/_Jam_MilkyWay/Players/MenuPlayer/GameRules/BP_DeliveryPoint Object Reference"))
  (`self.ServerActivatePoint` null))

(event `ServerActivatePoint`
  (params (PlayerRef :type "/Game/_Jam_MilkyWay/Players/FirstPerson/Blueprints/BP_Player Object Reference") (`Activate Point` :type Boolean))
  (bind _output_get (set `self.Player Ref` PlayerRef))
  (bind _output_get_2 (set `self.IsActive` `Activate Point`))
  (`/Game/_Jam_MilkyWay/Players/FirstPerson/Blueprints/BP_Player.CLIENT PINPOINT` _output_get _output_get_2 self))

(event `See`
  (`SceneComponent.SetHiddenInGame` (`self.Cylinder`) false false)
  (`ActorComponent.SetActive` (`self.Niagara`) true false))

(event `UnSee`
  (`SceneComponent.SetHiddenInGame` (`self.Cylinder`) true false)
  (`ActorComponent.SetActive` (`self.Niagara`) false false))

(event `UFO APPEAR`
  (params (NewLocation :type "Vector Structure") (NewRotation :type "Rotator Structure") (RelativeYaw :type "Float (double-precision)") (Alpha :type "Float (single-precision)"))
  (bind _sm_soucoupe (`self.SM_Soucoupe`))
  (`SceneComponent.K2_SetWorldLocationAndRotation` _sm_soucoupe NewLocation NewRotation false false)
  (`SceneComponent.K2_SetRelativeRotation` _sm_soucoupe (`KismetMathLibrary.MakeRotator` 0.0 0.0 RelativeYaw) false false)
  (`SceneComponent.SetHiddenInGame` (`self.SM_Soucoupe`) false false))

(event `SERVER UFO APPEAR`
  (bind _myspline (`self.MySpline`))
  (set `self.ActivateUFO` true)
  (bind _success (`self.Set Spline `))
  (if _success
    (bind (_direction _distance_on_spline _rotation _alpha) (`Timeline|APPEAR` :!via `PlayFromStart`)
      (:`Update`
        (bind _returnvalue (* (`SplineComponent.GetSplineLength` _myspline) _distance_on_spline))
        (bind (_returnvalue_roll _returnvalue_pitch _returnvalue_yaw) (`KismetMathLibrary.BreakRotator` (`SplineComponent.GetRotationAtDistanceAlongSpline` _myspline _returnvalue "World")))
        (`self.UFO APPEAR` (`SplineComponent.GetLocationAtDistanceAlongSpline` _myspline _returnvalue "World") (`KismetMathLibrary.MakeRotator` _returnvalue_roll _returnvalue_pitch _returnvalue_yaw) _rotation _alpha))
      (:`Finished`
        (`self.K2_DestroyActor` (`self.Cow in Range`))
        (set `self.Cow in Range` null)
        (set `self.ActivateUFO` false))
      (:`Grab`
        (`self.RPC Wave ON`))
      (:`StopGrab`
        (`self.RPC Wave OFF`))
      (:`HideCow`
        (`self.RPC HIDE COW`)))))

(event `RPC HIDE COW`
  (`SceneComponent.SetHiddenInGame` (`/Game/_Jam_MilkyWay/Gpe/Animals/BP_Cow.Meat` (`self.Cow in Range`)) true false))

(event `RPC Wave ON`
  (`MeshComponent.SetScalarParameterValueOnMaterials` (`self.SM_Soucoupe`) "WaveFadeOut" 0.0))

(event `RPC Wave OFF`
  (`MeshComponent.SetScalarParameterValueOnMaterials` (`self.SM_Soucoupe`) "WaveFadeOut" 10.0))

(fn `OnRep_ActivateUFO`
  (bind _sm_soucoupe (`self.SM_Soucoupe`))
  (bind _rectlight (`self.RectLight`))
  (if (`self.ActivateUFO`)
    (`SceneComponent.SetHiddenInGame` _sm_soucoupe false false)
    (`LightComponent.SetIntensity` _rectlight 100000.0)
    (else
      (`SceneComponent.SetHiddenInGame` _sm_soucoupe true false)
      (`LightComponent.SetIntensity` _rectlight 0.0))))

(fn `OnRep_IsActive`)

(fn `OnRep_MySpline`
  (`SplineComponent.SetSplinePoints` (`self.MySpline`) (`self.Spline Array`) "World" true))

(fn `Set Spline `
  (returns (Success :type Boolean))
  (bind _returnvalue (`SceneComponent.K2_GetComponentLocation` (`self.SplineMIDTarget`)))
  (bind _array (`|MakeArray` (+ _returnvalue (0.0 -100000.0 100000.0)) _returnvalue (+ _returnvalue (0.0 100000.0 100000.0))))
  (set `self.Spline Array` _array)
  (bind _returnvalue_2 (`AddComponent|NODE_AddSplineComponent-0`))
  (bind _output_get (set `self.MySpline` _returnvalue_2))
  (`SplineComponent.SetSplinePoints` _output_get _array "World" true)
  (return true))

(fn `UserConstructionScript`
  (`SphereComponent.SetSphereRadius` (`self.Sphere`) (`self.In Sphere Radius`) true))