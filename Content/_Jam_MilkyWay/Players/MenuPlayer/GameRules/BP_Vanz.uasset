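; BP_Vanz is the lobby gacha van that turns fed dropboxes into upgrade loot.
; Server-side cage overlaps consume BP_Dropbox actors, raise JuiceScore and update the tank materials and registered activators.
; When active with three activators enabled, it plays a timed gamble, then spawns the score tier's DataTable upgrades in SpawnBox and resets the juice.
; RepNotifies drive state effects; animal-to-kebab logic remains but its callers are disconnected.
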(event OnComponentBeginOverlap(SM_AlienCage)
  (params (OverlappedComponent :type Primitive%20Component%20Object%20Reference) (OtherActor :type Actor%20Object%20Reference) (OtherComp :type Primitive%20Component%20Object%20Reference) (OtherBodyIndex :type Integer) (bFromSweep :type Boolean) (SweepResult :type Hit%20Result%20Structure%20%28by%20ref%29))
  (CallFunction|ServerOverlapp OtherActor OtherComp (Transformation|GetWorldLocation (Variables|Default|GetJuiceGoingDownLocation))))

(event OnComponentBeginOverlap(SM_AlienCage1)
  (params (OverlappedComponent :type Primitive%20Component%20Object%20Reference) (OtherActor :type Actor%20Object%20Reference) (OtherComp :type Primitive%20Component%20Object%20Reference) (OtherBodyIndex :type Integer) (bFromSweep :type Boolean) (SweepResult :type Hit%20Result%20Structure%20%28by%20ref%29))
  (CallFunction|ServerOverlapp OtherActor OtherComp (Transformation|GetWorldLocation (Variables|Default|GetJuiceGoingDown1Location))))

(event Custom|ServerOverlapp
  (params (ActorOverlap :type Actor%20Object%20Reference) (Other%20Comp :type Primitive%20Component%20Object%20Reference) (UseCageLocation :type Vector))
  (Networking|SwitchHasAuthority
    (:Authority
      (bind _asbp_dropbox (Utilities|Casting|CastToBP_Dropbox ActorOverlap))
      (bind _output_get (Variables|Default|SetAs%20BP%20Dropbox _asbp_dropbox))
      (CallFunction|ServerGetBox _output_get UseCageLocation)
      (bind _output_get_2 (Variables|Default|SetJuiceScore (+ (Variables|Default|GetJuiceScore) 1.0)))
      (CallFunction|MCSETJUICETANKSCALAR _output_get_2)
      (for _array_element (Variables|/Game/_Jam_MilkyWay/Players/MenuPlayer/GS_Lobby.GS_Lobby_C|GetMyVanzActivator (Variables|Default|GetAs%20GS%20Lobby))
        (Default|RPCSetTextColor _array_element _output_get_2)))))

(event Custom|ServerGetBox
  (params (As%20BP%20Dropbox :type BP%20Dropbox%20Object%20Reference) (Location :type Vector))
  (Variables|Default|SetCurrentDropBoxQuality (Variables|/Game/_Jam_MilkyWay/Gpe/Dropbox/BP_Dropbox.BP_Dropbox_C|GetQuality As%20BP%20Dropbox))
  (Default|ManzUnActivateGrab (Variables|/Game/_Jam_MilkyWay/Gpe/Dropbox/BP_Dropbox.BP_Dropbox_C|GetPlayer%20Calling%20Grab As%20BP%20Dropbox) false false)
  (Actor|DestroyActor As%20BP%20Dropbox)
  (Audio|PlaySoundatLocation "/Game/_Jam_MilkyWay/SFX/Foleys/Van/JuiceTank_Fill_SFX.JuiceTank_Fill_SFX" Location "0, 0, 0" 1.2 1.0 0.0 "/Game/_Jam_MilkyWay/SFX/SA_VoiceChat.SA_VoiceChat" 0 0 0)
  (Niagara|SpawnSystematLocation "/Game/_Jam_MilkyWay/Vfx/VFX_Worm_Aspiration.VFX_Worm_Aspiration" Location))

(event Custom|MC_CallLarva
  (params (Condition :type Boolean))
  (Default|LarvaLoose (Variables|Default|GetAs%20W%20Rarity%20Info%20Screen) Condition))

(event Custom|MC_SET%20JUICE%20TANK%20SCALAR
  (params (JuiceScore :type Float%20%28double-precision%29))
  (bind _sm_juicetank1 (Variables|Default|GetSM_JuiceTank1))
  (bind _sm_juicetank (Variables|Default|GetSM_JuiceTank))
  (bind _sm_aliencage (Variables|Default|GetSM_AlienCage))
  (bind _sm_aliencage1 (Variables|Default|GetSM_AlienCage1))
  (bind _output_get (Variables|Default|SetJuiceScore JuiceScore))
  (switch int (Math|Float|Truncate _output_get)
    (:0
      (Utilities|FlowControl|Delay 1.1)
      (Rendering|Material|SetScalarParameterValueonMaterials _sm_juicetank "JuiceQuantity" 1.0)
      (Rendering|Material|SetScalarParameterValueonMaterials _sm_juicetank1 "JuiceQuantity" 1.0)
      (Rendering|Material|SetScalarParameterValueonMaterials _sm_aliencage "JuiceQuantity" 1.0)
      (Rendering|Material|SetScalarParameterValueonMaterials _sm_aliencage1 "JuiceQuantity" 1.0))
    (:1
      (Utilities|FlowControl|Delay 1.1)
      (Rendering|Material|SetScalarParameterValueonMaterials _sm_juicetank "JuiceQuantity" 0.8)
      (Rendering|Material|SetScalarParameterValueonMaterials _sm_juicetank1 "JuiceQuantity" 0.8)
      (Rendering|Material|SetScalarParameterValueonMaterials _sm_aliencage "JuiceQuantity" 0.8)
      (Rendering|Material|SetScalarParameterValueonMaterials _sm_aliencage1 "JuiceQuantity" 0.8))
    (:2
      (Utilities|FlowControl|Delay 1.1)
      (Rendering|Material|SetScalarParameterValueonMaterials _sm_juicetank "JuiceQuantity" 0.6)
      (Rendering|Material|SetScalarParameterValueonMaterials _sm_juicetank1 "JuiceQuantity" 0.6)
      (Rendering|Material|SetScalarParameterValueonMaterials _sm_aliencage "JuiceQuantity" 0.6)
      (Rendering|Material|SetScalarParameterValueonMaterials _sm_aliencage1 "JuiceQuantity" 0.6))
    (:3
      (Utilities|FlowControl|Delay 1.1)
      (Rendering|Material|SetScalarParameterValueonMaterials _sm_juicetank "JuiceQuantity" 0.4)
      (Rendering|Material|SetScalarParameterValueonMaterials _sm_juicetank1 "JuiceQuantity" 0.4)
      (Rendering|Material|SetScalarParameterValueonMaterials _sm_aliencage "JuiceQuantity" 0.4)
      (Rendering|Material|SetScalarParameterValueonMaterials _sm_aliencage1 "JuiceQuantity" 0.4))
    (:4
      (Utilities|FlowControl|Delay 1.1)
      (Rendering|Material|SetScalarParameterValueonMaterials _sm_juicetank "JuiceQuantity" 0.2)
      (Rendering|Material|SetScalarParameterValueonMaterials _sm_juicetank1 "JuiceQuantity" 0.2)
      (Rendering|Material|SetScalarParameterValueonMaterials _sm_aliencage "JuiceQuantity" 0.2)
      (Rendering|Material|SetScalarParameterValueonMaterials _sm_aliencage1 "JuiceQuantity" 0.2))
    (:5
      (Utilities|FlowControl|Delay 1.1)
      (Rendering|Material|SetScalarParameterValueonMaterials _sm_juicetank "JuiceQuantity" 0.0)
      (Rendering|Material|SetScalarParameterValueonMaterials _sm_juicetank1 "JuiceQuantity" 0.0)
      (Rendering|Material|SetScalarParameterValueonMaterials _sm_aliencage "JuiceQuantity" 0.0)
      (Rendering|Material|SetScalarParameterValueonMaterials _sm_aliencage1 "JuiceQuantity" 0.0))))

(event Custom|RPC_Set%20Juice%20Tank%20Scalar
  (params (JuiceScore :type Float%20%28double-precision%29))
  (CallFunction|MCSETJUICETANKSCALAR JuiceScore))

(event Custom|RPCGetBOX
  (params (Target :type Actor%20Object%20Reference))
  (Transformation|AttachComponentToComponent Target 0 "None" "SnapToTarget" "SnapToTarget" "KeepRelative" true))

(event Custom|ServerLootBox
  (switch int (Math|Float|Truncate (Variables|Default|GetJuiceScore))
    (:1
      (for _array_element (Variables|Default|GetLowUpgrades)
        (bind _returnvalue (Utilities|GetDataTableRow (.DataTable (Utilities|Struct|BreakDataTableRowHandle _array_element)) (.RowName (Utilities|Struct|BreakDataTableRowHandle _array_element)))
          (:then
            (CallFunction|ActivateUpgrade _returnvalue))))
      (bind _output_get (Variables|Default|SetJuiceScore 0.0 :!label _label))
      (CallFunction|MCSETJUICETANKSCALAR _output_get)
      (for _array_element_2 (Variables|/Game/_Jam_MilkyWay/Players/MenuPlayer/GS_Lobby.GS_Lobby_C|GetMyVanzActivator (Variables|Default|GetAs%20GS%20Lobby))
        (Default|RPCSetTextColor _array_element_2 _output_get))
      (Utilities|FlowControl|Delay 3.0)
      (Variables|Default|SetIsClosed true)
      (Utilities|FlowControl|DoOnce false) ; enters at Reset
    )
    (:2
      (for _array_element_3 (Variables|Default|GetCommonUpgrades)
        (bind _returnvalue_2 (Utilities|GetDataTableRow (.DataTable (Utilities|Struct|BreakDataTableRowHandle _array_element_3)) (.RowName (Utilities|Struct|BreakDataTableRowHandle _array_element_3)))
          (:then
            (CallFunction|ActivateUpgrade _returnvalue_2))))
      (goto _label))
    (:3
      (for _array_element_4 (Variables|Default|GetGood%20Upgrades)
        (bind _returnvalue_3 (Utilities|GetDataTableRow (.DataTable (Utilities|Struct|BreakDataTableRowHandle _array_element_4)) (.RowName (Utilities|Struct|BreakDataTableRowHandle _array_element_4)))
          (:then
            (CallFunction|ActivateUpgrade _returnvalue_3)
            (goto _label))))
      (goto _label))
    (:4
      (for _array_element_5 (Variables|Default|GetEpic%20Upgrades)
        (bind _returnvalue_4 (Utilities|GetDataTableRow (.DataTable (Utilities|Struct|BreakDataTableRowHandle _array_element_5)) (.RowName (Utilities|Struct|BreakDataTableRowHandle _array_element_5)))
          (:then
            (CallFunction|ActivateUpgrade _returnvalue_4)
            (goto _label)))))
    (:5
      (for _array_element_6 (Variables|Default|GetLegendary%20Upgrades)
        (bind _returnvalue_5 (Utilities|GetDataTableRow (.DataTable (Utilities|Struct|BreakDataTableRowHandle _array_element_6)) (.RowName (Utilities|Struct|BreakDataTableRowHandle _array_element_6)))
          (:then
            (CallFunction|ActivateUpgrade _returnvalue_5)
            (goto _label)))))))

(event Custom|ServerGetKebab
  (params (CowBP :type BP%20Cow%20Object%20Reference))
  (Variables|Default|SetAnimal%20Type (Variables|/Game/_Jam_MilkyWay/Gpe/Animals/BP_Cow.BP_Cow_C|GetAnimalType CowBP))
  (Default|ManzUnActivateGrab (Variables|/Game/_Jam_MilkyWay/Gpe/Animals/BP_Cow.BP_Cow_C|GetPlayer%20Calling%20Grab CowBP) false false)
  (Actor|DestroyActor CowBP))

(event Custom|ServerLootKebab
  (bind _spawnbox (Variables|Default|GetSpawnBox))
  (bind _good_upgrades (Variables|Default|GetGood%20Upgrades))
  (bind (_origin _boxextent) (Collision|GetComponentBounds _spawnbox))
  (switch Utilities|FlowControl|Switch|SwitchonAnimalsList (Variables|Default|GetAnimal%20Type)
    (:NewEnumerator0
      (Variables|Default|SetDataToSpawn (Utilities|Array|Get(acopy) _good_upgrades)))
    (:NewEnumerator1
      (Variables|Default|SetDataToSpawn (Utilities|Array|Get(acopy) _good_upgrades 1) :!label _label))
    (:NewEnumerator2
      (goto _label)))
  (bind _returnvalue (Utilities|GetDataTableRow (.DataTable (Utilities|Struct|BreakDataTableRowHandle (Variables|Default|GetDataToSpawn))) (.RowName (Utilities|Struct|BreakDataTableRowHandle (Variables|Default|GetDataToSpawn))))
    (:then
      (for _index (range 0 (.Numbers (Utilities|Struct|BreakS_ActorItems (.Actor_Structure (Utilities|Struct|BreakS_DropBox_Upgrade _returnvalue)))))
        (Game|SpawnActorfromClass (.ActorToSpawn (Utilities|Struct|BreakS_ActorItems (.Actor_Structure (Utilities|Struct|BreakS_DropBox_Upgrade _returnvalue)))) (Math|Transform|MakeTransform (Math|Random|RandomPointinBoundingBox _origin _boxextent) "0, 0, 0" "1.000000,1.000000,1.000000") "Undefined" "MultiplyWithRoot" 0 0)))))

(event Custom|RPC%20PLAY%20IS%20ACTIVE%20SOUND
  (CallFunction|MCPLAYISACTIVESOUND))

(event Custom|MC%20PLAY%20IS%20ACTIVE%20SOUND
  (if (Variables|Default|GetIsActive?)
    (Audio|PlaySoundatLocation "/Game/_Jam_MilkyWay/SFX/Foleys/Horns/beep-beep-101391.beep-beep-101391" (Transformation|GetActorLocation) "0, 0, 0" 1.0 1.0 0.0 "/Game/_Jam_MilkyWay/SFX/Attenuation_Types/SA_MailBox.SA_MailBox" 0 0 0)
    (else
      (Audio|Components|Audio|Stop (Variables|Default|GetVan_OnLoop_SFX_Cue)))))

(event Custom|CheckActivator
  (if (Variables|Default|GetIsActive?)
    (if (== (Variables|Default|GetActivatorEnable) 3)
      (Utilities|FlowControl|DoOnce false
        (:Completed
          (Variables|Default|SetIsGanbling true)
          (for _array_element (Variables|/Game/_Jam_MilkyWay/Players/MenuPlayer/GS_Lobby.GS_Lobby_C|GetMyVanzActivator (Variables|Default|GetAs%20GS%20Lobby))
            (Default|MCEnableWidgetGanblingAnim _array_element))
          (Utilities|FlowControl|Delay 3.0)
          (Variables|Default|SetIsGanbling false)
          (Variables|Default|SetBoxReveal true)
          (Variables|Default|SetIsClosed false)
          (CallFunction|ServerLootBox))))))

(event Custom|RPC_CallLarva
  (params (Condition :type Boolean))
  (CallFunction|MCCallLarva Condition))

(event EventBeginPlay
  (bind _screenwidget (Variables|Default|GetScreenWidget))
  (bind _asgs_lobby (Utilities|Casting|CastToGS_Lobby (Game|GetGameState)))
  (bind _output_get (Variables|Default|SetAs%20GS%20Lobby _asgs_lobby))
  (Variables|/Game/_Jam_MilkyWay/Players/MenuPlayer/GS_Lobby.GS_Lobby_C|SetVanz _output_get self)
  (Networking|SwitchHasAuthority
    (:Authority
      (bind _asw_rarity_info_screen (Utilities|Casting|CastToW_RarityInfoScreen (UserInterface|GetWidget _screenwidget)))
      (Variables|Default|SetAs%20W%20Rarity%20Info%20Screen _asw_rarity_info_screen))
    (:Remote
      (bind _asw_rarity_info_screen_2 (Utilities|Casting|CastToW_RarityInfoScreen (UserInterface|GetUserWidgetObject _screenwidget)))
      (Variables|Default|SetAs%20W%20Rarity%20Info%20Screen _asw_rarity_info_screen_2))))

(event EventTick
  (params (DeltaSeconds :type Float%20%28single-precision%29)))

(fn ConstructionScript)

(fn OnRepIsGanbling
  (bind _vfxendspawnlocation (Variables|Default|GetVfxEndSpawnLocation))
  (bind _returnvalue (Transformation|GetWorldLocation _vfxendspawnlocation))
  (if (Variables|Default|GetIsGanbling)
    (Rendering|Material|SetMaterial (Variables|Default|GetSkeletalMesh) 0 "/Game/_Jam_MilkyWay/Environment/Vehicles/Van/MI_Gatcha.MI_Gatcha")
    (Audio|SpawnSoundatLocation "/Game/_Jam_MilkyWay/SFX/Foleys/Shutter_Closed_SFX.Shutter_Closed_SFX" _returnvalue "0, 0, 0" 1.0 1.0 0.0 "/Game/_Jam_MilkyWay/SFX/Attenuation_Types/SA_Spells.SA_Spells" 0)
    (Audio|SpawnSoundatLocation "/Game/_Jam_MilkyWay/Musics/ChestOpening.ChestOpening" _returnvalue "0, 0, 0" 1.0 1.0 0.0 "/Game/_Jam_MilkyWay/SFX/Attenuation_Types/SA_Vehicles.SA_Vehicles" 0)
    (Development|SetHiddeninGame (Variables|Default|GetVFX_RadioWave) false false)
    (else
      (Rendering|Material|SetMaterial (Variables|Default|GetSkeletalMesh) 0 "/Game/_Jam_MilkyWay/Environment/Vehicles/Van/MI_Van.MI_Van")
      (Development|SetHiddeninGame (Variables|Default|GetVFX_RadioWave) true false))))

(fn OnRepBoxReveal
  (bind _vfxendspawnlocation (Variables|Default|GetVfxEndSpawnLocation))
  (bind _pointlightgenerator (Variables|Default|GetPointLightGenerator))
  (bind _returnvalue (Transformation|GetWorldLocation _vfxendspawnlocation))
  (if (Variables|Default|GetBoxReveal)
    (Rendering|Components|Light|SetIntensity _pointlightgenerator 5e+02)
    (Audio|SpawnSoundatLocation "/Game/_Jam_MilkyWay/SFX/Foleys/Shutter_Open_SFX.Shutter_Open_SFX" _returnvalue "0, 0, 0" 1.0 1.0 0.0 "/Game/_Jam_MilkyWay/SFX/Attenuation_Types/SA_Spells.SA_Spells" 0)
    (Niagara|SpawnSystematLocation "/Game/_Jam_MilkyWay/Vfx/VFX_GatchaEnd.VFX_GatchaEnd" _returnvalue)
    (else
      (Rendering|Components|Light|SetIntensity _pointlightgenerator 0.0))))

(fn ActivateUpgrade
  (params (UpgradeStructure :type S%20Drop%20Box%20Upgrade%20Structure))
  (bind _spawnbox (Variables|Default|GetSpawnBox))
  (bind _spawnbox_2 (Variables|Default|GetSpawnBox))
  (bind (_origin _boxextent) (Collision|GetComponentBounds _spawnbox))
  (bind (_origin_2 _boxextent_2) (Collision|GetComponentBounds _spawnbox_2))
  (bind _output_get (LocalVariables|SetDATA_local UpgradeStructure))
  (switch Utilities|FlowControl|Switch|SwitchonE_UpgradeType (.UpgradeType (Utilities|Struct|BreakS_DropBox_Upgrade _output_get))
    (:NewEnumerator0
      (for _index (range 1 (.Numbers (Utilities|Struct|BreakS_ActorItems (.Actor_Structure (Utilities|Struct|BreakS_DropBox_Upgrade _output_get)))))
        (Game|SpawnActorfromClass (.ActorToSpawn (Utilities|Struct|BreakS_ActorItems (.Actor_Structure (Utilities|Struct|BreakS_DropBox_Upgrade _output_get)))) (Math|Transform|MakeTransform (Math|Random|RandomPointinBoundingBox _origin_2 _boxextent_2) "0, 0, 0" "1.000000,1.000000,1.000000") "Undefined" "MultiplyWithRoot" 0 0)))
    (:NewEnumerator1
      (for _index_2 (range 1 (.Numbers (Utilities|Struct|BreakS_Items (.Item_Structure (Utilities|Struct|BreakS_DropBox_Upgrade _output_get)))))
        (bind _returnvalue (Game|SpawnActorfromClass "/Game/_Jam_MilkyWay/Players/DataTable/Items/BP_MasterItemPhysx.BP_MasterItemPhysx_C" (Math|Transform|MakeTransform (Math|Random|RandomPointinBoundingBox _origin _boxextent) "0, 0, 0" "1.000000,1.000000,1.000000") "Undefined" "MultiplyWithRoot" 0 3e+02 (.Buff_to_Call (Utilities|Struct|BreakS_Items (.Item_Structure (Utilities|Struct|BreakS_DropBox_Upgrade _output_get)))) _output_get 0))
        (Default|SETDATA _returnvalue _output_get)))))

(fn OnRepIsActive?
  (bind _van_onloop_sfx_cue (Variables|Default|GetVan_OnLoop_SFX_Cue))
  (if (Variables|Default|GetIsActive?)
    (Audio|PlaySoundatLocation "/Game/_Jam_MilkyWay/SFX/Foleys/Horns/beep-beep-101391.beep-beep-101391" (Transformation|GetActorLocation) "0, 0, 0" 1.0 1.0 0.0 "/Game/_Jam_MilkyWay/SFX/Attenuation_Types/SA_MailBox.SA_MailBox" 0 0 0)
    (Development|SetHiddeninGame (Variables|Default|GetVFX_SlowRadioWave) false false)
    (Audio|Components|Audio|Play _van_onloop_sfx_cue 0.0)
    (else
      (Development|SetHiddeninGame (Variables|Default|GetVFX_SlowRadioWave) true false)
      (Audio|Components|Audio|Stop _van_onloop_sfx_cue))))