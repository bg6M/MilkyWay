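; BP_KillZone is a lobby volume that sends players who touch it back to their team's spawn.
; On BeginPlay it caches GS_Lobby, then on box overlap reads the BP_Player's Team, MANZ or GREEZ.
; It teleports the player to the box of a random entry in that team's spawn zone array, with zero rotation.
; The construction script sizes the trigger box from InBoxExtent.
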(event `self.ReceiveBeginPlay`
  (bind _asgs_lobby (cast `/Game/_Jam_MilkyWay/Players/MenuPlayer/GS_Lobby` (`GameplayStatics.GetGameState`)))
  (set `self.As GS Lobby` _asgs_lobby))

(event `self.Box.OnComponentBeginOverlap`
  (params (OverlappedComponent :type "PrimitiveComponent Object Reference") (OtherActor :type "Actor Object Reference") (OtherComp :type "PrimitiveComponent Object Reference") (OtherBodyIndex :type Integer) (bFromSweep :type Boolean) (SweepResult :type "HitResult Structure (by ref)"))
  (bind _as_gs_lobby (`self.As GS Lobby`))
  (bind _greezspawnzone (`/Game/_Jam_MilkyWay/Players/MenuPlayer/GS_Lobby.GreezSpawnZone` _as_gs_lobby))
  (bind _manzspawnzone (`/Game/_Jam_MilkyWay/Players/MenuPlayer/GS_Lobby.ManzSpawnZone` _as_gs_lobby))
  (bind _asbp_player (cast `/Game/_Jam_MilkyWay/Players/FirstPerson/Blueprints/BP_Player` OtherActor))
  (switch `/Game/_Jam_MilkyWay/Players/MenuPlayer/E_PlayersTeam` (`/Game/_Jam_MilkyWay/Players/FirstPerson/Blueprints/BP_Player.Team` _asbp_player)
    (:`NewEnumerator0`
      (`self.K2_TeleportTo` :`self` _asbp_player :`DestLocation` (`SceneComponent.K2_GetComponentLocation` (`/Game/_Jam_MilkyWay/Players/MenuPlayer/BP_MANZ_SpawnZone.Box` (`|GetArrayItem` _manzspawnzone (`KismetMathLibrary.RandomIntegerInRange` 0 (- (`KismetArrayLibrary.Array_Length` _manzspawnzone) 1)))))))
    (:`NewEnumerator1`
      (`self.K2_TeleportTo` :`self` _asbp_player :`DestLocation` (`SceneComponent.K2_GetComponentLocation` (`/Game/_Jam_MilkyWay/Players/MenuPlayer/BP_GREEZ_SpawnZone.Box` (`|GetArrayItem` _greezspawnzone (`KismetMathLibrary.RandomIntegerInRange` 0 (- (`KismetArrayLibrary.Array_Length` _greezspawnzone) 1)))))))))

(fn `UserConstructionScript`
  (`BoxComponent.SetBoxExtent` (`self.Box`) (`self.In Box Extent`) true))