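; Interactable Vanz activator in the lobby that registers with GS_Lobby and counts toward the Vanz's enabled activators.
; When active, interaction multicasts a DoOnce-guarded trigger that increments the Vanz count, calls CheckActivator, then reverts after a one-second window.
; RepNotify IsActive shows or hides its info widget, while RepNotify IsTrigger plays sounds and the widget's interact animation.
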(event `self.ReceiveBeginPlay`
  (bind _widget (`self.Widget`))
  (bind _asgs_lobby (cast `/Game/_Jam_MilkyWay/Players/MenuPlayer/GS_Lobby` (`GameplayStatics.GetGameState`)))
  (bind _output_get (set `self.As GS Lobby` _asgs_lobby))
  (`KismetArrayLibrary.Array_Add` (`/Game/_Jam_MilkyWay/Players/MenuPlayer/GS_Lobby.MyVanzActivator` _output_get) self)
  (`/Engine/EditorBlueprintResources/ActorMacros.Switch Has Authority`
    (:`Authority`
      (bind _asw_vanz_activator_info (cast `/Game/_Jam_MilkyWay/Players/MenuPlayer/GameWidgets/W_VanzActivatorInfo` (`WidgetComponent.GetWidget` _widget)))
      (set `self.MyWidget` _asw_vanz_activator_info))
    (:`Remote`
      (bind _asw_vanz_activator_info_2 (cast `/Game/_Jam_MilkyWay/Players/MenuPlayer/GameWidgets/W_VanzActivatorInfo` (`WidgetComponent.GetUserWidgetObject` _widget)))
      (set `self.MyWidget` _asw_vanz_activator_info_2))))

(event `/Game/_Jam_MilkyWay/Players/FirstPerson/Blueprints/Interface/BPI_Interaction.Interact_Int`
  (params (Bp_Player :type "/Game/_Jam_MilkyWay/Players/FirstPerson/Blueprints/BP_Player Object Reference"))
  (if (`self.IsActive?`)
    (`self.Activate`)))

(event `MC_Activate`
  (bind _vanz (`/Game/_Jam_MilkyWay/Players/MenuPlayer/GS_Lobby.Vanz` (`self.As GS Lobby`)))
  (bind _vanz_2 (`/Game/_Jam_MilkyWay/Players/MenuPlayer/GS_Lobby.Vanz` (`self.As GS Lobby`)))
  (`/Engine/EditorBlueprintResources/StandardMacros.DoOnce` false :!label _label
    (:`Completed`
      (set `self.IsTrigger` true)
      (set `/Game/_Jam_MilkyWay/Players/MenuPlayer/GameRules/BP_Vanz.ActivatorEnable` (+ (`/Game/_Jam_MilkyWay/Players/MenuPlayer/GameRules/BP_Vanz.ActivatorEnable` _vanz_2) 1) _vanz_2)
      (`/Game/_Jam_MilkyWay/Players/MenuPlayer/GameRules/BP_Vanz.CheckActivator` _vanz_2)
      (`KismetSystemLibrary.Delay` 1.0)
      (set `self.IsTrigger` false)
      (set `/Game/_Jam_MilkyWay/Players/MenuPlayer/GameRules/BP_Vanz.ActivatorEnable` (- (`/Game/_Jam_MilkyWay/Players/MenuPlayer/GameRules/BP_Vanz.ActivatorEnable` _vanz) 1) _vanz)
      (goto _label :!via `Reset`))))

(event `Activate`
  (`self.MC_Activate`))

(event `/Game/_Jam_MilkyWay/Players/FirstPerson/Blueprints/Interface/BPI_Interaction.ToggleWidget`
  (params (`On/Off` :type Boolean) (PlayerCallingWidget :type "/Game/_Jam_MilkyWay/Players/FirstPerson/Blueprints/BP_Player Object Reference")))

(event `/Game/_Jam_MilkyWay/Players/FirstPerson/Blueprints/Interface/BPI_Interaction.ToggleOutlineInteractible`
  (params (`Player Calling` :type "/Game/_Jam_MilkyWay/Players/FirstPerson/Blueprints/BP_Player Object Reference"))
  (`/Game/_Jam_MilkyWay/Players/FirstPerson/Blueprints/BP_Player.ACTIVATE OUTLINE` `Player Calling` true (`self.StaticMesh`)))

(fn `OnRep_IsActive?`
  (bind _mywidget (`self.MyWidget`))
  (if (`self.IsActive?`)
    (`Widget.SetVisibility` _mywidget "Visible")
    (else
      (`Widget.SetVisibility` _mywidget "Hidden"))))

(fn `OnRep_IsTrigger`
  (bind _returnvalue (`self.K2_GetActorLocation`))
  (if (`self.IsTrigger`)
    (`GameplayStatics.PlaySoundAtLocation` "/Engine/EditorSounds/Notifications/CompileSuccess.CompileSuccess" _returnvalue (struct) 1.0 1.0 0.0 "/Game/_Jam_MilkyWay/SFX/Attenuation_Types/SA_Blaster.SA_Blaster" null null null)
    (`/Game/_Jam_MilkyWay/Players/MenuPlayer/GameWidgets/W_VanzActivatorInfo.ToggleAnimInteract` (`self.MyWidget`))
    (else
      (`GameplayStatics.PlaySoundAtLocation` "/Engine/EditorSounds/Notifications/CompileFailed.CompileFailed" _returnvalue (struct) 1.0 1.0 0.0 "/Game/_Jam_MilkyWay/SFX/Attenuation_Types/SA_Blaster.SA_Blaster" null null null))))

(fn `UserConstructionScript`)