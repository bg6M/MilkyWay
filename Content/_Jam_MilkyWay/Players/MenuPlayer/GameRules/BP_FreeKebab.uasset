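; BP_FreeKebab is a short-lived spawner actor that drops free food items at its location, based on an animal selection.
; On BeginPlay it plays an attenuated sound, then calls RPCSPAWNKEBAB.
; That event spawns several chicken wings for Chicken or kebabs for Sheep and Cow slightly above itself, then destroys the actor.
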(event `self.ReceiveBeginPlay`
  (`GameplayStatics.PlaySoundAtLocation` "/Game/_Jam_MilkyWay/SFX/GPE/Alien/Alien_InvisibilityTrigger_SFX.Alien_InvisibilityTrigger_SFX" (`self.K2_GetActorLocation`) (struct) 1.0 1.0 0.0 "/Game/_Jam_MilkyWay/SFX/Attenuation_Types/SA_AnimalsLot.SA_AnimalsLot" null null null)
  (`self.RPCSPAWNKEBAB`))

(event `RPCSPAWNKEBAB`
  (bind _returnvalue (`KismetMathLibrary.Conv_VectorToTransform` (+ (`self.K2_GetActorLocation`) (0.0 0.0 50.0))))
  (switch `/Game/_Jam_MilkyWay/Players/MenuPlayer/GameRules/AnimalsList` (`self.Selection`)
    (:`NewEnumerator0`
      (for _ (range 3)
        (`|SpawnActorFromClass` "/Game/_Jam_MilkyWay/Players/DataTable/Items/Bp_ChickenWing.Bp_ChickenWing_C" _returnvalue "Undefined" "MultiplyWithRoot" null null)))
    (:`NewEnumerator1`
      (for _ (range 3) :!label _label
        (`|SpawnActorFromClass` "/Game/_Jam_MilkyWay/Players/DataTable/Items/Bp_Kebab.Bp_Kebab_C" _returnvalue "Undefined" "MultiplyWithRoot" null null)))
    (:`NewEnumerator2`
      (goto _label)))
  (`self.K2_DestroyActor`))

(fn `UserConstructionScript`)