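; Replicated lobby worm that MANZ players grab to drain its health, earning a worm buff through GS_Lobby when it dies.
; Server RPCs track grabbers, whose count sets per-tick damage, multicast to drive inflate and speed material parameters.
; Spline movement calls are multicast, with a line trace snapping the mesh to ground height.
; RepNotifies handle parent-spline activation and grab widget/sound, while separate events request destruction or spawn a BP_Dropbox.
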(event `ServerMoveOnspline`
  (params (NewLocation :type "Vector Structure") (NewRotation :type "Rotator Structure"))
  (`self.MC_MoveOnspline` NewLocation NewRotation))

(event `self.ReceiveTick`
  (params (DeltaSeconds :type "Float (single-precision)"))
  (if (`self.IsActive`)
    (if (`self.IsGrabed`)
      (`self.Server_GrabWorm` (`self.NumPlayerGrab`))
      (if (<= (`self.Health`) 0.0)
        (`/Engine/EditorBlueprintResources/StandardMacros.DoOnce` false
          (:`Completed`
            (set `self.Dead` true)
            (`/Game/_Jam_MilkyWay/Players/MenuPlayer/GS_Lobby.SERVER_ADD WORM BUFF` (`self.As GS Lobby`) self)))))))

(event `MC_MoveOnspline`
  (params (NewLocation :type "Vector Structure") (NewRotation :type "Rotator Structure"))
  (bind _skeletalmesh (`self.SkeletalMesh`))
  (bind _outhit (`KismetSystemLibrary.LineTraceSingle` (+ NewLocation (0.0 0.0 300.0)) (- NewLocation (0.0 0.0 1500.0)) "TraceTypeQuery1"))
  (bind (_bblockinghit _binitialoverlap _time _distance _location) (`GameplayStatics.BreakHitResult` _outhit))
  (if _bblockinghit
    (`SceneComponent.K2_SetWorldLocationAndRotation` _skeletalmesh (`KismetMathLibrary.MakeVector` (.x NewLocation) (.y NewLocation) (.z _location)) NewRotation false false)
    (else
      (`SceneComponent.K2_SetWorldLocationAndRotation` _skeletalmesh NewLocation NewRotation false false))))

(event `SET DATA`
  (params (MyPArent :type "/Game/_Jam_MilkyWay/Players/MenuPlayer/GameRules/BP_WormSpline Object Reference") (MySpline :type "SplineComponent Object Reference"))
  (set `self.MyPArent` MyPArent)
  (set `self.MySpline` MySpline))

(event `self.ReceiveBeginPlay`
  (bind _asgs_lobby (cast `/Game/_Jam_MilkyWay/Players/MenuPlayer/GS_Lobby` (`GameplayStatics.GetGameState`))
    (:`then`
      (bind _output_get (set `self.As GS Lobby` _asgs_lobby)))
    (:`CastFailed`
      _))
  (bind _asw_worm_life (cast `/Game/_Jam_MilkyWay/Players/MenuPlayer/GameWidgets/W_WormLife` (`WidgetComponent.GetWidget` (`self.Widget`))))
  (bind _output_get_2 (set `self.As W Worm Life` _asw_worm_life))
  (set `/Game/_Jam_MilkyWay/Players/MenuPlayer/GameWidgets/W_WormLife.MyWorm` self _output_get_2))

(event `/Game/_Jam_MilkyWay/Players/FirstPerson/Blueprints/Interface/BPI_Grab.Grab Interface`
  (params (`Player calling grab` :type "/Game/_Jam_MilkyWay/Players/FirstPerson/Blueprints/BP_Player Object Reference") (PlayerTeam :type "/Game/_Jam_MilkyWay/Players/MenuPlayer/E_PlayersTeam Enum" :default "NewEnumerator0"))
  (if (`self.IsActive`)
    (switch `/Game/_Jam_MilkyWay/Players/MenuPlayer/E_PlayersTeam` PlayerTeam
      (:`NewEnumerator0`
        (if (not (`KismetArrayLibrary.Array_Contains` (`self.Player Calling Grab`) `Player calling grab`))
          (`self.Server_AddPlayer` `Player calling grab`))))))

(event `Server_GrabWorm`
  (params (NumPlayerGrab :type Integer))
  (`self.MC_GrabWorm` NumPlayerGrab))

(event `MC_GrabWorm`
  (params (InputPin :type Integer))
  (bind _skeletalmesh (`self.SkeletalMesh`))
  (bind _health (`self.Health`))
  (bind _returnvalue (`KismetMathLibrary.FClamp` (`KismetMathLibrary.MapRangeClamped` (* (`KismetMathLibrary.NormalizeToRange` _health 0.0 100.0) -1.0) -1.0 0.0 0.0 3.0) 0.0 2.0))
  (set `self.Health` (- _health (`|GetArrayItem` (`self.HealthModifier`) InputPin)))
  (`MeshComponent.SetScalarParameterValueOnMaterials` _skeletalmesh "InflateIntensity" _returnvalue)
  (`MeshComponent.SetScalarParameterValueOnMaterials` _skeletalmesh "Speed" (`KismetMathLibrary.FClamp` (`|GetArrayItem` (`self.SpeedModifier`) (`self.NumPlayerGrab`)) 0.75 2.5))
  (`MeshComponent.SetScalarParameterValueOnMaterials` _skeletalmesh "InflateIntensityWORM" (* _returnvalue 2.0)))

(event `CanBekilled`
  (`/Game/_Jam_MilkyWay/Players/MenuPlayer/GameRules/BP_WormSpline.Server_Destroy my Worm` (`self.MyPArent`) true))

(event `SERVER_SpawnLoot`
  (bind (_returnvalue_location _returnvalue_rotation) (`KismetMathLibrary.BreakTransform` (`self.GetTransform`)))
  (`|SpawnActorFromClass` "/Game/_Jam_MilkyWay/Gpe/Dropbox/BP_Dropbox.BP_Dropbox_C" (`KismetMathLibrary.MakeTransform` _returnvalue_location _returnvalue_rotation) "Undefined" "MultiplyWithRoot" null "NewEnumerator0" null null)
  (`self.MC_DESTROY`))

(event `Server_AddPlayer`
  (params (PlayercallingGrab :type "/Game/_Jam_MilkyWay/Players/FirstPerson/Blueprints/BP_Player Object Reference (by ref)"))
  (bind _player_calling_grab (`self.Player Calling Grab`))
  (`KismetArrayLibrary.Array_AddUnique` (`self.Player Calling Grab`) PlayercallingGrab)
  (if (`KismetArrayLibrary.Array_IsEmpty` _player_calling_grab) :!label _label
    (set `self.NumPlayerGrab` 0)
    (set `self.IsGrabed` false)
    (else
      (set `self.NumPlayerGrab` (+ (`KismetArrayLibrary.Array_Length` _player_calling_grab) 1))
      (set `self.IsGrabed` true))))

(event `MC_DESTROY`
  (`self.K2_DestroyActor`))

(event `/Game/_Jam_MilkyWay/Players/FirstPerson/Blueprints/Interface/BPI_Grab.UnGrab Interface`
  (params (`Player Calling Grab` :type "/Game/_Jam_MilkyWay/Players/FirstPerson/Blueprints/BP_Player Object Reference"))
  (`self.Server_Ungrab` `Player Calling Grab`))

(event `Server_Ungrab`
  (params (`Player Calling Grab` :type "/Game/_Jam_MilkyWay/Players/FirstPerson/Blueprints/BP_Player Object Reference (by ref)"))
  (bind _player_calling_grab (`self.Player Calling Grab`))
  (if (`KismetArrayLibrary.Array_Contains` _player_calling_grab `Player Calling Grab`)
    (`KismetArrayLibrary.Array_RemoveItem` _player_calling_grab (`|GetArrayItem` _player_calling_grab (`KismetArrayLibrary.Array_Find` _player_calling_grab `Player Calling Grab`)))
    (goto _label)))

(fn `OnRep_IsActive`
  (bind _skeletalmesh (`self.SkeletalMesh`))
  (if (`self.IsActive`)
    (`SceneComponent.SetHiddenInGame` _skeletalmesh false false)
    (else
      (`SceneComponent.SetHiddenInGame` _skeletalmesh false false))))

(fn `OnRep_IsGrabed`
  (bind _isgrabed (`self.IsGrabed`))
  (bind _worm_grab_sfx (`self.Worm_Grab_SFX`))
  (`SceneComponent.SetHiddenInGame` (`self.Widget`) (not _isgrabed) false)
  (if _isgrabed
    (`AudioComponent.Play` _worm_grab_sfx 0.0)
    (else
      (`AudioComponent.Stop` _worm_grab_sfx))))

(fn `OnRep_MyPArent`
  (bind _myparent (`self.MyPArent`))
  (`/Engine/EditorBlueprintResources/StandardMacros.IsValid` _myparent
    (:`Is Valid`
      (set `self.MySpline` (`/Game/_Jam_MilkyWay/Players/MenuPlayer/GameRules/BP_WormSpline.Spline` _myparent))
      (set `self.IsActive` true)
      (set `/Game/_Jam_MilkyWay/Players/MenuPlayer/GameRules/BP_WormSpline.WormIsActive` true _myparent))))

(fn `OnRep_Player Calling Grab`
  (bind _player_calling_grab (`self.Player Calling Grab`))
  (if (`KismetArrayLibrary.Array_IsEmpty` _player_calling_grab)
    (set `self.IsGrabed` false)
    (else
      (`/Engine/EditorBlueprintResources/StandardMacros.IsValid` (`|GetArrayItem` _player_calling_grab)
        (:`Is Valid`
          (set `self.IsGrabed` true))))))

(fn `UserConstructionScript`)