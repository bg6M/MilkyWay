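; Spline path actor that spawns a BP_Worm and drives it along its length, registering in GS_Lobby's WormSplineBank or spawning immediately outside that game state.
; While active, the server moves the worm in a randomly chosen direction, wrapping at the ends and slowing it by grabbing-player count.
; Destruction optionally triggers loot, resets state and notifies the lobby.
; The construction script trace-snaps spline points to surfaces and scatters randomized decals along the path.
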(event `self.ReceiveBeginPlay`
  (bind _asgs_lobby (cast `/Game/_Jam_MilkyWay/Players/MenuPlayer/GS_Lobby` (`GameplayStatics.GetGameState`))
    (:`then`
      (bind _output_get (set `self.As GS Lobby` _asgs_lobby))
      (`KismetArrayLibrary.Array_Add` (`/Game/_Jam_MilkyWay/Players/MenuPlayer/GS_Lobby.WormSplineBank` _output_get) self))
    (:`CastFailed`
      (`self.SERVER_SpawnWorm`))))

(event `SERVER_SpawnWorm`
  (bind _spline (`self.Spline`))
  (bind (_returnvalue_location _returnvalue_rotation) (`KismetMathLibrary.BreakTransform` (`SceneComponent.K2_GetComponentToWorld` (`self.Spline`))))
  (set `self.ReversedSpline?` (`KismetMathLibrary.RandomBool`))
  (`/Engine/EditorBlueprintResources/StandardMacros.IsValid` (`self.MyWorm`)
    (:`Is Valid`
      (`self.Server_Destroy my Worm` false))
    (:`Is Not Valid`
      _))
  (bind _returnvalue (`|SpawnActorFromClass` "/Game/_Jam_MilkyWay/Players/MenuPlayer/GameRules/BP_Worm.BP_Worm_C" (`KismetMathLibrary.MakeTransform` _returnvalue_location _returnvalue_rotation) "AdjustIfPossibleButAlwaysSpawn" "MultiplyWithRoot" null _spline self null))
  (bind _output_get (set `self.MyWorm` _returnvalue))
  (`self.MC_SetDATA` _output_get _spline))

(event `MC_SetDATA`
  (params (Target :type "/Game/_Jam_MilkyWay/Players/MenuPlayer/GameRules/BP_Worm Object Reference") (Spline :type "SplineComponent Object Reference"))
  (`/Game/_Jam_MilkyWay/Players/MenuPlayer/GameRules/BP_Worm.SET DATA` (stale `SERVER_SpawnWorm` _returnvalue) self Spline)
  (`/Game/_Jam_MilkyWay/Players/MenuPlayer/GameRules/BP_Worm.SET DATA` Target self Spline))

(event `self.ReceiveTick`
  (params (DeltaSeconds :type "Float (single-precision)"))
  (`/Engine/EditorBlueprintResources/ActorMacros.Switch Has Authority`
    (:`Authority`
      (if (`self.WormIsActive`)
        (`self.Server_MoveOnspline`)))))

(event `Server_MoveOnspline`
  (bind _spline (`self.Spline`))
  (bind _spline_2 (`self.Spline`))
  (`/Engine/EditorBlueprintResources/ActorMacros.Switch Has Authority`
    (:`Authority`
      (bind _myworm (`self.MyWorm` :!label _label)
        (:`then`
          (set `self.Speed` (- 900 (`|GetArrayItem` (`self.SpeedModifier`) (`/Game/_Jam_MilkyWay/Players/MenuPlayer/GameRules/BP_Worm.NumPlayerGrab` _myworm))))
          (if (`self.ReversedSpline?`)
            (bind _output_get (set `self.Distance` (- (`self.Distance`) (* (`self.Speed`) (`GameplayStatics.GetWorldDeltaSeconds`)))))
            (if (<= _output_get 0.0)
              (set `self.Distance` (`SplineComponent.GetSplineLength` _spline_2))
              (else
                (`/Game/_Jam_MilkyWay/Players/MenuPlayer/GameRules/BP_Worm.ServerMoveOnspline` (`self.MyWorm`) (`SplineComponent.GetLocationAtDistanceAlongSpline` _spline_2 _output_get "World") (`SplineComponent.GetRotationAtDistanceAlongSpline` _spline_2 _output_get "World") true)))
            (else
              (bind _output_get_2 (set `self.Distance` (+ (`self.Distance`) (* (`self.Speed`) (`GameplayStatics.GetWorldDeltaSeconds`)))))
              (if (>= _output_get_2 (`SplineComponent.GetSplineLength` _spline))
                (set `self.Distance` 0.0)
                (else
                  (`/Game/_Jam_MilkyWay/Players/MenuPlayer/GameRules/BP_Worm.ServerMoveOnspline` (`self.MyWorm`) (`SplineComponent.GetLocationAtDistanceAlongSpline` _spline _output_get_2 "World") (`SplineComponent.GetRotationAtDistanceAlongSpline` _spline _output_get_2 "World") false))))))
        (:`else`)))))

(event `MC_MoveOnspline`
  (goto _label))

(event `Server_Destroy my Worm`
  (params (`Loot?` :type Boolean))
  (bind _myworm (`self.MyWorm`))
  (if `Loot?`
    (`/Game/_Jam_MilkyWay/Players/MenuPlayer/GameRules/BP_Worm.SERVER_SpawnLoot` _myworm)
    (else
      (`/Engine/EditorBlueprintResources/StandardMacros.IsValid` _myworm
        (:`Is Valid`
          (`/Game/_Jam_MilkyWay/Players/MenuPlayer/GameRules/BP_Worm.MC_DESTROY` _myworm))
        (:`Is Not Valid`
          _))))
  (set `self.WormIsActive` false)
  (set `self.Distance` 0.0)
  (set `self.MyWorm` null)
  (`/Game/_Jam_MilkyWay/Players/MenuPlayer/GS_Lobby.RPC_IsAnyWormAlive?` (`self.As GS Lobby`)))

(fn `UserConstructionScript`
  (bind _returnvalue (`KismetMathLibrary.RandomFloatInRange` 0.2 1.0))
  (`TextRenderComponent.K2_SetText` (`self.DevTool`) (`KismetTextLibrary.Conv_DoubleToText` (`SplineComponent.GetSplineLength` (`self.Spline`)) "HalfToEven"))
  (`|ExecutionSequence`
    (:`then_0`
      ;[1 1 1] SNAP DECALS TO POINT
      (for _index (range (`SplineComponent.GetNumberOfSplinePoints` (`self.Spline`)))
        (bind (_returnvalue_x _returnvalue_y _returnvalue_z) (`KismetMathLibrary.BreakVector` (`SplineComponent.GetLocationAtSplinePoint` (`self.Spline`) _index "World")))
        (bind (_returnvalue_x_2 _returnvalue_y_2 _returnvalue_z_2) (`KismetMathLibrary.BreakVector` (`SplineComponent.GetLocationAtSplinePoint` (`self.Spline`) _index "World")))
        (bind (_outhit _returnvalue_2) (`KismetSystemLibrary.LineTraceSingle` :`Start` (`KismetMathLibrary.MakeVector` _returnvalue_x _returnvalue_y (+ _returnvalue_z (`self.DecalSnapThreshold`))) :`End` (`KismetMathLibrary.MakeVector` _returnvalue_x_2 _returnvalue_y_2 (- _returnvalue_z_2 (`self.DecalSnapThreshold`))) :`TraceChannel` "TraceTypeQuery1" :`DrawDebugType` "ForDuration" :`DrawTime` 2.0))
        (if _returnvalue_2
          (`SplineComponent.SetLocationAtSplinePoint` (`self.Spline`) _index (`.Location` (`GameplayStatics.BreakHitResult` _outhit)) "World" true))))
    (:`then_1`
      (for _index_2 (range (+ (`KismetMathLibrary.FTrunc` (/ (`SplineComponent.GetSplineLength` (`self.Spline`)) 512.0)) 1))
        (bind _returnvalue_3 (`AddComponent|NODE_AddDecalComponent-0` :`RelativeTransform` (`KismetMathLibrary.MakeTransform` (0.0 0.0 0.0) (struct :`Pitch` 90.0) (`KismetMathLibrary.MakeVector` 1.0 _returnvalue _returnvalue))))
        (`SceneComponent.K2_SetWorldLocationAndRotation` _returnvalue_3 (`SplineComponent.GetLocationAtDistanceAlongSpline` (`self.Spline`) (`KismetMathLibrary.Conv_IntToDouble` (* _index_2 512)) "World") (`KismetMathLibrary.MakeRotator` 0.0 90.0 (`KismetMathLibrary.RandomFloatInRange` 0.0 360.0)) false false)
        (`DecalComponent.SetDecalMaterial` _returnvalue_3 (`|GetArrayItem` (`self.DecalToPlace`) (`KismetMathLibrary.Clamp` (`KismetMathLibrary.RandomInteger` 3) 0 3)))))))