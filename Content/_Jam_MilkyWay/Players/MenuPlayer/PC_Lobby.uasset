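; Lobby player controller that opens the lobby UI and relays player actions for the MANZ and GREEZ teams, including game start and QTE success.
; Server and multicast events replicate each team's grab, with Tick re-sending it while held and BP_Worm exempt from attachment.
; Cage-code consoles use view blending and a widget-interaction pointer.
; Onset VOIP provides proximity chat, MANZ channel, radio and alien effects, and amplitude-driven mouth values.
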(event `/Game/_Jam_MilkyWay/Players/FirstPerson/Blueprints/Interface/BPI_Interaction.QTE SUCCESS CHECK`
  (params (`Actor to Trigger` :type "Actor Object Reference") (`Success?` :type Boolean))
  ;[1 1 1 1 75] QTE SUCCESS REPLICATION
  (bind _output_get (set `self.Success?` `Success?`))
  (if _output_get
    (`self.RPC_SucessQTE` `Actor to Trigger` _output_get)))

(event `RPC_SucessQTE`
  (params (`Actor to Trigger` :type "Actor Object Reference") (`Success?` :type Boolean))
  ;[1 1 1 1 75] QTE SUCCESS REPLICATION
  (`/Game/_Jam_MilkyWay/Players/MenuPlayer/GS_Lobby.RPC_QTETRIGGER` (`self.As GS Lobby`) null true))

(event `Client_Widget_Message`
  (params (Text :type Text) (Duration :type "Float (single-precision)"))
  (bind _mymessagewidget (`self.MyMessageWidget`))
  (`/Engine/EditorBlueprintResources/StandardMacros.IsValid` _mymessagewidget
    (:`Is Valid`
      (`Widget.RemoveFromParent` _mymessagewidget)
      (set `self.MyMessageWidget` null))
    (:`Is Not Valid`
      _))
  (bind _returnvalue (`|CreateWidget` "/Game/_Jam_MilkyWay/Players/MenuPlayer/GameWidgets/W_GameStateMesage.W_GameStateMesage_C"))
  (bind _output_get (set `self.MyMessageWidget` _returnvalue))
  (`UserWidget.AddToViewport` _output_get 0)
  (`/Game/_Jam_MilkyWay/Players/MenuPlayer/GameWidgets/W_GameStateMesage.SET FONT BY TEAM` _returnvalue (`/Game/_Jam_MilkyWay/Players/FirstPerson/Blueprints/BP_Player.Team` (`self.MyBpPlayer`)))
  (`/Game/_Jam_MilkyWay/Players/MenuPlayer/GameWidgets/W_GameStateMesage.Activate` _output_get Text Duration))

(event `ServerStargame`
  ;[1 1 1] START GAME
  (`/Engine/EditorBlueprintResources/ActorMacros.Switch Has Authority`
    (:`Authority`
      (`/Game/_Jam_MilkyWay/Players/MenuPlayer/GM_Lobby.Server Start Game` (`/Game/_Jam_MilkyWay/Players/MenuPlayer/GS_Lobby.As GM Lobby` (`self.As GS Lobby`))))))

(event `Key|AnyKey`
  (params (Key :type "Key Structure"))
  (bind _widgetinteraction_pointer (`/Game/_Jam_MilkyWay/Players/FirstPerson/Blueprints/BP_Player.WidgetInteraction_POINTER` (`self.MyBpPlayer`)))
  (bind _returnvalue (`ActorComponent.IsActive` _widgetinteraction_pointer))
  ;[1 1 1 1 100] CAGE CODE REPLICATION
  (:`Pressed`
    (if _returnvalue
      (`WidgetInteractionComponent.PressKey` _widgetinteraction_pointer Key false)
      (`Widget.SetKeyboardFocus` (`WidgetComponent.GetUserWidgetObject` (`WidgetInteractionComponent.GetHoveredWidgetComponent` _widgetinteraction_pointer)) :!label _label)))
  (:`Released`
    (if _returnvalue
      (`WidgetInteractionComponent.ReleaseKey` _widgetinteraction_pointer Key)
      (goto _label))))

(event `TRYVALIDATECAGECODE`
  (params (Code :type String) (MyActor :type "/Game/_Jam_MilkyWay/Players/MenuPlayer/GameRules/BP_CageActivator Object Reference"))
  (bind _returnvalue (`self.K2_GetActorLocation` (`self.MyBpPlayer`)))
  ;[1 1 1 1 100] CAGE CODE REPLICATION
  (if (== Code (`/Game/_Jam_MilkyWay/Players/MenuPlayer/GS_Lobby.CageCode` (`self.As GS Lobby`)))
    (`/Game/_Jam_MilkyWay/Players/MenuPlayer/GameRules/BP_CageActivator.ACTIVATE` MyActor)
    (`GameplayStatics.PlaySoundAtLocation` "/Game/_Jam_MilkyWay/SFX/GPE/Terminal/Terminal_Granted__SFX.Terminal_Granted__SFX" _returnvalue (struct) 1.0 1.0 0.0 null null null null)
    (else
      (`GameplayStatics.PlaySoundAtLocation` "/Game/_Jam_MilkyWay/SFX/GPE/Terminal/Terminal_Denied__SFX.Terminal_Denied__SFX" _returnvalue (struct) 1.0 1.0 0.0 null null null null)))
  (`/Game/_Jam_MilkyWay/Players/MenuPlayer/GameRules/BP_CageActivator.ExitConsole` MyActor))

(event `W_StartGameTimer`
  ;[1 1 1] START GAME
  (bind _returnvalue (`|CreateWidget` "/Game/_Jam_MilkyWay/Players/MenuPlayer/W_TimerStartGame.W_TimerStartGame_C"))
  (`UserWidget.AddToViewport` _returnvalue 0))

(event `self.ReceiveBeginPlay`
  (bind _returnvalue (`GameplayStatics.GetPlayerController` 0))
  (bind _returnvalue_2 (subsystem `EnhancedInputLocalPlayerSubsystem`))
  (bind _returnvalue_3 (subsystem `EnhancedInputLocalPlayerSubsystem`))
  ;[0.1782 0.5827 1 1 150] BEGINPLAY
  (bind _asbp_game_instance (cast `/Game/_Jam_MilkyWay/Players/FirstPerson/Blueprints/BP_GameInstance` (`GameplayStatics.GetGameInstance`)))
  (bind _output_get (set `self.As BP Game Instance` _asbp_game_instance))
  (bind _savegamedata (`/Game/_Jam_MilkyWay/Players/FirstPerson/Blueprints/BP_GameInstance.GetGameData` _output_get))
  (bind _output_get_2 (set `self.Save Game Data` _savegamedata))
  (set `self.Player Customisation` (`/Game/_Jam_MilkyWay/Players/SaveGame/BP_SaveGame.PlayerCustomisation` _output_get_2))
  (bind _asgs_lobby (cast `/Game/_Jam_MilkyWay/Players/MenuPlayer/GS_Lobby` (`GameplayStatics.GetGameState`))
    (:`then`
      (set `self.As GS Lobby` _asgs_lobby)
      (`/Engine/EditorBlueprintResources/StandardMacros.IsValid` _returnvalue_3
        (:`Is Valid`
          (`EnhancedInputSubsystemInterface.AddMappingContext` _returnvalue_3 "/Game/_Jam_MilkyWay/Players/FirstPerson/Inputs/IMC_Default.IMC_Default" 0 (struct))
          (`/Engine/EditorBlueprintResources/StandardMacros.IsValid` _returnvalue :!label _label_2
            (:`Is Valid`
              (bind _returnvalue_4 (`|CreateWidget` "/Game/_Jam_MilkyWay/Players/MenuPlayer/W_Lobby.W_Lobby_C" self self))
              (bind _output_get_3 (set `self.MyLobbyWidget` _returnvalue_4))
              (`UserWidget.AddToViewport` _output_get_3 0)
              (`WidgetBlueprintLibrary.SetInputMode_UIOnlyEx` _returnvalue _output_get_3 "DoNotLock" true)
              (set `PlayerController.bShowMouseCursor` true (`GameplayStatics.GetPlayerController` 0)))
            (:`Is Not Valid`
              (`KismetSystemLibrary.Delay` 3.0)
              (goto _label_2))))))
    (:`CastFailed`
      (`/Engine/EditorBlueprintResources/StandardMacros.IsValid` _returnvalue_2
        (:`Is Valid`
          (`EnhancedInputSubsystemInterface.AddMappingContext` _returnvalue_2 "/Game/_Jam_MilkyWay/Players/FirstPerson/Inputs/IMC_Default.IMC_Default" 0 (struct)))))))

(event `Server_SendCutsomization`)

(event `Client_ReturnToMenu`)

(event `/Game/_Jam_MilkyWay/Players/FirstPerson/Blueprints/Interface/BPI_Interaction.Interact_Int`
  (params (Bp_Player :type "/Game/_Jam_MilkyWay/Players/FirstPerson/Blueprints/BP_Player Object Reference"))
  (bind _mylobbywidget (`self.MyLobbyWidget`))
  ;[1 1 1] START GAME
  (`/Engine/EditorBlueprintResources/StandardMacros.IsValid` _mylobbywidget
    (:`Is Valid`
      (`Widget.RemoveFromParent` _mylobbywidget))))

(event `CreateCodeCageWidget`
  (params (MyActor :type "/Game/_Jam_MilkyWay/Players/MenuPlayer/GameRules/BP_CageActivator Object Reference") (MyConsoleWidget :type "/Game/_Jam_MilkyWay/Players/MenuPlayer/GameWidgets/W_CageCodeManz Object Reference"))
  ;[1 1 1 1 100] CAGE CODE REPLICATION
  (`GameplayStatics.PlaySoundAtLocation` "/Game/_Jam_MilkyWay/SFX/GPE/Terminal/Terminal_Interact__SFX.Terminal_Interact__SFX" (`self.K2_GetActorLocation` (`self.MyBpPlayer`)) (struct) 1.0 1.0 0.0 null null null null)
  (`self.SetViewTargetWithBlend` MyActor)
  (`ActorComponent.Activate` (`/Game/_Jam_MilkyWay/Players/FirstPerson/Blueprints/BP_Player.WidgetInteraction_POINTER` (`self.MyBpPlayer`)) true)
  (bind _asw_cage_code_manz (cast `/Game/_Jam_MilkyWay/Players/MenuPlayer/GameWidgets/W_CageCodeManz` (`WidgetComponent.GetUserWidgetObject` (`/Game/_Jam_MilkyWay/Players/MenuPlayer/GameRules/BP_CageActivator.ScreenWidget` MyActor))))
  (bind _output_get (set `self.MyConsoleWidget` _asw_cage_code_manz))
  (`WidgetBlueprintLibrary.SetInputMode_GameAndUIEx` self _output_get "DoNotLock" false)
  (set `self.bShowMouseCursor` true)
  (`Widget.SetKeyboardFocus` _output_get)
  (`Widget.SetKeyboardFocus` (`WidgetComponent.GetUserWidgetObject` (`WidgetInteractionComponent.GetHoveredWidgetComponent` (`/Game/_Jam_MilkyWay/Players/FirstPerson/Blueprints/BP_Player.WidgetInteraction_POINTER` (`self.MyBpPlayer`))))))

(event `ExitCodeCageWidget`
  ;[1 1 1 1 100] CAGE CODE REPLICATION
  (`/Game/_Jam_MilkyWay/Players/MenuPlayer/GameRules/BP_CageActivator.ExitConsole` (`/Game/_Jam_MilkyWay/Players/MenuPlayer/GameWidgets/W_CageCodeManz.MyActor` (`self.MyConsoleWidget`)))
  (`self.SetViewTargetWithBlend` (`self.MyBpPlayer`))
  (`WidgetBlueprintLibrary.SetInputMode_GameOnly` self)
  (set `self.bShowMouseCursor` false)
  (`ActorComponent.Deactivate` (`/Game/_Jam_MilkyWay/Players/FirstPerson/Blueprints/BP_Player.WidgetInteraction_POINTER` (`self.MyBpPlayer`))))

(event `self.ReceiveTick`
  (params (DeltaSeconds :type "Float (single-precision)"))
  ;[1 0 0.8389 1 150] EVENT TICK
  (bind _mybpplayer (`self.MyBpPlayer`)
    (:`then`
      (`|ExecutionSequence`
        (:`then_0`
          (`/Game/_Jam_MilkyWay/Players/FirstPerson/Blueprints/BP_Player.MyGrabedActor` _mybpplayer
            (:`then`
              (if (`self.ActivateGrabReplication`)
                (`self.RPC GRAB TRANSFORM`)))
            (:`else`)))
        (:`then_1`
          (set `/Game/_Jam_MilkyWay/Players/FirstPerson/Blueprints/BP_Player.MoutValue` (`self.GetMouthVolume`) _mybpplayer)
          (`/Game/_Jam_MilkyWay/Players/FirstPerson/Blueprints/BP_Player.MyController` _mybpplayer
            (:`then`)
            (:`else`
              (set `/Game/_Jam_MilkyWay/Players/FirstPerson/Blueprints/BP_Player.MyController` self _mybpplayer))))))
    (:`else`)))

(event `/Game/_Jam_MilkyWay/Players/FirstPerson/Blueprints/Interface/BPI_Interaction.AskVOIPAmp`
  (params (BP_Player :type "/Game/_Jam_MilkyWay/Players/FirstPerson/Blueprints/BP_Player Object Reference"))
  ;[0.09306 0.1221 0.9216 1 150] VOIP
  (`self.RPC_UpdateMouth` BP_Player))

(event `RPC_UpdateMouth`
  (params (Target :type "/Game/_Jam_MilkyWay/Players/FirstPerson/Blueprints/BP_Player Object Reference"))
  ;[0.09306 0.1221 0.9216 1 150] VOIP
  (`self.MC_UpdateMouth` Target))

(event `MC_UpdateMouth`
  (params (Target :type "/Game/_Jam_MilkyWay/Players/FirstPerson/Blueprints/BP_Player Object Reference"))
  ;[0.09306 0.1221 0.9216 1 150] VOIP
  (set `/Game/_Jam_MilkyWay/Players/FirstPerson/Blueprints/BP_Player.MoutValue` (`self.GetMouthVolume`) Target))

(event `Toggle Proxi Chat`
  (bind _returnvalue (subsystem `OnsetVoipLocalPlayerSubsystem`))
  ;[0.09306 0.1221 0.9216 1 150] VOIP
  (`/Engine/EditorBlueprintResources/StandardMacros.IsValid` _returnvalue :!label _label_3
    (:`Is Valid`
      (bind _returnvalue_2 (`OnsetVoipLocalPlayerSubsystem.ToggleVoiceCaptureWithChannel` _returnvalue true 0))
      (set `self.ChatEnable` _returnvalue_2))
    (:`Is Not Valid`
      (`KismetSystemLibrary.Delay` 1.0)
      (goto _label_3))))

(event `Initialize VOIP`
  (params (Team :type "/Game/_Jam_MilkyWay/Players/MenuPlayer/E_PlayersTeam Enum" :default "NewEnumerator0"))
  (bind _returnvalue (`OnsetVoipWorldSubsystem.GetVoipTalker` (subsystem `OnsetVoipWorldSubsystem`) (`self.PlayerState`)))
  ;[0.09306 0.1221 0.9216 1 150] VOIP
  (`self.PlayerState` :!label _label_4
    (:`then`
      (`OnsetVoipTalker.SetVoiceChannel` _returnvalue 0 true)
      (switch `/Game/_Jam_MilkyWay/Players/MenuPlayer/E_PlayersTeam` Team
        (:`NewEnumerator0`
          (`OnsetVoipTalker.SetVoiceChannel` _returnvalue 5 true))
        (:`NewEnumerator1`
          _))
      (`self.Toggle Proxi Chat`))
    (:`else`
      (`KismetSystemLibrary.Delay` 0.5)
      (goto _label_4))))

(event `GetMouthValue`
  (bind _returnvalue (subsystem `OnsetVoipLocalPlayerSubsystem`))
  ;[0.09306 0.1221 0.9216 1 150] VOIP
  (if (`OnsetVoipLocalPlayerSubsystem.IsCapturingVoice` _returnvalue)
    (set `self.MouthVolume` (`OnsetVoipLocalPlayerSubsystem.GetCurrentAmplitude` _returnvalue))
    (else
      (set `self.MouthVolume` 0.0))))

(event `Server_AlienVoice`
  ;[0.09306 0.1221 0.9216 1 150] VOIP
  (set `SoundBase.SourceEffectChain` "/Game/_Jam_MilkyWay/SFX/SEPC_ALIEN.SEPC_ALIEN" (`OnsetVoipAudioComponent.VoipSoundWave` (`OnsetVoipTalker.GetVoiceAudioComponent` (`OnsetVoipWorldSubsystem.GetVoipTalker` (subsystem `OnsetVoipWorldSubsystem`) (`self.PlayerState`)) "RELEVANT_3D"))))

(event `Server_ToggleRadio`
  (params (bCapture :type Boolean) (Team :type "/Game/_Jam_MilkyWay/Players/MenuPlayer/E_PlayersTeam Enum" :default "NewEnumerator0"))
  ;[0.09306 0.1221 0.9216 1 150] VOIP
  (if (not bCapture)
    (`self.Initialize VOIP` "NewEnumerator0"))
  (`self.MC_ToggleRadio` bCapture))

(event `MC_ToggleRadio`
  (params (bCapture :type Boolean))
  (bind _voipsoundwave (`OnsetVoipAudioComponent.VoipSoundWave` (`OnsetVoipTalker.GetVoiceAudioComponent` (`OnsetVoipWorldSubsystem.GetVoipTalker` (subsystem `OnsetVoipWorldSubsystem`) (`self.PlayerState`)) "RELEVANT_2D")))
  ;[0.09306 0.1221 0.9216 1 150] VOIP
  (if bCapture
    (set `SoundBase.SourceEffectChain` "/OnsetVoip/SEPC_VoIP_Radio.SEPC_VoIP_Radio" _voipsoundwave)
    (`OnsetVoipLocalPlayerSubsystem.ToggleVoiceCapture` (subsystem `OnsetVoipLocalPlayerSubsystem`) true)
    (else
      (set `SoundBase.SourceEffectChain` null _voipsoundwave))))

(event `Key|V`
  (params (Key :type "Key Structure"))
  (bind _voipsettingswidget (`self.VOIPSettingsWidget`))
  ;[0.09306 0.1221 0.9216 1 150] VOIP
  (:`Pressed`
    (`/Engine/EditorBlueprintResources/StandardMacros.IsValid` _voipsettingswidget
      (:`Is Valid`
        (`/Game/_Jam_MilkyWay/Players/MenuPlayer/GameWidgets/W_VOIPSettings.CloseWidget` _voipsettingswidget)
        (set `self.VOIPSettingsWidget` null))
      (:`Is Not Valid`
        (bind _returnvalue (`|CreateWidget` "/Game/_Jam_MilkyWay/Players/MenuPlayer/GameWidgets/W_VOIPSettings.W_VOIPSettings_C"))
        (bind _output_get (set `self.VOIPSettingsWidget` _returnvalue))
        (`UserWidget.AddToViewport` _output_get 0)))))

(event `Server_LeaveTeamChat`
  ;[0.09306 0.1221 0.9216 1 150] VOIP
)

(event `RPC_ManzSwitchItem`
  (params (ItemIndex :type Integer))
  ;[1 1 1 1 100] MANZ SWITCH ITEM
  (bind _output_get (set `/Game/_Jam_MilkyWay/Players/FirstPerson/Blueprints/BP_Player.ItemIndex` ItemIndex (`self.MyBpPlayer`)))
  (`self.MC_ManzSwitchItem` _output_get))

(event `Manz_ForceUngrab`
  (params (MyPlayer :type "/Game/_Jam_MilkyWay/Players/FirstPerson/Blueprints/BP_Player Object Reference") (`Exhausted?` :type Boolean))
  ;[1 1 1 1 150] MANZ UNGRAB
  (`self.RPC GRAB ACTIVATION` false)
  (`self.MC_Manz_ForceUngrab` MyPlayer `Exhausted?`))

(event `RPC MANZ GRAB`
  (params (Actor :type "Actor Object Reference"))
  ;[1 1 1 1 150] MANZ GRAB
  ;;[1 1 1 1 50] SERVER
  (`/Engine/EditorBlueprintResources/StandardMacros.IsValid` (`/Game/_Jam_MilkyWay/Players/FirstPerson/Blueprints/BP_Player.MyGrabedActor` (`self.MyBpPlayer`))
    (:`Is Valid`
      _)
    (:`Is Not Valid`
      (bind _output_get (set `/Game/_Jam_MilkyWay/Players/FirstPerson/Blueprints/BP_Player.MyGrabedActor` Actor (`self.MyBpPlayer`)))
      (message `/Game/_Jam_MilkyWay/Players/FirstPerson/Blueprints/Interface/BPI_Grab.Grab Interface` _output_get (`self.MyBpPlayer`) "NewEnumerator0")))
  (`self.RPC GRAB ACTIVATION` true)
  (`self.MC_ManzGrab` Actor))

(event `MC_ManzSwitchItem`
  (params (Index :type Integer))
  ;[1 1 1 1 100] MANZ SWITCH ITEM
  (message `/Game/_Jam_MilkyWay/Players/FirstPerson/Blueprints/Interface/BPI_AnimeReplication.Set Item Index Anim BP` (`/Game/_Jam_MilkyWay/Players/FirstPerson/Blueprints/BP_Player.Manz_TPS_Mesh` (`self.MyBpPlayer`)) Index))

(event `MC_Manz_ForceUngrab`
  (params (Player :type "/Game/_Jam_MilkyWay/Players/FirstPerson/Blueprints/BP_Player Object Reference") (GradExausht :type Boolean))
  (bind _mybpplayer (`self.MyBpPlayer`))
  (bind _mygrabedactor (`/Game/_Jam_MilkyWay/Players/FirstPerson/Blueprints/BP_Player.MyGrabedActor` _mybpplayer))
  ;[1 1 1 1 150] MANZ UNGRAB
  (if (!= (`GameplayStatics.GetObjectClass` _mygrabedactor) "/Game/_Jam_MilkyWay/Players/MenuPlayer/GameRules/BP_Worm.BP_Worm_C")
    (`self.K2_DetachFromActor` _mygrabedactor "KeepWorld" "KeepWorld" "KeepRelative"))
  (message `/Game/_Jam_MilkyWay/Players/FirstPerson/Blueprints/Interface/BPI_Grab.UnGrab Interface` _mygrabedactor _mybpplayer)
  (`self.MC_Replicate BPI GRAB ONCE` false)
  (set `/Game/_Jam_MilkyWay/Players/FirstPerson/Blueprints/BP_Player.MyGrabedActor` null _mybpplayer)
  (bind _output_get (set `/Game/_Jam_MilkyWay/Players/FirstPerson/Blueprints/BP_Player.GradExausht` GradExausht _mybpplayer))
  (set `/Game/_Jam_MilkyWay/Players/FirstPerson/Blueprints/BP_Player.GunFire` false _mybpplayer)
  (`/Game/_Jam_MilkyWay/Players/FirstPerson/Blueprints/BP_Player.RPCVFXGUN` _mybpplayer false)
  (if _output_get
    (`KismetSystemLibrary.Delay` 3.0)
    (set `/Game/_Jam_MilkyWay/Players/FirstPerson/Blueprints/BP_Player.GradExausht` false _mybpplayer)))

(event `MC_ManzGrab`
  (params (A :type "Object Object Reference"))
  (bind _mybpplayer (`self.MyBpPlayer`))
  (bind _mybpplayer_2 (`self.MyBpPlayer`))
  (bind _mygrabedactor (`/Game/_Jam_MilkyWay/Players/FirstPerson/Blueprints/BP_Player.MyGrabedActor` (`self.MyBpPlayer`)))
  ;[1 1 1 1 150] MANZ GRAB
  ;;[1 1 1 1 50] MC MANZ GRAB
  (`/Engine/EditorBlueprintResources/StandardMacros.IsValid` _mygrabedactor
    (:`Is Valid`
      (set `/Game/_Jam_MilkyWay/Players/FirstPerson/Blueprints/BP_Player.GunFire` true _mybpplayer_2)
      (`/Game/_Jam_MilkyWay/Players/FirstPerson/Blueprints/BP_Player.RPCVFXGUN` _mybpplayer_2 true)
      (`self.MC_Replicate BPI GRAB ONCE` true)
      (`/Game/_Jam_MilkyWay/Players/FirstPerson/Blueprints/BP_Player.RPC_Replicate FX gun trail` _mybpplayer_2)
      (if (!= (`GameplayStatics.GetObjectClass` _mygrabedactor) "/Game/_Jam_MilkyWay/Players/MenuPlayer/GameRules/BP_Worm.BP_Worm_C")
        (`self.K2_AttachToComponent` (`/Game/_Jam_MilkyWay/Players/FirstPerson/Blueprints/BP_Player.MyGrabedActor` _mybpplayer) (`/Game/_Jam_MilkyWay/Players/FirstPerson/Blueprints/BP_Player.Manz_Grab_Fps_Location` _mybpplayer) "None" "SnapToTarget" "KeepWorld" "KeepRelative" true)))))

(event `RPC MANZ NO GRAB DETECTED`
  ;[1 1 1] RPC NO GRAB DETECTED
  (`/Game/_Jam_MilkyWay/Players/FirstPerson/Blueprints/BP_Player.RPCVFXGUN` (`self.MyBpPlayer`) true))

(event `RPC_PitchnYaw`
  (`self.MC_PitchNYaw`))

(event `MC_PitchNYaw`
  (set `self.RemoteViewPitch` (.pitch (`self.GetControlRotation`))))

(event `RPC GRAB TRANSFORM`
  (bind _mybpplayer (`self.MyBpPlayer`))
  (bind _mygrabedactor (`/Game/_Jam_MilkyWay/Players/FirstPerson/Blueprints/BP_Player.MyGrabedActor` _mybpplayer))
  (switch `/Game/_Jam_MilkyWay/Players/MenuPlayer/E_PlayersTeam` (`/Game/_Jam_MilkyWay/Players/FirstPerson/Blueprints/BP_Player.Team` _mybpplayer)
    (:`NewEnumerator0`
      (`self.MC_ManzGrab` _mygrabedactor))
    (:`NewEnumerator1`
      (`self.MC_GreezGrab` _mygrabedactor))))

(event `RPC GRAB ACTIVATION`
  (params (`ON/OFF` :type Boolean))
  (if (!= (`GameplayStatics.GetObjectClass` (`/Game/_Jam_MilkyWay/Players/FirstPerson/Blueprints/BP_Player.MyGrabedActor` (`self.MyBpPlayer`))) "/Game/_Jam_MilkyWay/Players/MenuPlayer/GameRules/BP_Worm.BP_Worm_C")
    (set `self.ActivateGrabReplication` `ON/OFF`)
    (else
      (set `self.ActivateGrabReplication` false))))

(event `RPC_GREEZUNGRAB`
  (`self.MC_GREEZUNGRAB`))

(event `RPC_GREEZGRAB`
  (params (Actor :type "Actor Object Reference"))
  ;[1 1 1 1 150] GREEZ GRAB
  ;;[1 1 1 1 50] SERVER
  (`/Engine/EditorBlueprintResources/StandardMacros.IsValid` (`/Game/_Jam_MilkyWay/Players/FirstPerson/Blueprints/BP_Player.MyGrabedActor` (`self.MyBpPlayer`))
    (:`Is Valid`
      _)
    (:`Is Not Valid`
      (bind _output_get (set `/Game/_Jam_MilkyWay/Players/FirstPerson/Blueprints/BP_Player.MyGrabedActor` Actor (`self.MyBpPlayer`)))
      (message `/Game/_Jam_MilkyWay/Players/FirstPerson/Blueprints/Interface/BPI_Grab.Grab Interface` _output_get (`self.MyBpPlayer`) "NewEnumerator1")))
  (`self.RPC GRAB ACTIVATION` true)
  (`self.MC_GreezGrab` Actor))

(event `MC_GREEZUNGRAB`
  (bind _mybpplayer (`self.MyBpPlayer`))
  (bind _mybpplayer_2 (`self.MyBpPlayer`))
  (bind _mygrabedactor (`/Game/_Jam_MilkyWay/Players/FirstPerson/Blueprints/BP_Player.MyGrabedActor` _mybpplayer))
  (`/Engine/EditorBlueprintResources/StandardMacros.IsValid` _mygrabedactor
    (:`Is Valid`
      (message `/Game/_Jam_MilkyWay/Players/FirstPerson/Blueprints/Interface/BPI_Grab.UnGrab Interface` _mygrabedactor _mybpplayer)
      (set `/Game/_Jam_MilkyWay/Players/FirstPerson/Blueprints/BP_Player.MyGrabedActor` null _mybpplayer_2)
      (set `/Game/_Jam_MilkyWay/Players/FirstPerson/Blueprints/BP_Player.Grab On/Off` false _mybpplayer_2)
      (`/Game/_Jam_MilkyWay/Players/FirstPerson/Blueprints/BP_Player.ReplicateGrabedActorTransform` _mybpplayer_2 false)
      (`self.MC_Replicate BPI GRAB ONCE` false "NewEnumerator1"))))

(event `MC_GreezGrab`
  (params (A :type "Object Object Reference"))
  ;[1 1 1 1 150] GREEZ GRAB
  ;;[1 1 1 1 50] MC_GREEZGRAB
  (`/Engine/EditorBlueprintResources/StandardMacros.IsValid` (`/Game/_Jam_MilkyWay/Players/FirstPerson/Blueprints/BP_Player.MyGrabedActor` (`self.MyBpPlayer`))
    (:`Is Valid`
      (set `/Game/_Jam_MilkyWay/Players/FirstPerson/Blueprints/BP_Player.Grab On/Off` true (`self.MyBpPlayer`))
      (if (!= A "/Game/_Jam_MilkyWay/Players/MenuPlayer/GameRules/BP_Worm.BP_Worm")
        (`self.MC_Replicate BPI GRAB ONCE` true "NewEnumerator1")
        (else
          (`self.RPC_GREEZUNGRAB`))))))

(event `MC_Replicate BPI GRAB ONCE`
  (params (`On/Off` :type Boolean) (PlayerTeam :type "/Game/_Jam_MilkyWay/Players/MenuPlayer/E_PlayersTeam Enum" :default "NewEnumerator0"))
  (bind _mybpplayer (`self.MyBpPlayer`))
  (bind _mybpplayer_2 (`self.MyBpPlayer`))
  (bind _returnvalue (`self.K2_GetActorLocation` (`self.MyBpPlayer`)))
  (bind _returnvalue_2 (`self.K2_GetActorLocation` (`self.MyBpPlayer`)))
  (bind _mygrabedactor (`/Game/_Jam_MilkyWay/Players/FirstPerson/Blueprints/BP_Player.MyGrabedActor` _mybpplayer))
  (bind _mygrabedactor_2 (`/Game/_Jam_MilkyWay/Players/FirstPerson/Blueprints/BP_Player.MyGrabedActor` _mybpplayer))
  (if `On/Off`
    (`/Engine/EditorBlueprintResources/StandardMacros.DoOnce` false :!label _label_5
      (:`Completed`
        (switch `/Game/_Jam_MilkyWay/Players/MenuPlayer/E_PlayersTeam` PlayerTeam
          (:`NewEnumerator0`
            (`GameplayStatics.PlaySoundAtLocation` "/Game/_Jam_MilkyWay/SFX/GPE/ItemGrab_SFX.ItemGrab_SFX" _returnvalue_2 (struct) 1.0 1.0 0.0 null null null null))
          (:`NewEnumerator1`
            (`GameplayStatics.PlaySoundAtLocation` "/Game/_Jam_MilkyWay/SFX/GPE/Alien/Alien_Telekinesis_SFX.Alien_Telekinesis_SFX" _returnvalue_2 (struct) 1.0 1.0 0.0 null null null null)
            (if (`/Game/_Jam_MilkyWay/Players/FirstPerson/Blueprints/BP_Player.IsFufu` _mybpplayer_2)
              (`/Game/_Jam_MilkyWay/Players/FirstPerson/Blueprints/BP_Player.ActiveStealth` _mybpplayer_2 false)))
          (:`NewEnumerator2`
            _))
        (message `/Game/_Jam_MilkyWay/Players/FirstPerson/Blueprints/Interface/BPI_Grab.Grab Interface` _mygrabedactor_2 _mybpplayer PlayerTeam)
        (if (!= (`GameplayStatics.GetObjectClass` _mygrabedactor_2) "/Game/_Jam_MilkyWay/Players/MenuPlayer/GameRules/BP_Worm.BP_Worm_C")
          (switch `/Game/_Jam_MilkyWay/Players/MenuPlayer/E_PlayersTeam` PlayerTeam
            (:`NewEnumerator0`
              (`self.K2_AttachToComponent` _mygrabedactor (`/Game/_Jam_MilkyWay/Players/FirstPerson/Blueprints/BP_Player.Manz_Grab_Fps_Location` _mybpplayer) "None" "SnapToTarget" "KeepWorld" "KeepRelative" true))
            (:`NewEnumerator1`
              (`self.K2_AttachToComponent` _mygrabedactor (`/Game/_Jam_MilkyWay/Players/FirstPerson/Blueprints/BP_Player.Greez_Grab_Fps_Location` _mybpplayer) "None" "SnapToTarget" "KeepWorld" "KeepRelative" true))))))
    (else
      (`self.RPC GRAB ACTIVATION` false)
      (switch `/Game/_Jam_MilkyWay/Players/MenuPlayer/E_PlayersTeam` PlayerTeam
        (:`NewEnumerator0`
          (`GameplayStatics.PlaySoundAtLocation` "/Game/_Jam_MilkyWay/SFX/GPE/ItemDrop_SFX.ItemDrop_SFX" _returnvalue (struct) 1.0 1.0 0.0 null null null null)
          (goto _label_5 :!via `Reset`))
        (:`NewEnumerator1`
          (`GameplayStatics.PlaySoundAtLocation` "/Game/_Jam_MilkyWay/SFX/GPE/Alien/Alien_UnGrab_SFX.Alien_UnGrab_SFX" _returnvalue (struct) 1.0 1.0 0.0 null null null null)
          (goto _label_5 :!via `Reset`))))))

(fn `GetMouthVolume`
  (returns (MouthVolume :type "Float (single-precision)"))
  (bind _returnvalue (subsystem `OnsetVoipLocalPlayerSubsystem`))
  (`/Engine/EditorBlueprintResources/StandardMacros.IsValid` _returnvalue
    (:`Is Valid`
      (return (`KismetMathLibrary.FClamp` (* (`OnsetVoipLocalPlayerSubsystem.GetCurrentAmplitude` _returnvalue) 2.0))))
    (:`Is Not Valid`
      (return 0.0))))

(fn `OnRep_RemoteViewPitch`
  (bind _mybpplayer (`self.MyBpPlayer`))
  (`/Engine/EditorBlueprintResources/StandardMacros.IsValid` _mybpplayer
    (:`Is Valid`
      (`SceneComponent.K2_SetWorldRotation` (`/Game/_Jam_MilkyWay/Players/FirstPerson/Blueprints/BP_Player.GrabSpringArm` _mybpplayer) (`KismetMathLibrary.MakeRotator` 0.0 (.pitch (`self.GetControlRotation`)) (.yaw (`self.GetControlRotation`))) false false)
      (`SceneComponent.K2_SetWorldRotation` (`/Game/_Jam_MilkyWay/Players/FirstPerson/Blueprints/BP_Player.ManzGrabSpringArm` _mybpplayer) (`KismetMathLibrary.MakeRotator` 0.0 (.pitch (`self.GetControlRotation`)) (.yaw (`self.GetControlRotation`))) false false)
      (`SceneComponent.K2_SetWorldRotation` (`/Game/_Jam_MilkyWay/Players/FirstPerson/Blueprints/BP_Player.GreezCamera` _mybpplayer) (`KismetMathLibrary.MakeRotator` 0.0 (.pitch (`self.GetControlRotation`)) (.yaw (`self.GetControlRotation`))) false false)
      (`SceneComponent.K2_SetWorldRotation` (`/Game/_Jam_MilkyWay/Players/FirstPerson/Blueprints/BP_Player.ManzCamera` _mybpplayer) (`KismetMathLibrary.MakeRotator` 0.0 (.pitch (`self.GetControlRotation`)) (.yaw (`self.GetControlRotation`))) false false))))

(fn `UserConstructionScript`)