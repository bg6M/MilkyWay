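; Lobby game mode that gathers players for a session and starts the match once the lobby is full.
; Each login is tracked, then after a retriggerable delay the player count is checked against the session's connection limit, kicking any excess as "Server Full".
; At or over capacity it updates the session, waits, then runs the console command selected by the game instance's MapIndex.
; Logout untracks and kicks the leaving controller; a spawn-and-possess loop is unconnected.
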(event `self.ReceiveBeginPlay`
  (bind _asbp_game_instance (cast `/Game/DEV/Players/FirstPerson/Blueprints/BP_GameInstance` (`GameplayStatics.GetGameInstance`)))
  (set `self.As BP Game Instance` _asbp_game_instance))

(event `self.K2_OnLogout`
  (params (ExitingController :type "Controller Object Reference"))
  (bind _asplayer_controller (cast `PlayerController` ExitingController))
  (`KismetArrayLibrary.Array_RemoveItem` (`self.PlayersController`) _asplayer_controller)
  (`AdvancedSessionsLibrary.KickPlayer` _asplayer_controller "Quit"))

(event `self.K2_PostLogin`
  (params (NewPlayer :type "PlayerController Object Reference"))
  (`KismetArrayLibrary.Array_AddUnique` (`self.PlayersController`) NewPlayer)
  (`KismetSystemLibrary.RetriggerableDelay` 2.0)
  (bind (_numconnections _numprivateconnections _bislan _bisdedicated _ballowinvites _ballowjoininprogress _bisanticheatenabled _builduniqueid _extrasettings) (`AdvancedSessionsLibrary.GetSessionSettings`)
    (:`OnSuccess`
      (if (> (`KismetArrayLibrary.Array_Length` (`GameStateBase.PlayerArray` (`GameplayStatics.GetGameState`))) _numconnections)
        (bind (_arrayindex _arrayelement) (`/Engine/EditorBlueprintResources/StandardMacros.ReverseForEachLoop` (`self.PlayersController`))
          (:`LoopBody`
            (if (>= _arrayindex _numconnections)
              (`AdvancedSessionsLibrary.KickPlayer` _arrayelement "Server Full")))
          (:`Completed`
            (`UpdateSessionCallbackProxyAdvanced.UpdateSession` _extrasettings _numconnections 0 _bislan :!label _label
              (:`OnSuccess`
                (`KismetSystemLibrary.Delay` 3.0)
                (`KismetSystemLibrary.ExecuteConsoleCommand` (`|GetArrayItem` (`self.Command`) (`/Game/DEV/Players/FirstPerson/Blueprints/BP_GameInstance.MapIndex` (`self.As BP Game Instance`))) null)))))
        (elif (== _numconnections (`KismetArrayLibrary.Array_Length` (`GameStateBase.PlayerArray` (`GameplayStatics.GetGameState`))))
          (goto _label))))))

(fn `UserConstructionScript`)