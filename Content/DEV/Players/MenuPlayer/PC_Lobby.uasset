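; PC_Lobby is a lobby Blueprint, apparently a player controller, that sets up input and on-screen UI on BeginPlay.
; If the Enhanced Input subsystem is valid, it adds IMC_Default, then checks for player controller 0, retrying after a delay until valid.
; It then creates a widget, adds it to the viewport, switches to UI-only input focused on it and shows the mouse cursor.
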(event `self.ReceiveBeginPlay`
  (bind _returnvalue (`GameplayStatics.GetPlayerController` 0))
  (bind _returnvalue_2 (subsystem `EnhancedInputLocalPlayerSubsystem`))
  (`/Engine/EditorBlueprintResources/StandardMacros.IsValid` _returnvalue_2
    (:`Is Valid`
      (`EnhancedInputSubsystemInterface.AddMappingContext` _returnvalue_2 "/Game/DEV/Players/FirstPerson/Input/IMC_Default.IMC_Default" 0 (struct))
      (`/Engine/EditorBlueprintResources/StandardMacros.IsValid` _returnvalue :!label _label
        (:`Is Valid`
          (bind _returnvalue_3 (`|CreateWidget` (`self.Class`) _returnvalue))
          (`UserWidget.AddToViewport` _returnvalue_3 0)
          (`WidgetBlueprintLibrary.SetInputMode_UIOnlyEx` _returnvalue _returnvalue_3 "DoNotLock" true)
          (set `PlayerController.bShowMouseCursor` true _returnvalue))
        (:`Is Not Valid`
          (`KismetSystemLibrary.Delay` 3.0)
          (goto _label))))))

(fn `UserConstructionScript`)